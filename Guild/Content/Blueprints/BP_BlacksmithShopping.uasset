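; BP_BlacksmithShopping is a clickable blacksmith shop actor that opens the weapon shop UI.
; BeginPlay enables click events on player controller 0, and clicking the StaticMesh hides every top-level user widget.
; The click then shows the existing WB_BlacksmithShop_Weapon or, if none is valid, creates one and adds it to the viewport.
; An unconnected variant that always creates a new widget remains in the graph and never runs.
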(event OnClicked(StaticMesh)
  (params (TouchedComponent :type Primitive%20Component%20Object%20Reference) (ButtonPressed :type Key%20Structure))
  (Development|PrintString "Blacksmith shop hit")
  (bind _foundwidgets (Widget|GetAllWidgetsOfClass "/Script/UMG.UserWidget" true))
  (for _array_element _foundwidgets
    (Widget|SetVisibility _array_element "Hidden"))
  (bind _foundwidgets_2 (Widget|GetAllWidgetsOfClass "/Game/Blueprints/UI/WB_BlacksmithShop_Weapon.WB_BlacksmithShop_Weapon_C" true))
  (Utilities|IsValid (Utilities|Array|Get(acopy) _foundwidgets_2)
    (:Is%20Valid
      (Widget|SetVisibility (Utilities|Array|Get(acopy) _foundwidgets_2) "Visible"))
    (:Is%20Not%20Valid
      (Development|PrintString "No blacksmith widget found")
      (bind _returnvalue (UserInterface|CreateWidget "/Game/Blueprints/UI/WB_BlacksmithShop_Weapon.WB_BlacksmithShop_Weapon_C"))
      (UserInterface|Viewport|AddtoViewport _returnvalue 0)))
  (Variables|/Script/Engine.PlayerController|SetbEnableClickEvents (Game|GetPlayerController 0) true))

(event EventBeginPlay
  (Variables|/Script/Engine.PlayerController|SetbEnableClickEvents (Game|GetPlayerController 0) true))

(event Collision|EventActorBeginOverlap
  (params (OtherActor :type Actor%20Object%20Reference)))

(event EventTick
  (params (DeltaSeconds :type Float%20%28single-precision%29)))

(fn ConstructionScript)