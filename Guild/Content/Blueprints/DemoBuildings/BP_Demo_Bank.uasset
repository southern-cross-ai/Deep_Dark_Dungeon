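; Demo bank building for a grid-based building system that counts the demo houses around it.
; On BeginPlay it sets its static mesh's yaw in quarter turns from ObjectDirection.
; SetupPlaceableObject runs the parent setup, then sphere-overlaps for BP_Demo_House around the occupied center cell and stores the count in BuildingsInArea.
; The sphere radius is half of RadiusInCells times the grid cell size; a per-house cast loop is left unconnected.
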(event EventBeginPlay
  (|CallParentFunction)
  (Transformation|SetWorldRotation (Variables|Components|GetStaticMesh) (Math|Rotator|MakeRotator 0.0 0.0 (Utilities|Select :Index (Variables|Default|GetObjectDirection) :Option%200 0.0 :Option%201 9e+01 :Option%202 1.8e+02 :Option%203 -9e+01)) false false))

(fn ConstructionScript)

(fn SetupPlaceableObject
  (bind _occupiedcentercell (Variables|Default|GetOccupiedCenterCell))
  (bind _buildmanager (Variables|Default|GetBuildManager))
  (bind _location (Default|GetCellCenter _buildmanager _occupiedcentercell))
  (|CallParentFunction)
  (bind _outactors (Collision|SphereOverlapActors (Math|Vector|MakeVector (.x _location) (.y _location) (.z (Transformation|GetActorLocation))) (* (* (Variables|Settings|GetRadiusInCells) (Variables|/Game/Blueprints/BP_BuildManager.BP_BuildManager_C|GetGridCellSizeXY _buildmanager)) 0.5) (Utilities|Array|MakeArray "ObjectTypeQuery1" "ObjectTypeQuery2") "/Game/Blueprints/DemoBuildings/BP_Demo_House.BP_Demo_House_C"))
  (Variables|Default|SetBuildingsInArea (Utilities|Array|Length _outactors)))