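; Turn-based JRPG battle controller that runs unit turns, deals damage and saves combat data to the game instance when battle ends.
; Turn start applies buff effects, updates the turn-order UI, then starts the turn or skips stunned and death's-door units.
; Position swaps use a confirmation widget and temporary placeholder actors filling empty player slots as targets.
; Helpers order units by Speed and spawn floating damage text.
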(event Custom|Swap%20Position
  ;[1 1 1] New Custom ent Swap Position
  (Utilities|FlowControl|Sequence
    (:then_0
      (CallFunction|FillSwapPlaceholder))
    (:then_1
      (bind _asbp_combat_player_unit_base (Utilities|Casting|CastToBP_CombatPlayerUnitBase (Variables|Default|GetcurrentAttackingUnit)))
      (Default|ChangeCameraforSwap _asbp_combat_player_unit_base)
      (Utilities|IsValid (Variables|Default|GetswapUI)
        (:Is%20Valid
          _)
        (:Is%20Not%20Valid
          ;;[1 1 1] Create New Widget Window
          (bind _returnvalue (UserInterface|CreateWidget "/Game/Combat/Blueprints/UI/Dialogues/BP_SwapConfirmDialogue.BP_SwapConfirmDialogue_C" (Variables|Default|GetjRPGPlayerController) "Swap Position"))
          (bind _output_get (Variables|Default|SetswapUI _returnvalue))
          (UserInterface|Viewport|AddtoViewport _output_get 0)))
      (Widget|SetRenderOpacity (Variables|Default|GetswapUI) 1.0)
      (Default|ShowSwap (Variables|Default|GetswapUI))
      (EventDispatchers|BindEventtoOnConfirmed (Variables|Default|GetswapUI) (delegate Custom|On%20Swap%20Confirmed%20Handler))
      (EventDispatchers|BindEventtoOnCancelled (Variables|Default|GetswapUI) (delegate Custom|On%20Swap%20Cancelled%20Handler)))))

(event Custom|Idle
  (bind _currentattackingunit (Variables|Default|GetcurrentAttackingUnit))
  ;[1 1 1] New custom event idle
  (Utilities|IsValid _currentattackingunit
    (:Is%20Valid
      (Default|EndTurn _currentattackingunit))))

(event Custom|On%20Swap%20Confirmed%20Handler
  ;[1 1 1] New Custom ent Swap Position
  ;;[1 1 1] Swap
  (bind _targetunit (Default|GetTargetUnit (stale Custom|Swap%20Position _asbp_combat_player_unit_base) true))
  (if (== _targetunit (stale Custom|Swap%20Position _asbp_combat_player_unit_base)) ; if swap with it self; equal to cancel
    ;;[1 1 1] Cancel Swap
    (Widget|SetRenderOpacity (Variables|Default|GetswapUI) 0.0)
    (Default|StartTurn (Variables|Default|GetcurrentAttackingUnit))
    (CallFunction|RemoveSwapPlaceholder)
    (else
      (Utilities|FlowControl|Sequence
        (:then_0
          (bind _asbp_combat_player_unit_base (Utilities|Casting|CastToBP_CombatPlayerUnitBase _targetunit))
          (Default|SwapPositionwith _asbp_combat_player_unit_base (stale Custom|Swap%20Position _asbp_combat_player_unit_base)))
        (:then_1
          (Utilities|FlowControl|Delay 2.0)
          (Widget|SetRenderOpacity (Variables|Default|GetswapUI) 0.0)
          (Default|EndTurn (stale Custom|Swap%20Position _asbp_combat_player_unit_base)))
        (:then_2
          (CallFunction|RemoveSwapPlaceholder))))))

(event Custom|On%20Swap%20Cancelled%20Handler
  ;[1 1 1] New Custom ent Swap Position
  ;;[1 1 1] Cancel Swap
  (Widget|SetRenderOpacity (Variables|Default|GetswapUI) 0.0)
  (Default|StartTurn (Variables|Default|GetcurrentAttackingUnit))
  (CallFunction|RemoveSwapPlaceholder))

(event EventOnUnitsTurnStarted
  (bind _battleui (Variables|Default|GetbattleUI))
  ;[1 1 1] Units turn starts
  (bind _output_get (Variables|Default|SetcurrentAttackingUnit (Utilities|GetNextReadyUnit)))
  (Utilities|IsValid _output_get
    (:Is%20Valid
      (EventDispatchers|BindEventtoOnTurnEnded (Variables|Default|GetcurrentAttackingUnit) (delegate EventOnTurnEndedHandler))
      (bind _isunitdead (Default|IsUnitDead (Variables|Default|GetcurrentAttackingUnit)))
      (if _isunitdead
        (if (or (Variables|/Game/TurnBasedJRPGTemplate/Blueprints/Units/BP_UnitBase.BP_UnitBase_C|GetisStun (Variables|Default|GetcurrentAttackingUnit)) (Variables|/Game/Combat/Blueprints/Unit/PlayerUnits/BP_CombatPlayerUnitBase.BP_CombatPlayerUnitBase_C|Getis%20On%20DeathDoor (stale _asbp_combat_player_unit_base_2))) :!label _label
          (Default|EndTurn (Variables|Default|GetcurrentAttackingUnit) :!label _label_2)
          (else
            (Default|StartTurn (Variables|Default|GetcurrentAttackingUnit) :!label _label_3)
            (bind _asbp_combat_player_unit_base (Utilities|Casting|CastToBP_CombatPlayerUnitBase (Variables|Default|GetcurrentAttackingUnit))
              (:then
                (Default|SetReachableEnemies _asbp_combat_player_unit_base)
                (bind _targetunit (Default|GetTargetUnit (Variables|Default|GetcurrentAttackingUnit) false))
                (Utilities|IsValid _targetunit
                  (:Is%20Valid
                    (Default|ShowUnitBattleDetails _battleui))))
              (:CastFailed
                (Default|HideUnitBattleDetails _battleui)))))
        (else
          ;;[0.4084 0.1946 1] Buff Effects
          (bind _keys (Utilities|Map|Keys (Variables|/Game/TurnBasedJRPGTemplate/Blueprints/Units/BP_UnitBase.BP_UnitBase_C|GetactiveBuffs (Variables|Default|GetcurrentAttackingUnit))))
          (for _array_element _keys
            (Default|ProcessTurnEffect (.Value (Utilities|Map|Find (Variables|/Game/TurnBasedJRPGTemplate/Blueprints/Units/BP_UnitBase.BP_UnitBase_C|GetactiveBuffs (Variables|Default|GetcurrentAttackingUnit)) _array_element))))
          (Default|UpdateTurnOrderList (Variables|Default|GetbattleUI) (Variables|Default|GetcurrentAttackingUnit))
          (bind _asbp_combat_player_unit_base_2 (Utilities|Casting|CastToBP_CombatPlayerUnitBase (Variables|Default|GetcurrentAttackingUnit))
            (:then
              (goto _label))
            (:CastFailed
              (if (Variables|/Game/TurnBasedJRPGTemplate/Blueprints/Units/BP_UnitBase.BP_UnitBase_C|GetisStun (Variables|Default|GetcurrentAttackingUnit))
                (goto _label_2)
                (else
                  (goto _label_3))))))))
    (:Is%20Not%20Valid
      (Variables|Default|SetcurrentAttackingUnit 0)
      (Default|HideUnitBattleDetails (Variables|Default|GetbattleUI))
      (CallFunction|OnUnitsTurnEnded))))

(event EventOnTurnEndedHandler
  ;[1 1 1] Units turn starts
  (EventDispatchers|UnbindEventfromOnTurnEnded (Utilities|GetNextReadyUnit) (delegate EventOnTurnEndedHandler))
  (Variables|Default|SetcurrentAttackingUnit 0)
  (Default|HideUnitBattleDetails (Variables|Default|GetbattleUI))
  (CallFunction|OnUnitsTurnEnded))

(event EventOnBattleOver
  (Development|PrintString "Battle Over; Start Next Scene" true true "(R=1.000000,G=0.099172,B=0.000000,A=1.000000)" 5e+01)
  (bind _asbp_combat_game_instance (Utilities|Casting|CastToBP_CombatGameInstance (Game|GetGameInstance)))
  (Default|SaveCombatData _asbp_combat_game_instance)
  (|CallParentFunction))

(event EventBeginPlay
  ;[1 1 1] Load game if needed
  (CallFunction|PlayExploreTheme)
  (if true
    (Utilities|FlowControl|Delay 0.1)))

(fn ConstructionScript
  (|CallParentFunction))

(fn DealDamage
  (params (pureDamage :type Integer) (damageMultiplier :type Float%20%28double-precision%29))
  (if (Utilities|IsValid (Variables|Default|GetcurrentTargetUnit))
    (bind _ishit (|CallParentFunction pureDamage damageMultiplier))
    (return _ishit)))

(fn SwapPlayerPosition
  (params (player_01 :type BP%20Combat%20Player%20Unit%20Base%20Object%20Reference) (player_02 :type BP%20Combat%20Player%20Unit%20Base%20Object%20Reference))
  (Utilities|FlowControl|Sequence
    (:then_0
      (bind _output_get (LocalVariables|SetpositionTemp (Variables|/Game/Combat/Blueprints/Unit/PlayerUnits/BP_CombatPlayerUnitBase.BP_CombatPlayerUnitBase_C|GetcurrentPosition player_01)))
      (Variables|/Game/Combat/Blueprints/Unit/PlayerUnits/BP_CombatPlayerUnitBase.BP_CombatPlayerUnitBase_C|SetcurrentPosition player_01 (Variables|/Game/Combat/Blueprints/Unit/PlayerUnits/BP_CombatPlayerUnitBase.BP_CombatPlayerUnitBase_C|GetcurrentPosition player_02))
      (Variables|/Game/Combat/Blueprints/Unit/PlayerUnits/BP_CombatPlayerUnitBase.BP_CombatPlayerUnitBase_C|SetcurrentPosition player_02 _output_get))
    (:then_1
      (LocalVariables|Setplayer01NewPosition (Transformation|GetActorLocation player_02))
      (LocalVariables|Setplayer02NewPosition (Transformation|GetActorLocation player_01)))
    (:then_2
      (Default|MovetoTargetwithRoot player_02 (LocalVariables|Getplayer02NewPosition) false 7e+02)
      (Default|MovetoTargetwithRoot player_01 (LocalVariables|Getplayer01NewPosition) false 7e+02))))

(fn FillSwapPlaceholder
  (bind _currentbattle (Variables|Default|GetcurrentBattle))
  (Utilities|FlowControl|Sequence
    (:then_0
      (for _array_element (Variables|/Game/TurnBasedJRPGTemplate/Blueprints/Battle/BP_BattleBase.BP_BattleBase_C|GetplayerUnits (Variables|Default|GetcurrentBattle))
        (bind _asbp_combat_player_unit_base (Utilities|Casting|CastToBP_CombatPlayerUnitBase _array_element))
        (Utilities|Array|SetArrayElem (LocalVariables|GetpositionLog) (Variables|/Game/Combat/Blueprints/Unit/PlayerUnits/BP_CombatPlayerUnitBase.BP_CombatPlayerUnitBase_C|GetcurrentPosition _asbp_combat_player_unit_base) true)
        (Development|PrintString (Utilities|String|Append (Utilities|String|ToString(Integer) (Variables|/Game/Combat/Blueprints/Unit/PlayerUnits/BP_CombatPlayerUnitBase.BP_CombatPlayerUnitBase_C|GetcurrentPosition _asbp_combat_player_unit_base)) " do have Player"))))
    (:then_1
      (for (_array_element_2 _array_index) (LocalVariables|GetpositionLog)
        (if (not _array_element_2)
          (bind _returnvalue (Game|SpawnActorfromClass :Class "/Game/Combat/Blueprints/Unit/PlayerUnits/BP_CombatSwapPlaceHolder.BP_CombatSwapPlaceHolder_C" :SpawnTransform (Transformation|GetActorTransform (Utilities|Array|Get(acopy) (Variables|/Game/TurnBasedJRPGTemplate/Blueprints/Battle/BP_BattleBase.BP_BattleBase_C|GetplayerSpawnLocations _currentbattle) _array_index)) :CollisionHandlingOverride "Undefined" :TransformScaleMethod "MultiplyWithRoot" :currentPosition _array_index :battle _currentbattle :Instigator 0))
          (Utilities|Array|Add (Variables|/Game/TurnBasedJRPGTemplate/Blueprints/Battle/BP_BattleBase.BP_BattleBase_C|GetplayerUnits (Variables|Default|GetcurrentBattle)) _returnvalue))))
    (:then_2
      (Utilities|Array|Clear (LocalVariables|GetpositionLog)))))

(fn RemoveSwapPlaceholder
  (bind _currentbattle (Variables|Default|GetcurrentBattle))
  (bind _playerunits (Variables|/Game/TurnBasedJRPGTemplate/Blueprints/Battle/BP_BattleBase.BP_BattleBase_C|GetplayerUnits _currentbattle))
  (Utilities|FlowControl|Sequence
    (:then_0
      (for _array_element _playerunits
        (bind _asbp_combat_swap_place_holder (Utilities|Casting|CastToBP_CombatSwapPlaceHolder _array_element))
        (Utilities|Array|RemoveItem _playerunits _asbp_combat_swap_place_holder)
        (Actor|DestroyActor _asbp_combat_swap_place_holder)))))

(fn DealDamageto
  (params (pure%20Damage :type Integer) (Damage%20Multiplier :type Float%20%28double-precision%29) (target :type BP%20Unit%20Base%20Object%20Reference))
  ;[1 1 1] Attacker deals damage to target unit
  (bind _damage (CallFunction|CalculateDamage pure%20Damage Damage%20Multiplier))
  (Game|SpawnActorfromClass "/Game/TurnBasedJRPGTemplate/Blueprints/Battle/BP_DamageText.BP_DamageText_C" (Math|Conversions|ToTransform(Vector) (Transformation|GetWorldLocation (Variables|/Game/TurnBasedJRPGTemplate/Blueprints/Units/BP_UnitBase.BP_UnitBase_C|GetProjectileHitLocation (Variables|Default|GetcurrentTargetUnit)))) "Undefined" "OverrideRootScale" 0 _damage target false false 0)
  (Default|TakeDamage target _damage)
  (return (> _damage 0)))

(fn GetReadyUnitsBasedonSpeed
  (bind _currentbattle (Variables|Default|GetcurrentBattle))
  (bind _allunits (LocalVariables|GetallUnits))
  ;[1 1 1] Get next ready to attack unit based on speed
  (Utilities|Array|AppendArray (LocalVariables|GetallUnits) (Variables|/Game/TurnBasedJRPGTemplate/Blueprints/Battle/BP_BattleBase.BP_BattleBase_C|GetplayerUnits _currentbattle))
  (Utilities|Array|AppendArray (LocalVariables|GetallUnits) (Variables|/Game/TurnBasedJRPGTemplate/Blueprints/Battle/BP_BattleBase.BP_BattleBase_C|GetenemyUnits _currentbattle))
  (for _array_element (LocalVariables|GetallUnits) :!label _label
    (if (>= (Variables|/Game/TurnBasedJRPGTemplate/Blueprints/Units/BP_UnitBase.BP_UnitBase_C|Getspeed _array_element) (LocalVariables|GetcurrentHighestSpeed))
      (LocalVariables|SetcurrentHighestSpeed (Variables|/Game/TurnBasedJRPGTemplate/Blueprints/Units/BP_UnitBase.BP_UnitBase_C|Getspeed _array_element))
      (LocalVariables|SethighestSpeedUnit _array_element)))
  (Utilities|Array|Add (LocalVariables|GetcurrentReadyToAttackUnits) (LocalVariables|GethighestSpeedUnit))
  (Utilities|Array|RemoveItem _allunits (LocalVariables|GethighestSpeedUnit))
  (LocalVariables|SetcurrentHighestSpeed 0)
  (if (!= (Utilities|Array|Length _allunits) 0)
    (goto _label)
    (else
      (return (LocalVariables|GetcurrentReadyToAttackUnits)))))