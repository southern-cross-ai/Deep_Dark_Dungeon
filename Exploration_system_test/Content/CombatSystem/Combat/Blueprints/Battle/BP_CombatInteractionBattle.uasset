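; Turn-based RPG battle actor that starts combat shortly after BeginPlay and overrides how player and enemy units spawn.
; Party members, sorted by speed, take their first free preferred slot, with level derived from Exp and hero data from the save game.
; Each enemy slot spawns a random enemy, tallying drops and Exp/gold rewards.
; Rewards scale by slot index for BP_CombatEnemyUnitBase enemies, by level for others.
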(event EventBeginPlay
  (|CallParentFunction)
  (Utilities|FlowControl|Delay 0.1)
  (CallFunction|StartBattle (Variables|Default|GetEnemy%20List) (Variables|Default|GetOff%20Level%20Battle%20Data)))

(fn ConstructionScript
  (|CallParentFunction))

(fn CallSpawnPlayerUnits
  ;[1 1 1] Spawn player units
  (bind _asbp_combat_player_controller (Utilities|Casting|CastToBP_CombatPlayerController (Variables|Default|GetjRPGPlayerController)))
  (Default|SortPartyMemberbySpeed _asbp_combat_player_controller)
  (Utilities|Map|Clear (Variables|Default|GetplayerUnitLevels))
  (for _array_element (Variables|/Game/TurnBasedJRPGTemplate/Blueprints/Controllers/BP_JRPGPlayerController.BP_JRPGPlayerController_C|GetpartyMembers _asbp_combat_player_controller)
    (bind _asbp_combat_player_unit_base (Utilities|Casting|CastToBP_CombatPlayerUnitBaseClass _array_element))
    (bind _array_element_2 (Utilities|Array|ForEachLoopwithBreak (.preferredPosition (Utilities|Struct|BreakS_PlayerUnitData (.Value (Utilities|Map|Find (Variables|/Game/TurnBasedJRPGTemplate/Blueprints/Controllers/BP_JRPGPlayerController.BP_JRPGPlayerController_C|GetplayerUnits _asbp_combat_player_controller) _array_element)))) :!label _label)
      (:LoopBody
        (if (not (.Value (Utilities|Map|Find (LocalVariables|GetpositionMap) _array_element_2)))
          (bind _level (CallFunction|GetLevel (.Exp (Utilities|Struct|BreakS_PlayerUnitData (.Value (Utilities|Map|Find (Variables|/Game/TurnBasedJRPGTemplate/Blueprints/Controllers/BP_JRPGPlayerController.BP_JRPGPlayerController_C|GetplayerUnits _asbp_combat_player_controller) _array_element)))) (.expExponent (Utilities|GetClassDefaults _array_element)) (.maxLevel (Utilities|GetClassDefaults _array_element))))
          (Utilities|Map|Add (Variables|Default|GetplayerUnitLevels) _array_element _level)
          (bind _asbp_shared_data_game_instance (Utilities|Casting|CastToBP_SharedDataGameInstance (Game|GetGameInstance)))
          (bind _returnvalue (Game|SpawnActorfromClass _asbp_combat_player_unit_base (Math|Transform|MakeTransform (Transformation|GetActorLocation (Utilities|Array|Get(acopy) (Variables|Default|GetplayerSpawnLocations) _array_element_2)) (Transformation|GetActorRotation (Utilities|Array|Get(acopy) (Variables|Default|GetplayerSpawnLocations) _array_element_2))) "Undefined" "SelectDefaultAtRuntime" 0 _array_element_2 (.preferredPosition (Utilities|Struct|BreakS_PlayerUnitData (.Value (Utilities|Map|Find (Variables|/Game/TurnBasedJRPGTemplate/Blueprints/Controllers/BP_JRPGPlayerController.BP_JRPGPlayerController_C|GetplayerUnits _asbp_combat_player_controller) _array_element)))) (.Value (Utilities|Map|Find (Variables|/Game/Combat/Blueprints/Controller/BP_CombatPlayerController.BP_CombatPlayerController_C|GetParty%20Member%20UUIDs _asbp_combat_player_controller) _asbp_combat_player_unit_base)) (.Value (Utilities|Map|Find (Variables|/Game/Combat/Blueprints/SaveGame/BP_CombatSaveGame_HeroData.BP_CombatSaveGame_HeroData_C|GetHeroData (Variables|/Game/Maps/BP_SharedDataGameInstance.BP_SharedDataGameInstance_C|GetHero%20Data%20SaveGame _asbp_shared_data_game_instance)) (.Value (Utilities|Map|Find (Variables|/Game/Combat/Blueprints/Controller/BP_CombatPlayerController.BP_CombatPlayerController_C|GetParty%20Member%20UUIDs _asbp_combat_player_controller) _asbp_combat_player_unit_base)))) _level self 0))
          (Utilities|Array|Add (Variables|Default|GetplayerUnits) _returnvalue)
          (Utilities|Map|Add (LocalVariables|GetpositionMap) _array_element_2 true)
          (Development|PrintString (Utilities|String|Append "Spawn Actor: " (Utilities|GetDisplayName _returnvalue) " in Position: " (Utilities|String|ToString(Integer) _array_element_2)))
          (goto _label Break)))))
  (CallFunction|DisablePlayerUnits true))

(fn CallSpawnEnemyUnits
  (bind _self self)
  (Utilities|Map|Clear (Variables|Default|GetusableItemDrops))
  (Variables|Default|SettotalExpReward 0)
  (Variables|Default|SettotalGoldReward 0)
  (for (_array_element _array_index) (Variables|Default|GetenemySpawnLocations)
    (Default|Init _array_element self)
    (bind _enemyspawndata (CallFunction|GetEnemySpawnData _array_index))
    (bind (_enemyunit _level) (CallFunction|GetRandomEnemy _enemyspawndata))
    (bind _asbp_combat_enemy_unit_base (Utilities|Casting|CastToBP_CombatEnemyUnitBaseClass _enemyunit)
      (:then
        (if (Utilities|IsValidClass _asbp_combat_enemy_unit_base)
          (bind _returnvalue (Game|SpawnActorfromClass _asbp_combat_enemy_unit_base (Math|Transform|MakeTransform (Transformation|GetActorLocation _array_element) (Transformation|GetActorRotation _array_element)) "Undefined" "MultiplyWithRoot" 0 _array_index (.preferredPosition (Utilities|GetClassDefaults _asbp_combat_enemy_unit_base)) _level _self 0))
          (Variables|/Game/TurnBasedJRPGTemplate/Blueprints/Units/BP_UnitBase.BP_UnitBase_C|Settitle _returnvalue (Utilities|Text|ToText(String) (Utilities|String|Append (Utilities|String|ToString(Text) (Variables|/Game/TurnBasedJRPGTemplate/Blueprints/Units/BP_UnitBase.BP_UnitBase_C|Gettitle _returnvalue)) " " (Utilities|String|ToString(Integer) _array_index))))
          (Utilities|Array|Add (Variables|Default|GetenemyUnits) _returnvalue)
          (Variables|Default|SettotalExpReward (+ (Variables|Default|GettotalExpReward) (* (Variables|/Game/TurnBasedJRPGTemplate/Blueprints/Units/EnemyUnits/BP_EnemyUnitBase.BP_EnemyUnitBase_C|GetexpReward _returnvalue) _array_index)))
          (Variables|Default|SettotalGoldReward (+ (Variables|Default|GettotalGoldReward) (* (Variables|/Game/TurnBasedJRPGTemplate/Blueprints/Units/EnemyUnits/BP_EnemyUnitBase.BP_EnemyUnitBase_C|GetgoldReward _returnvalue) _array_index)))
          (CallFunction|DropUsableItems _returnvalue)
          (CallFunction|DropMiscItems _returnvalue)
          (CallFunction|DropEquipment _returnvalue)))
      (:CastFailed
        (if (Utilities|IsValidClass _enemyunit)
          (bind _returnvalue_2 (Game|SpawnActorfromClass _enemyunit (Math|Transform|MakeTransform (Transformation|GetActorLocation _array_element) (Transformation|GetActorRotation _array_element)) "Undefined" "SelectDefaultAtRuntime" 0 _level _self 0))
          (Utilities|Array|Add (Variables|Default|GetenemyUnits) _returnvalue_2)
          (Variables|Default|SettotalExpReward (+ (Variables|Default|GettotalExpReward) (* (Variables|/Game/TurnBasedJRPGTemplate/Blueprints/Units/EnemyUnits/BP_EnemyUnitBase.BP_EnemyUnitBase_C|GetexpReward _returnvalue_2) _level)))
          (Variables|Default|SettotalGoldReward (+ (Variables|Default|GettotalGoldReward) (* (Variables|/Game/TurnBasedJRPGTemplate/Blueprints/Units/EnemyUnits/BP_EnemyUnitBase.BP_EnemyUnitBase_C|GetgoldReward _returnvalue_2) _level)))
          (CallFunction|DropUsableItems _returnvalue_2)
          (CallFunction|DropMiscItems _returnvalue_2)
          (CallFunction|DropEquipment _returnvalue_2)))))
  (CallFunction|DisableEnemyUnits true))