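; BP_PlayerStatus is an actor that takes a snapshot of the health of two player teams when play begins.
; BeginPlay finds all BP_PlayerTeam actors and stores the first two as TeamA and TeamB, relying on the returned array order.
; It copies each team's TeamCurrentHealth once, with a validity check only on TeamB.
; Nothing here updates the values afterwards, as Tick and overlap are unused.
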(event EventBeginPlay
  (bind _outactors (Actor|GetAllActorsOfClass "/Game/Blueprints/BP_PlayerTeam.BP_PlayerTeam_C"))
  (bind _output_get (Variables|Default|SetTeamA (Utilities|Array|Get(acopy) _outactors)))
  (bind _output_get_2 (Variables|Default|SetTeamB (Utilities|Array|Get(acopy) _outactors 1)))
  (Variables|Default|SetTeamA%20Current%20Health (Variables|/Game/Blueprints/BP_PlayerTeam.BP_PlayerTeam_C|GetTeamCurrentHealth _output_get))
  (Utilities|IsValid (Variables|Default|GetTeamB)
    (:Is%20Valid
      (Variables|Default|SetTeamB%20Current%20Health (Variables|/Game/Blueprints/BP_PlayerTeam.BP_PlayerTeam_C|GetTeamCurrentHealth _output_get_2)))))

(event Collision|EventActorBeginOverlap
  (params (OtherActor :type Actor%20Object%20Reference)))

(event EventTick
  (params (DeltaSeconds :type Float%20%28single-precision%29)))

(fn ConstructionScript)