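; BP_TravelTrigger is a level-travel trigger volume that moves the player to another map when they walk into it.
; On overlap of TriggerCollision, it checks for a player-controlled Character and opens the level named by TargetName, if that string is not empty.
; The construction script applies an optional Niagara EffectAsset to its NiagaraEffect component, so each placed trigger can show its own visual.
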(event OnComponentBeginOverlap(TriggerCollision)
  (params (OverlappedComponent :type Primitive%20Component%20Object%20Reference) (OtherActor :type Actor%20Object%20Reference) (OtherComp :type Primitive%20Component%20Object%20Reference) (OtherBodyIndex :type Integer) (bFromSweep :type Boolean) (SweepResult :type Hit%20Result%20Structure%20%28by%20ref%29))
  (bind _targetname (Variables|Default|GetTargetName))
  (bind _ascharacter (Utilities|Casting|CastToCharacter OtherActor))
  (if (Pawn|IsPlayerControlled _ascharacter)
    (if (> (Utilities|String|Len _targetname) 0)
      (Game|OpenLevel(byName) (Utilities|String|StringToName _targetname)))))

(event EventBeginPlay)

(event Collision|EventActorBeginOverlap
  (params (OtherActor :type Actor%20Object%20Reference)))

(event EventTick
  (params (DeltaSeconds :type Float%20%28single-precision%29)))

(fn ConstructionScript
  (bind _effectasset (Variables|Default|GetEffectAsset))
  (Utilities|IsValid _effectasset
    (:Is%20Valid
      (Class|NiagaraComponent|SetAsset (Variables|Default|GetNiagaraEffect) _effectasset true))))