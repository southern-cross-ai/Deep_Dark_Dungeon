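; BP_TeamTool is a helper attached to BP_PlayerTeam that persists the player's four-hero team lineup between sessions.
; SaveTeamInfo copies the owner's four hero slot indices into a BP_SaveTeamInfo object and writes it to the TeamInfoSave slot.
; LoadTeamInfo reads that slot, or creates a fresh save object if none exists, and prints the indices.
; LoadTeamIndices runs the load and returns the four indices.
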(event Custom|Save%20TeamInfo
  (Utilities|IsValid (Variables|Default|GetTeamInfo)
    (:Is%20Valid
      _)
    (:Is%20Not%20Valid
      (bind _returnvalue (SaveGame|CreateSaveGameObject "/Game/Blueprints/BP_SaveTeamInfo.BP_SaveTeamInfo_C"))
      (Variables|Default|SetTeamInfo _returnvalue)))
  (bind _asbp_player_team (Utilities|Casting|CastToBP_PlayerTeam (Components|GetOwner)))
  (Utilities|Array|SetArrayElem (Variables|/Game/Blueprints/BP_SaveTeamInfo.BP_SaveTeamInfo_C|GetTeamIndices (Variables|Default|GetTeamInfo)) 0 (Variables|/Game/Blueprints/BP_PlayerTeam.BP_PlayerTeam_C|GetHeroSlot1Index _asbp_player_team) true)
  (Utilities|Array|SetArrayElem (Variables|/Game/Blueprints/BP_SaveTeamInfo.BP_SaveTeamInfo_C|GetTeamIndices (Variables|Default|GetTeamInfo)) 1 (Variables|/Game/Blueprints/BP_PlayerTeam.BP_PlayerTeam_C|GetHeroSlot2Index _asbp_player_team) true)
  (Utilities|Array|SetArrayElem (Variables|/Game/Blueprints/BP_SaveTeamInfo.BP_SaveTeamInfo_C|GetTeamIndices (Variables|Default|GetTeamInfo)) 2 (Variables|/Game/Blueprints/BP_PlayerTeam.BP_PlayerTeam_C|GetHeroSlot3Index _asbp_player_team) true)
  (Utilities|Array|SetArrayElem (Variables|/Game/Blueprints/BP_SaveTeamInfo.BP_SaveTeamInfo_C|GetTeamIndices (Variables|Default|GetTeamInfo)) 3 (Variables|/Game/Blueprints/BP_PlayerTeam.BP_PlayerTeam_C|GetHeroSlot4Index _asbp_player_team) true)
  (SaveGame|SaveGametoSlot (Variables|Default|GetTeamInfo) "TeamInfoSave"))

(event Custom|Load%20TeamInfo
  (bind _returnvalue (SaveGame|DoesSaveGameExist "TeamInfoSave"))
  (if _returnvalue
    (bind _returnvalue_2 (SaveGame|LoadGamefromSlot "TeamInfoSave"))
    (bind _asbp_save_team_info (Utilities|Casting|CastToBP_SaveTeamInfo _returnvalue_2))
    (Variables|Default|SetTeamInfo _asbp_save_team_info)
    (else
      (bind _returnvalue_3 (SaveGame|CreateSaveGameObject "/Game/Blueprints/BP_SaveTeamInfo.BP_SaveTeamInfo_C"))
      (Variables|Default|SetTeamInfo _returnvalue_3)))
  (Development|PrintString (Utilities|String|ToString(Integer) (Utilities|Array|Get(acopy) (Variables|/Game/Blueprints/BP_SaveTeamInfo.BP_SaveTeamInfo_C|GetTeamIndices (Variables|Default|GetTeamInfo)))))
  (Development|PrintString (Utilities|String|ToString(Integer) (Utilities|Array|Get(acopy) (Variables|/Game/Blueprints/BP_SaveTeamInfo.BP_SaveTeamInfo_C|GetTeamIndices (Variables|Default|GetTeamInfo)) 1)))
  (Development|PrintString (Utilities|String|ToString(Integer) (Utilities|Array|Get(acopy) (Variables|/Game/Blueprints/BP_SaveTeamInfo.BP_SaveTeamInfo_C|GetTeamIndices (Variables|Default|GetTeamInfo)) 2)))
  (Development|PrintString (Utilities|String|ToString(Integer) (Utilities|Array|Get(acopy) (Variables|/Game/Blueprints/BP_SaveTeamInfo.BP_SaveTeamInfo_C|GetTeamIndices (Variables|Default|GetTeamInfo)) 3))))

(event EventBeginPlay)

(event EventTick
  (params (DeltaSeconds :type Float%20%28single-precision%29)))

(fn LoadTeamIndices
  (bind _teaminfo (Variables|Default|GetTeamInfo))
  (bind _teamindices (Variables|/Game/Blueprints/BP_SaveTeamInfo.BP_SaveTeamInfo_C|GetTeamIndices _teaminfo))
  (CallFunction|LoadTeamInfo)
  (return (Utilities|Array|Get(acopy) _teamindices) (Utilities|Array|Get(acopy) _teamindices 1) (Utilities|Array|Get(acopy) _teamindices 2) (Utilities|Array|Get(acopy) _teamindices 3)))