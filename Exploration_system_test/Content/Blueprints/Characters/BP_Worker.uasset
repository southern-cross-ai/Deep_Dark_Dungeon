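; BP_Worker is a worker character that loops an aiming animation with a weapon in hand and a sparks effect.
; On BeginPlay it snaps the Weapon component to the skeletal mesh's "Weapon" socket, starts the animation and attaches a P_Sparks emitter there with a random location value.
; The MoveToLocation event is an empty stub; its AIMoveTo node is disconnected, so the event moves nothing.
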(event Custom|MoveToLocation
  (params (TargetLocation :type Vector)))

(event EventBeginPlay
  (bind _skeletalmesh (Variables|Default|GetSkeletalMesh))
  (Transformation|AttachComponentToComponent (Variables|Default|GetWeapon) _skeletalmesh "Weapon" "SnapToTarget" "SnapToTarget" "SnapToTarget" true)
  (Components|Animation|PlayAnimation _skeletalmesh "/Game/Characters/Anim/Aim_Space_Ironsights.Aim_Space_Ironsights" true)
  (Effects|SpawnEmitterAttached "/Game/StarterContent/Particles/P_Sparks.P_Sparks" _skeletalmesh "Weapon" (Math|Conversions|ToVector(Float) (Math|Random|RandomFloatinRange 0.0 3e+01)) "0, 0, 0" "1.000000,1.000000,1.000000" "SnapToTarget"))

(event Collision|EventActorBeginOverlap
  (params (OtherActor :type Actor%20Object%20Reference)))

(event EventTick
  (params (DeltaSeconds :type Float%20%28single-precision%29)))

(fn ConstructionScript)