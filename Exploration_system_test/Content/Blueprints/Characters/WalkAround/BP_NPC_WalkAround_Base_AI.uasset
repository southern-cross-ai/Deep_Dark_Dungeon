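; Base Blueprint for a walk-around NPC that seeds its AI blackboard at BeginPlay.
; It picks a random walk speed between its min and max, caches the blackboard and writes the speed as MaxWalkSpeed.
; It then stores its spawn location as StartLocation and the PatrolPoint component's world position as PatrolLocation.
; No movement logic runs here; the graph only supplies these blackboard values.
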(event EventBeginPlay
  (CallFunction|SetRandomWalkSpeed)
  (AI|Components|Blackboard|SetValueasVector (Variables|Default|GetBB) (Utilities|Name|MakeLiteralName "StartLocation") (Transformation|GetActorLocation))
  (AI|Components|Blackboard|SetValueasVector (Variables|Default|GetBB) (Utilities|Name|MakeLiteralName "PatrolLocation") (Transformation|GetWorldLocation (Variables|Default|GetPatrolPoint))))

(event Collision|EventActorBeginOverlap
  (params (OtherActor :type Actor%20Object%20Reference)))

(event EventTick
  (params (DeltaSeconds :type Float%20%28single-precision%29)))

(fn ConstructionScript)

(fn SetRandomWalkSpeed
  (Variables|Default|SetRandomWalkSpeed (Math|Random|RandomFloatinRange (Variables|Default|GetMinWalkSpeed) (Variables|Default|GetMaxWalkSpeed)))
  (Variables|Default|SetBB (AI|GetBlackboard 0))
  (AI|Components|Blackboard|SetValueasFloat (Variables|Default|GetBB) (Utilities|Name|MakeLiteralName "MaxWalkSpeed") (Variables|Default|GetRandomWalkSpeed)))