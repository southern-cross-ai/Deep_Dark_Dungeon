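; Fog of war manager that records the areas revealed by bases and player team actors in the RT_ViewPath render target.
; BeginPlay clears the target to black and stamps each BP_Base once, while Tick stamps every BP_PlayerTeam actor each frame.
; Each stamp converts the BP_FogViewComponent owner's location to map UV and draws a new M_FogBrush dynamic material, sized by view range relative to map size.
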(event EventTick
  (params (DeltaSeconds :type Float%20%28single-precision%29))
  (bind _outactors (Actor|GetAllActorsOfClass "/Game/Blueprints/BP_PlayerTeam.BP_PlayerTeam_C"))
  (for _array_element _outactors
    (CallFunction|DrawRTwithSelectedFogViewComponent (Actor|GetComponentbyClass _array_element "/Game/Blueprints/BP_FogViewComponent.BP_FogViewComponent_C"))))

(event EventBeginPlay
  (Rendering|ClearRenderTarget2D "/Game/Material/RT_ViewPath.RT_ViewPath")
  (bind _outactors (Actor|GetAllActorsOfClass "/Game/Blueprints/Structures/BP_Base.BP_Base_C"))
  (for _array_element _outactors
    (CallFunction|DrawRTwithSelectedFogViewComponent (Actor|GetComponentbyClass _array_element "/Game/Blueprints/BP_FogViewComponent.BP_FogViewComponent_C"))))

(fn DrawRTwithSelectedFogViewComponent
  (params (FogViewCompnent :type Fog%20View%20Component%20Object%20Reference))
  (bind _mapsize (Variables|Default|GetMapSize))
  (bind _uvresult (Class|FogViewComponent|GetHitUVbyOwnerLoc FogViewCompnent _mapsize))
  (bind _returnvalue (Rendering|Material|CreateDynamicMaterialInstance "/Game/Material/M_FogBrush.M_FogBrush" "None" "None" :!class /Script/Engine.KismetMaterialLibrary))
  (Rendering|Material|SetVectorParameterValue _returnvalue "Location" (Utilities|Struct|MakeLinearColor (.x _uvresult) (.y _uvresult) 0.0 1.0) :!class /Script/Engine.MaterialInstanceDynamic)
  (Rendering|Material|SetScalarParameterValue _returnvalue "BrushSize" (/ (Variables|/Script/Exploration.FogViewComponent|GetViewRange FogViewCompnent) _mapsize) :!class /Script/Engine.MaterialInstanceDynamic)
  (Rendering|DrawMaterialtoRenderTarget "/Game/Material/RT_ViewPath.RT_ViewPath" _returnvalue))