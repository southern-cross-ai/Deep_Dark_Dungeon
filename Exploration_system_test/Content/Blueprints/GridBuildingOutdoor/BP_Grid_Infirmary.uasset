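; Grid building actor for the outdoor infirmary that acts as a clickable entrance to the infirmary level.
; BeginPlay turns on click events for the first player controller.
; Clicking its static mesh saves through the shared data game instance, then opens the Infirmary_Test level and prints a debug message.
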(event OnClicked(StaticMesh)
  (params (TouchedComponent :type Primitive%20Component%20Object%20Reference) (ButtonPressed :type Key%20Structure))
  (bind _asbp_shared_data_game_instance (Utilities|Casting|CastToBP_SharedDataGameInstance (Game|GetGameInstance)))
  (Default|Save _asbp_shared_data_game_instance)
  (Game|OpenLevel(byName) "Infirmary_Test")
  (Development|PrintString "oepn level"))

(event EventBeginPlay
  (|CallParentFunction)
  (Variables|/Script/Engine.PlayerController|SetbEnableClickEvents (Game|GetPlayerController 0) true))

(event Collision|EventActorBeginOverlap
  (params (OtherActor :type Actor%20Object%20Reference)))

(event EventTick
  (params (DeltaSeconds :type Float%20%28single-precision%29))
  (|CallParentFunction DeltaSeconds) ; This node is disabled and will not be called.\nDrag off pins to build functionality.
)

(fn ConstructionScript
  (|CallParentFunction))