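; BP_Tree_04 is a placeable tree for the outdoor grid building system that appears through timed construction stages.
; On spawn it disables the BP_BuildManager building tool and applies its placement rotation.
; Tick maps elapsed time over BuildingTime to staged meshes, ending on the current level's mesh.
; Releasing a click on the finished tree re-enables the tool with this object, frees its occupied cells and destroys the actor.
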(event EventBeginPlay
  (|CallParentFunction)
  (Utilities|FlowControl|Sequence
    (:then_0
      (Actor|Tick|SetActorTickEnabled true))
    (:then_1
      (bind _returnvalue (Actor|GetActorOfClass "/Game/Blueprints/BP_BuildManager.BP_BuildManager_C"))
      (Default|DisableBuildingTool _returnvalue))
    (:then_2
      (Transformation|SetWorldRotation (Variables|Default|GetStaticMesh) (Math|Rotator|MakeRotator 0.0 0.0 (Utilities|Select :Index (Variables|Default|GetObjectDirection) :Option%200 0.0 :Option%201 9e+01 :Option%202 1.8e+02 :Option%203 -9e+01)) false false))))

(event EventTick
  (params (DeltaSeconds :type Float%20%28single-precision%29))
  (Utilities|FlowControl|Sequence
    (:then_0
      ;[1 1 1] Add spawned Time each Tick
      (bind _output_get (Variables|Default|SetspawnedTime (+ (Variables|Default|GetspawnedTime) DeltaSeconds)))
      (Development|PrintString (Utilities|String|ToString(Float) _output_get) false false "(R=0.848929,G=1.000000,B=0.423130,A=1.000000)" 2e+01))
    (:then_1
      (if (not (Variables|Default|GetbuildingComplete))
        (bind _mesh (CallFunction|GetBuildingProcedureMesh))
        (Components|StaticMesh|SetStaticMesh (Variables|Default|GetStaticMesh) _mesh)))))

(event EventActorOnReleased
  (params (ButtonReleased :type Key%20Structure))
  ;[1 1 1] Actor Click Event /// TODO: Open UI ///
  (if (Variables|Default|GetbuildingComplete)
    (Utilities|FlowControl|Sequence
      (:then_0
        (bind _returnvalue (Actor|GetActorOfClass "/Game/Blueprints/BP_BuildManager.BP_BuildManager_C"))
        (Utilities|FlowControl|Delay 0.0001)
        (Default|EnableBuildingTool _returnvalue (Variables|Default|GetObjectNameInTable)))
      (:then_1
        (for _array_element (Variables|Default|GetOccupiedCells)
          (Default|SetOccupancyData _returnvalue _array_element false)))
      (:then_3
        (Utilities|FlowControl|Delay 0.0001)
        (Actor|DestroyActor)))))

(fn ConstructionScript)

(fn GetBuildingProcedureMesh
  (bind _spawnedtime (Variables|Default|GetspawnedTime))
  (bind _buildingtime (Variables|Default|GetbuildingTime))
  (bind _buildingproceduremesh (Variables|Default|GetBuildingProcedureMesh))
  (bind _returnvalue (/ _spawnedtime _buildingtime))
  (if (>= _returnvalue 1.0)
    (Variables|Default|SetbuildingComplete true)
    (return (Utilities|Array|Get(acopy) (Variables|Default|GetMeshLevels) (Variables|Default|GetcurrentLevel)))
    (else
      (return (Utilities|Array|Get(acopy) _buildingproceduremesh (Math|Float|Floor (* _returnvalue (Utilities|Array|Length _buildingproceduremesh))))))))