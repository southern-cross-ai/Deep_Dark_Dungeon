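; BP_Grid_Farm is an outdoor grid building that periodically produces food once construction is complete.
; Tick compares elapsed spawn time against an interval for the current level, then calls ProduceFood.
; ProduceFood loads the "Resources" save slot, adds the level's amount to one enum-keyed resource and saves it back.
; Before saving, it passes a string-keyed copy of the totals to BP_BuildManager to update resource values.
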(event EventBeginPlay
  (|CallParentFunction) ; This node is disabled and will not be called.\nDrag off pins to build functionality.
)

(event Collision|EventActorBeginOverlap
  (params (OtherActor :type Actor%20Object%20Reference)))

(event EventTick
  (params (DeltaSeconds :type Float%20%28single-precision%29))
  (|CallParentFunction DeltaSeconds)
  (if (Variables|Default|GetbuildingComplete)
    (if (>= (- (Variables|Default|GetspawnedTime) (Variables|Default|GetproducedTime)) (Utilities|Array|Get(acopy) (Variables|Default|GetproducePerTime) (Variables|Default|GetcurrentLevel)))
      (Variables|Default|SetproducedTime (Variables|Default|GetspawnedTime))
      (CallFunction|ProduceFood))))

(fn ConstructionScript
  (|CallParentFunction))

(fn ProduceFood
  (bind _returnvalue (SaveGame|LoadGamefromSlot "Resources"))
  (bind _asbp_building_resources (Utilities|Casting|CastToBP_Building_Resources _returnvalue))
  (LocalVariables|SetResources%20Save%20Game _asbp_building_resources)
  (LocalVariables|Setresources%20E (Variables|/Game/Blueprints/SaveGame/BP_Building_Resources.BP_Building_Resources_C|Getresources _asbp_building_resources))
  (bind _returnvalue_2 (Actor|GetActorOfClass "/Game/Blueprints/BP_BuildManager.BP_BuildManager_C"))
  (Utilities|Map|Add (LocalVariables|Getresources%20E) "NewEnumerator3" (+ (.Value (Utilities|Map|Find (LocalVariables|Getresources%20E) "NewEnumerator3")) (Utilities|Array|Get(acopy) (Variables|Default|GetproducePerAmount) (Variables|Default|GetcurrentLevel))))
  (bind _keys (Utilities|Map|Keys (LocalVariables|Getresources%20E)))
  (for _array_element _keys
    (Utilities|Map|Add (LocalVariables|Getresources) (Utilities|String|EnumtoString _array_element) (.Value (Utilities|Map|Find (LocalVariables|Getresources%20E) _array_element))))
  (Default|UpdateResourcesValue _returnvalue_2 (Utilities|Struct|MakeS_ConstructionCost (LocalVariables|Getresources)) false false)
  (Variables|/Game/Blueprints/SaveGame/BP_Building_Resources.BP_Building_Resources_C|Setresources (LocalVariables|GetResources%20Save%20Game) (LocalVariables|Getresources%20E))
  (SaveGame|SaveGametoSlot (LocalVariables|GetResources%20Save%20Game) "Resources"))