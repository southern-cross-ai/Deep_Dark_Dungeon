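; Random generation actor that scatters actors from MeshArray across the BP_BuildManager grid shortly after BeginPlay.
; Each loop pass checks a random cell's occupancy in the build manager, printing a debug string if true and otherwise spawning a random class.
; The spawn position rolls fresh random coordinates scaled by cell size, so it is independent of the checked cell.
; The class pick uses RandomInteger(Length - 1), which excludes the last entry.
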(event EventBeginPlay
  (Utilities|FlowControl|Delay 0.1)
  (for _index (range 0 10)
    (bind _returnvalue (Actor|GetActorOfClass "/Game/Blueprints/BP_BuildManager.BP_BuildManager_C"))
    (if (Default|GetOccupancyData _returnvalue (Class|KismetMathLibrary|ToIntPoint(Vector2D) (Math|Vector2D|MakeVector2D (Math|Conversions|ToFloat(Integer) (Math|Random|RandomIntegerinRange (Math|Float|Truncate (+ (.X (Math|Vector|BreakVector (.Origin (Collision|GetActorBounds _returnvalue false false)))) (* (.X (Utilities|Struct|BreakIntPoint (Variables|/Game/Blueprints/BP_BuildManager.BP_BuildManager_C|GetGridSize _returnvalue))) -0.5))) (Math|Float|Truncate (+ (* (.X (Utilities|Struct|BreakIntPoint (Variables|/Game/Blueprints/BP_BuildManager.BP_BuildManager_C|GetGridSize _returnvalue))) 0.5) (.X (Math|Vector|BreakVector (.Origin (Collision|GetActorBounds _returnvalue false false)))))))) (Math|Conversions|ToFloat(Integer) (Math|Random|RandomIntegerinRange (Math|Float|Truncate (+ (.Y (Math|Vector|BreakVector (.Origin (Collision|GetActorBounds _returnvalue false false)))) (* (.Y (Utilities|Struct|BreakIntPoint (Variables|/Game/Blueprints/BP_BuildManager.BP_BuildManager_C|GetGridSize _returnvalue))) -0.5))) (Math|Float|Truncate (+ (* (.Y (Utilities|Struct|BreakIntPoint (Variables|/Game/Blueprints/BP_BuildManager.BP_BuildManager_C|GetGridSize _returnvalue))) 0.5) (.Y (Math|Vector|BreakVector (.Origin (Collision|GetActorBounds _returnvalue false false)))))))))))
      (Development|PrintString "Hello")
      (else
        (Game|SpawnActorfromClass :Class (Utilities|Array|Get(acopy) (Variables|Default|GetMesh%20Array) (Math|Random|RandomInteger (- (Utilities|Array|Length (Variables|Default|GetMesh%20Array)) 1))) :SpawnTransform (Math|Conversions|ToTransform(Vector) (Math|Vector|MakeVector (* (Math|Conversions|ToFloat(Integer) (Math|Random|RandomIntegerinRange (Math|Float|Truncate (+ (.X (Math|Vector|BreakVector (.Origin (Collision|GetActorBounds _returnvalue false false)))) (* (.X (Utilities|Struct|BreakIntPoint (Variables|/Game/Blueprints/BP_BuildManager.BP_BuildManager_C|GetGridSize _returnvalue))) -0.5))) (Math|Float|Truncate (+ (* (.X (Utilities|Struct|BreakIntPoint (Variables|/Game/Blueprints/BP_BuildManager.BP_BuildManager_C|GetGridSize _returnvalue))) 0.5) (.X (Math|Vector|BreakVector (.Origin (Collision|GetActorBounds _returnvalue false false)))))))) (Variables|/Game/Blueprints/BP_BuildManager.BP_BuildManager_C|GetGridCellSizeXY _returnvalue)) (* (Math|Conversions|ToFloat(Integer) (Math|Random|RandomIntegerinRange (Math|Float|Truncate (+ (.Y (Math|Vector|BreakVector (.Origin (Collision|GetActorBounds _returnvalue false false)))) (* (.Y (Utilities|Struct|BreakIntPoint (Variables|/Game/Blueprints/BP_BuildManager.BP_BuildManager_C|GetGridSize _returnvalue))) -0.5))) (Math|Float|Truncate (+ (* (.Y (Utilities|Struct|BreakIntPoint (Variables|/Game/Blueprints/BP_BuildManager.BP_BuildManager_C|GetGridSize _returnvalue))) 0.5) (.Y (Math|Vector|BreakVector (.Origin (Collision|GetActorBounds _returnvalue false false)))))))) (Variables|/Game/Blueprints/BP_BuildManager.BP_BuildManager_C|GetGridCellSizeXY _returnvalue)) 1.0)) :CollisionHandlingOverride "Undefined" :TransformScaleMethod "MultiplyWithRoot" :Instigator 0)))))

(fn ConstructionScript)