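; Indoor grid placer that previews a placeable object's footprint under the cursor and spawns it when building is allowed.
; DrawPlacementIndicators moves the mesh and per-cell indicators, coloring cells by indoor layer occupancy, height difference and optional unit overlap.
; BuildObject forces a final validity check, spawns the object with grid data, applies its building-procedure mesh and switches the main UI mode back.
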(event EventBeginPlay
  (|CallParentFunction) ; This node is disabled and will not be called.\nDrag off pins to build functionality.
)

(event Collision|EventActorBeginOverlap
  (params (OtherActor :type Actor%20Object%20Reference)))

(event EventTick
  (params (DeltaSeconds :type Float%20%28single-precision%29))
  (|CallParentFunction DeltaSeconds) ; This node is disabled and will not be called.\nDrag off pins to build functionality.
)

(fn ConstructionScript
  (|CallParentFunction))

(fn DrawPlacementIndicators
  (bind _objectsize (Variables|Default|GetObjectSize))
  (bind _buildmanager (Variables|Default|GetBuildManager))
  (bind _cellundercursor (Variables|/Game/Blueprints/BP_BuildManager.BP_BuildManager_C|GetCellUnderCursor _buildmanager))
  (bind _center (Default|GetCenterOfRectangularArea _buildmanager _cellundercursor _objectsize))
  (Utilities|FlowControl|Sequence
    (:then_0
      (if (or (Variables|/Game/Blueprints/BP_BuildManager.BP_BuildManager_C|GetCellUnderCursorHasChanged (Variables|Default|GetBuildManager)) (Variables|Default|GetForceUpdatePlaceIndicators))
        (Variables|Default|SetForceUpdatePlaceIndicators false)
        (Variables|Default|SetCanBuild true)
        (Default|GetCellLocation _buildmanager _cellundercursor)
        (Transformation|SetWorldLocation (Variables|Default|GetObectMesh) (Math|Vector|MakeVector (.x _center) (.y _center) 0.0) false false)
        (bind _cells (Default|GetCellsinRectangularArea (Variables|Default|GetBuildManager) (Variables|/Game/Blueprints/BP_BuildManager.BP_BuildManager_C|GetCellUnderCursor (Variables|Default|GetBuildManager)) (Variables|Default|GetObjectSize)))
        (Variables|Default|SetCellsForBuild _cells)
        (bind _asbp_indoor_build_mananger (Utilities|Casting|CastToBP_IndoorBuildMananger (Variables|Default|GetBuildManager))
          (:then
            (for (_array_element _array_index) (Variables|Default|GetCellsForBuild)
              (bind (_location _success) (Default|GetCellLocation (Variables|Default|GetBuildManager) _array_element))
              (LocalVariables|SetLocationLOCAL (Math|Vector|MakeVector (.x _location) (.y _location) (.z _location)))
              (Transformation|SetWorldLocation (Utilities|Array|Get(acopy) (Variables|Default|GetPlaceIndicators) _array_index) (LocalVariables|GetLocationLOCAL) false false)
              (if (Math|Boolean|ANDBoolean (not (Default|GetOccupancyDatabyLayer _asbp_indoor_build_mananger _array_element (Variables|Default|GetplacingLayerIndex))) (< (Math|Float|Absolute(Float) (- (.z _location) (LocalVariables|GetBaseBuildLevelLOCAL))) (Variables|Default|GetMaxHeightDifferenceForConstruction)) _success)
                (Rendering|Material|SetMaterial (Utilities|Array|Get(acopy) (Variables|Default|GetPlaceIndicators) _array_index) 0 (Variables|Default|GetPlaceAcceptedMaterial))
                (else
                  (Rendering|Material|SetMaterial (Utilities|Array|Get(acopy) (Variables|Default|GetPlaceIndicators) _array_index) 0 (Variables|Default|GetPlaceRejectedMaterial))
                  (Variables|Default|SetCanBuild false)))))
          (:CastFailed
            (Development|PrintString "ERROR: Failed To Cast BuildManager To IndoorBuilddManager" true true "(R=0.590278,G=0.000000,B=0.010035,A=1.000000)" 1e+01)))))
    (:then_1
      (if (Variables|Default|GetCheckUnitsInBuildArea)
        (bind (_unitsfound _unitsincells) (Default|FindUnitsinRectangularArea (Variables|Default|GetBuildManager) (Variables|/Game/Blueprints/BP_BuildManager.BP_BuildManager_C|GetCellUnderCursor (Variables|Default|GetBuildManager)) (Variables|Default|GetObjectSize) "ObjectTypeQuery3" 5e+03))
        (Variables|Default|SetHasUnitsInBuildArea _unitsfound)
        (if _unitsfound
          (Variables|Default|SetForceUpdatePlaceIndicators true)
          (for _array_element_2 _unitsincells
            (LocalVariables|SetIndexLOCAL (Utilities|Array|FindItem (Variables|Default|GetCellsForBuild) _array_element_2))
            (if (>= (LocalVariables|GetIndexLOCAL) 0)
              (Rendering|Material|SetMaterial (Utilities|Array|Get(acopy) (Variables|Default|GetPlaceIndicators) (LocalVariables|GetIndexLOCAL)) 0 (Variables|Default|GetPlaceRejectedMaterial)))))))))

(fn BuildObject
  (bind _buildmanager (Variables|Default|GetBuildManager))
  (bind _buildmanager_2 (Variables|Default|GetBuildManager))
  (bind _objectsize (Variables|Default|GetObjectSize))
  (bind _cellundercursor (Variables|/Game/Blueprints/BP_BuildManager.BP_BuildManager_C|GetCellUnderCursor _buildmanager_2))
  (bind _center (Default|GetCenterOfRectangularArea _buildmanager _cellundercursor _objectsize))
  (Variables|Default|SetForceUpdatePlaceIndicators true)
  (CallFunction|DrawPlacementIndicators) ; Final check construction area
  (if (and (Variables|Default|GetCanBuild) (not (and (Variables|Default|GetCheckUnitsInBuildArea) (Variables|Default|GetHasUnitsInBuildArea))))
    (Variables|Default|SetForceUpdatePlaceIndicators true)
    (bind _returnvalue (Game|SpawnActorfromClass (Variables|Default|GetNewPlaceableObjectClass) (Math|Transform|MakeTransform (Math|Vector|MakeVector (.x _center) (.y _center) (.z (Variables|/Game/Blueprints/BP_BuildManager.BP_BuildManager_C|GetLocationUnderCursor%28Camera%29 _buildmanager))) "0, 0, 0" "1.000000,1.000000,1.000000") "Undefined" "SelectDefaultAtRuntime" 0 (Variables|Default|GetcurrentLevel) (Variables|Default|GetbuildingComplete) (Variables|Default|GetspawnedTime) (Variables|Default|GetObjectNameInTable) (Utilities|Struct|MakeS_PlaceableObjects_Dynamic_Data true _buildmanager _cellundercursor (Variables|Default|GetBuildDirection)) 0))
    (bind _mesh (Default|GetBuildingProcedureMesh _returnvalue))
    (Components|StaticMesh|SetStaticMesh (Variables|/Game/Blueprints/GridBuildingOutdoor/BP_Grid_NewPlaceableObject.BP_Grid_NewPlaceableObject_C|GetStaticMesh _returnvalue) _mesh)
    ;[1 1 1] Set the UI mode back to normal
    (bind _foundwidgets (Widget|GetAllWidgetsOfClass "/Game/Blueprints/UI/WB_UI_Base_Main.WB_UI_Base_Main_C" true))
    (Utilities|IsValid (Utilities|Array|Get(acopy) _foundwidgets)
      (:Is%20Valid
        (Default|FSwitchtoGameMode (Utilities|Array|Get(acopy) _foundwidgets) "NewEnumerator0"))
      (:Is%20Not%20Valid))))