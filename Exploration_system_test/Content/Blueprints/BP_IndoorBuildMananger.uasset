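; BP_IndoorBuildMananger tracks which grid cells are occupied for indoor building, with separate data per layer.
; Each layer maps cells to reference counts, so overlapping placements increment the count and a cell frees only when its last occupant is removed.
; Occupancy queries report cells outside the buildable boundary as occupied, and a clear function empties every layer.
; The event graph holds only disabled default events.
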(event EventBeginPlay
  (|CallParentFunction) ; This node is disabled and will not be called.\nDrag off pins to build functionality.
)

(event Collision|EventActorBeginOverlap
  (params (OtherActor :type Actor%20Object%20Reference)))

(event EventTick
  (params (DeltaSeconds :type Float%20%28single-precision%29))
  (|CallParentFunction DeltaSeconds) ; This node is disabled and will not be called.\nDrag off pins to build functionality.
)

(fn ConstructionScript
  (|CallParentFunction))

(fn GetOccupancyDatabyLayer
  (params (Cell :type Int%20Point%20Structure) (layerIndex :type Integer))
  (bind _success (CallFunction|CheckCellinBuilableBoundary Cell))
  (if _success
    (return (.ReturnValue (Utilities|Map|Find (Utilities|Struct|BreakS_OccupancyData (Utilities|Array|Get(acopy) (Variables|Default|GetLayeredOccupancyData) layerIndex)) Cell)))
    (else
      (return true))))

(fn SetOccupancyDatabyLayer
  (params (cell :type Int%20Point%20Structure) (occupied :type Boolean) (layerIndex :type Integer))
  (bind _layeredoccupancydata (Variables|Default|GetLayeredOccupancyData))
  (bind _output (Utilities|Array|Get(acopy) _layeredoccupancydata layerIndex))
  (bind _pointmapint (Utilities|Struct|BreakS_OccupancyData _output))
  (bind (_value _returnvalue) (Utilities|Map|Find _pointmapint cell))
  (bind (_value_2 _returnvalue_2) (Utilities|Map|Find _pointmapint cell))
  (if occupied
    (if _returnvalue_2
      (Utilities|Map|Add _pointmapint cell (+ _value_2 1))
      (else
        (Utilities|Map|Add _pointmapint cell 1)))
    (elif _returnvalue
      (if (< _value 2)
        (Utilities|Map|Remove _pointmapint cell)
        (else
          (Utilities|Map|Add _pointmapint cell (- _value 1)))))))

(fn ClearOcuupancyData
  (for _array_element (Variables|Default|GetLayeredOccupancyData)
    (Utilities|Map|Clear (Utilities|Struct|BreakS_OccupancyData _array_element))))