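; Placer for the demo tower house that previews its footprint on the build grid and spawns the building.
; On Tick it moves the mesh and per-cell indicator planes to the cell under the cursor, refreshing when that cell changes or an update is forced.
; Cells need tower data, no occupancy and limited height difference; an optional unit check also marks cells rejected.
; BuildObject re-runs validation before spawning the placeable with its grid data.
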(event EventBeginPlay
  (bind _objectsize (Variables|Default|GetObjectSize))
  (bind _buildmanager (Variables|Default|GetBuildManager))
  (bind _gridcellsizexy (Variables|/Game/Blueprints/BP_BuildManager.BP_BuildManager_C|GetGridCellSizeXY _buildmanager))
  (bind _returnvalue (/ _gridcellsizexy 1.1e+02))
  (|CallParentFunction) ; Object Data setting here
  (for _index (range 0 (- (* (.x _objectsize) (.y _objectsize)) 1))
    (Variables|Default|SetForceUpdatePlaceIndicators true)
    (bind _staticmesh (CallFunction|GetReusableMesh (Variables|Default|GetPlaceIndicators) (Variables|Default|GetPlaceMeshUsingAmount) "/Game/Meshes/SM_Plane_100x100.SM_Plane_100x100" true))
    (Transformation|SetRelativeScale3D _staticmesh (Math|Vector|MakeVector _returnvalue _returnvalue 1.0))))

(event EventTick
  (params (DeltaSeconds :type Float%20%28single-precision%29))
  (CallFunction|DrawPlacementIndicators))

(fn ConstructionScript)

(fn RotateObjectPlacer
  (params (Left :type Boolean))
  (|CallParentFunction Left)
  (Variables|Default|SetForceUpdatePlaceIndicators true))

(fn DrawPlacementIndicators
  (bind _objectsize (Variables|Default|GetObjectSize))
  (bind _buildmanager (Variables|Default|GetBuildManager))
  (bind _cellundercursor (Variables|/Game/Blueprints/BP_BuildManager.BP_BuildManager_C|GetCellUnderCursor _buildmanager))
  (bind _center (Default|GetCenterOfRectangularArea _buildmanager _cellundercursor _objectsize))
  (Utilities|FlowControl|Sequence
    (:then_0
      (if (or (Variables|/Game/Blueprints/BP_BuildManager.BP_BuildManager_C|GetCellUnderCursorHasChanged (Variables|Default|GetBuildManager)) (Variables|Default|GetForceUpdatePlaceIndicators))
        (Variables|Default|SetForceUpdatePlaceIndicators false)
        (Variables|Default|SetCanBuild true)
        (bind _location (Default|GetCellLocation _buildmanager _cellundercursor))
        (LocalVariables|SetBaseBuildLevelLOCAL (.z _location))
        (Transformation|SetWorldLocation (Variables|Default|GetObectMesh) (Math|Vector|MakeVector (.x _center) (.y _center) (LocalVariables|GetBaseBuildLevelLOCAL)) false false)
        (bind _cells (Default|GetCellsinRectangularArea (Variables|Default|GetBuildManager) (Variables|/Game/Blueprints/BP_BuildManager.BP_BuildManager_C|GetCellUnderCursor (Variables|Default|GetBuildManager)) (Variables|Default|GetObjectSize)))
        (Variables|Default|SetCellsForBuild _cells)
        (for (_array_element _array_index) (Variables|Default|GetCellsForBuild)
          (bind (_location_2 _success) (Default|GetCellLocation (Variables|Default|GetBuildManager) _array_element))
          (LocalVariables|SetLocationLOCAL (Math|Vector|MakeVector (.x _location_2) (.y _location_2) (.z _location_2)))
          (Transformation|SetWorldLocation (Utilities|Array|Get(acopy) (Variables|Default|GetPlaceIndicators) _array_index) (LocalVariables|GetLocationLOCAL) false false)
          (if (Math|Boolean|ANDBoolean (not (Default|GetOccupancyData (Variables|Default|GetBuildManager) _array_element)) (Default|GetTowerData (Variables|Default|GetBuildManager) _array_element) _success (< (Math|Float|Absolute(Float) (- (.z _location_2) (LocalVariables|GetBaseBuildLevelLOCAL))) (Variables|Default|GetMaxHeightDifferenceForConstruction)))
            (Rendering|Material|SetMaterial (Utilities|Array|Get(acopy) (Variables|Default|GetPlaceIndicators) _array_index) 0 (Variables|Default|GetPlaceAcceptedMaterial))
            (else
              (Rendering|Material|SetMaterial (Utilities|Array|Get(acopy) (Variables|Default|GetPlaceIndicators) _array_index) 0 (Variables|Default|GetPlaceRejectedMaterial))
              (Variables|Default|SetCanBuild false))))))
    (:then_1
      (if (Variables|Default|GetCheckUnitsInBuildArea)
        (bind (_unitsfound _unitsincells) (Default|FindUnitsinRectangularArea (Variables|Default|GetBuildManager) (Variables|/Game/Blueprints/BP_BuildManager.BP_BuildManager_C|GetCellUnderCursor (Variables|Default|GetBuildManager)) (Variables|Default|GetObjectSize) "ObjectTypeQuery3" 5e+03))
        (Variables|Default|SetHasUnitsInBuildArea _unitsfound)
        (if _unitsfound
          (Variables|Default|SetForceUpdatePlaceIndicators true)
          (for _array_element_2 _unitsincells
            (LocalVariables|SetIndexLOCAL (Utilities|Array|FindItem (Variables|Default|GetCellsForBuild) _array_element_2))
            (if (>= (LocalVariables|GetIndexLOCAL) 0)
              (Rendering|Material|SetMaterial (Utilities|Array|Get(acopy) (Variables|Default|GetPlaceIndicators) (LocalVariables|GetIndexLOCAL)) 0 (Variables|Default|GetPlaceRejectedMaterial)))))))))

(fn BuildObject
  (bind _buildmanager (Variables|Default|GetBuildManager))
  (bind _buildmanager_2 (Variables|Default|GetBuildManager))
  (bind _objectsize (Variables|Default|GetObjectSize))
  (bind _cellundercursor (Variables|/Game/Blueprints/BP_BuildManager.BP_BuildManager_C|GetCellUnderCursor _buildmanager_2))
  (bind _center (Default|GetCenterOfRectangularArea _buildmanager _cellundercursor _objectsize))
  (Variables|Default|SetForceUpdatePlaceIndicators true)
  (CallFunction|DrawPlacementIndicators) ; Final check construction area
  (if (and (Variables|Default|GetCanBuild) (not (and (Variables|Default|GetCheckUnitsInBuildArea) (Variables|Default|GetHasUnitsInBuildArea))))
    (Variables|Default|SetForceUpdatePlaceIndicators true)
    (Game|SpawnActorfromClass (Variables|Default|GetPlaceableObjectClass) (Math|Transform|MakeTransform (Math|Vector|MakeVector (.x _center) (.y _center) (.z (Variables|/Game/Blueprints/BP_BuildManager.BP_BuildManager_C|GetLocationUnderCursor%28Camera%29 _buildmanager))) "0, 0, 0" "1.000000,1.000000,1.000000") "Undefined" "SelectDefaultAtRuntime" 0 (Variables|Default|GetObjectNameInTable) (Utilities|Struct|MakeS_PlaceableObjects_Dynamic_Data true _buildmanager _cellundercursor (Variables|Default|GetBuildDirection)) 0)))