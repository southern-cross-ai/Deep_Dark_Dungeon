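; Demo road placer for grid building that previews and spawns single road pieces or drag-built L-shaped lines.
; Tick switches between a cursor mesh and reused line indicators, choosing mesh and yaw from a BuildManager-calculated part index.
; Accept/reject feedback reflects cell validity, occupancy and resources, with an optional unit check on the cursor preview.
; BuildObject spawns on free cells, optionally avoiding units, and caps lines by the player's Stone.
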(event Custom|EventBuildStarted
  (params (NewState :type Boolean))
  (bind _buildmanager (Variables|Default|GetBuildManager))
  (if NewState
    (if (Variables|/Game/Blueprints/BP_BuildManager.BP_BuildManager_C|GetBuildToolEnabled _buildmanager)
      (Variables|Default|SetBuildStartCell (Variables|/Game/Blueprints/BP_BuildManager.BP_BuildManager_C|GetCellUnderCursor _buildmanager)))))

(event EventBeginPlay
  (|CallParentFunction) ; Object Data setting here
  (EventDispatchers|BindEventtoEventBuildStarted (Variables|Default|GetBuildManager) (delegate Custom|EventBuildStarted))
  (Variables|Default|SetForceUpdatePlaceIndicators true))

(event EventTick
  (params (DeltaSeconds :type Float%20%28single-precision%29))
  (CallFunction|UpdateDraggingState)
  (if (Variables|Default|GetDragStarted)
    (if (not (Variables|/Game/Blueprints/BP_BuildManager.BP_BuildManager_C|GetDragWasInterrupted (Variables|Default|GetBuildManager)))
      (CallFunction|DrawLineOfIndicators)
      (Variables|Default|SetForceUpdatePlaceIndicators true))
    (else
      (CallFunction|DrawCursorIndicator))))

(fn ConstructionScript)

(fn RotateObjectPlacer
  (params (Left :type Boolean)))

(fn BuildObject
  (if (Variables|Default|GetDragStarted)
    (if (not (Variables|/Game/Blueprints/BP_BuildManager.BP_BuildManager_C|GetDragWasInterrupted (Variables|Default|GetBuildManager)))
      (CallFunction|CreateLineOfObjects))
    (CallFunction|HIdePlaceIndicators)
    (else
      (CallFunction|CreateSingleObject))))

(fn UpdateDraggingState
  (bind _buildmanager (Variables|Default|GetBuildManager))
  (bind _drag_started (Variables|/Game/Blueprints/BP_BuildManager.BP_BuildManager_C|GetDrag%20Started _buildmanager))
  (if (Math|Boolean|NotEqual(Boolean) _drag_started (Variables|Default|GetDragStarted))
    (Variables|Default|SetDragStarted _drag_started)
    (if (Variables|Default|GetDragStarted)
      (Rendering|SetVisibility (Variables|Default|GetObectMesh) false false)
      (else
        (Rendering|SetVisibility (Variables|Default|GetObectMesh) true false)))))

(fn DrawCursorIndicator
  (bind _buildmanager (Variables|Default|GetBuildManager))
  (bind _cellundercursor (Variables|/Game/Blueprints/BP_BuildManager.BP_BuildManager_C|GetCellUnderCursor _buildmanager))
  (Utilities|FlowControl|Sequence
    (:then_0
      (if (or (Variables|/Game/Blueprints/BP_BuildManager.BP_BuildManager_C|GetCellUnderCursorHasChanged (Variables|Default|GetBuildManager)) (Variables|Default|GetForceUpdatePlaceIndicators))
        (CallFunction|HIdePlaceIndicators)
        (Variables|Default|SetForceUpdatePlaceIndicators false)
        (Variables|Default|SetCanBuild true)
        (bind (_location _success) (Default|GetCellLocation (Variables|Default|GetBuildManager) _cellundercursor))
        (Transformation|SetWorldLocation (Variables|Default|GetObectMesh) _location false false)
        (bind _partindex (Default|4CalculatePartIndexforObject (Variables|Default|GetBuildManager) _cellundercursor (Variables|Default|GetPlaceableObjectClass)))
        (Components|StaticMesh|SetStaticMesh (Variables|Default|GetObectMesh) (Utilities|Array|Get(acopy) (Variables|Default|GetWallMeshes) (Utilities|Array|Get(acopy) (Variables|Default|GetWallIndexes) _partindex)))
        (Transformation|SetWorldRotation (Variables|Default|GetObectMesh) (Math|Rotator|MakeRotator 0.0 0.0 (Utilities|Array|Get(acopy) (Variables|Default|GetWallAngles) _partindex)) false false)
        (if (and (not (Default|GetOccupancyData (Variables|Default|GetBuildManager) _cellundercursor)) _success)
          (if (Default|CheckifEnoughResources (Variables|Default|GetBuildManager) (Utilities|Struct|BreakS_PlaceableObjects_Data (Variables|Default|GetObjectData)))
            (Rendering|Material|SetMaterial (Variables|Default|GetObectMesh) 0 (Variables|Default|GetPlaceAcceptedMaterial))
            (else
              (Rendering|Material|SetMaterial (Variables|Default|GetObectMesh) 0 (Variables|Default|GetPlaceRejectedMaterial) :!label _label)
              (Variables|Default|SetCanBuild false)))
          (else
            (goto _label)))))
    (:then_1
      (if (Variables|Settings|GetCheckUnitsInBuildArea)
        (bind _unitsfound (Default|FindUnitsinRectangularArea (Variables|Default|GetBuildManager) (Variables|/Game/Blueprints/BP_BuildManager.BP_BuildManager_C|GetCellUnderCursor (Variables|Default|GetBuildManager)) (Utilities|Struct|MakeIntPoint 1 1) "ObjectTypeQuery3" 5e+03))
        (Variables|Default|SetHasUnitsInBuildArea _unitsfound)
        (if (Variables|Default|GetHasUnitsInBuildArea)
          (Variables|Default|SetForceUpdatePlaceIndicators true)
          (Rendering|Material|SetMaterial (Variables|Default|GetObectMesh) 0 (Variables|Default|GetPlaceRejectedMaterial)))))))

(fn DrawLineOfIndicators
  (LocalVariables|SetOneSegmentCostLOCAL (.Value (Utilities|Map|Find (Utilities|Struct|BreakS_ConstructionCost (Utilities|Struct|BreakS_PlaceableObjects_Data (Variables|Default|GetObjectData))) "Stone")))
  (LocalVariables|SetPlayerRecourceAmountLOCAL (.Value (Utilities|Map|Find (.resourcedatatable (Variables|/Game/Blueprints/BP_BuildManager.BP_BuildManager_C|GetPlayerResources (Variables|Default|GetBuildManager))) "Stone")))
  (CallFunction|HIdePlaceIndicators)
  (bind _pathcellnumbers (Default|FindLShapedWayonGrid (Variables|Default|GetBuildManager) (Variables|Default|GetBuildStartCell) (Variables|/Game/Blueprints/BP_BuildManager.BP_BuildManager_C|GetCellUnderCursor (Variables|Default|GetBuildManager))))
  (for _array_element _pathcellnumbers
    (Utilities|Map|Add (LocalVariables|GetGridLOCAL) _array_element false))
  (for _array_element_2 _pathcellnumbers
    (LocalVariables|SetCellLOCAL _array_element_2)
    (bind _partindex (Default|4CalculatePartIndexforPlacer (Variables|Default|GetBuildManager) (LocalVariables|GetGridLOCAL) (LocalVariables|GetCellLOCAL)))
    (LocalVariables|SetPartIndexLOCAL _partindex)
    (LocalVariables|SetMeshRotationLOCAL (Utilities|Array|Get(acopy) (Variables|Default|GetWallAngles) (LocalVariables|GetPartIndexLOCAL)))
    (LocalVariables|SetMeshLOCAL (Utilities|Array|Get(acopy) (Variables|Default|GetWallMeshes) (Utilities|Array|Get(acopy) (Variables|Default|GetWallIndexes) (LocalVariables|GetPartIndexLOCAL))))
    (if (>= (- (LocalVariables|GetPlayerRecourceAmountLOCAL) (+ (LocalVariables|GetCurrentCostLOCAL) (LocalVariables|GetOneSegmentCostLOCAL))) 0)
      (LocalVariables|SetFreePlaceLOCAL (not (Default|GetOccupancyData (Variables|Default|GetBuildManager) (LocalVariables|GetCellLOCAL))))
      (bind (_location _success) (Default|GetCellLocation (Variables|Default|GetBuildManager) (LocalVariables|GetCellLOCAL)))
      (bind _staticmesh (CallFunction|GetReusableMesh (Variables|Default|GetPlaceIndicators) (Variables|Default|GetPlaceMeshUsingAmount) (LocalVariables|GetMeshLOCAL) (and _success (LocalVariables|GetFreePlaceLOCAL))))
      (Components|StaticMesh|SetStaticMesh _staticmesh (LocalVariables|GetMeshLOCAL))
      (Transformation|SetWorldLocation _staticmesh _location false false)
      (Transformation|SetWorldRotation _staticmesh (Math|Rotator|MakeRotator 0.0 0.0 (LocalVariables|GetMeshRotationLOCAL)) false false)
      (if (LocalVariables|GetFreePlaceLOCAL)
        (LocalVariables|SetCurrentCostLOCAL (+ (LocalVariables|GetCurrentCostLOCAL) (LocalVariables|GetOneSegmentCostLOCAL))))
      (else
        (bind _location_2 (Default|GetCellLocation (Variables|Default|GetBuildManager) (LocalVariables|GetCellLOCAL)))
        (bind _staticmesh_2 (CallFunction|GetReusableMesh (Variables|Default|GetPlaceIndicators) (Variables|Default|GetPlaceMeshUsingAmount) (LocalVariables|GetMeshLOCAL) false))
        (Components|StaticMesh|SetStaticMesh _staticmesh_2 (LocalVariables|GetMeshLOCAL))
        (Transformation|SetWorldLocation _staticmesh_2 _location_2 false false)
        (Transformation|SetWorldRotation _staticmesh_2 (Math|Rotator|MakeRotator 0.0 0.0 (LocalVariables|GetMeshRotationLOCAL)) false false)))))

(fn CreateSingleObject
  (bind _buildmanager (Variables|Default|GetBuildManager))
  (bind _buildmanager_2 (Variables|Default|GetBuildManager))
  (bind _objectsize (Variables|Default|GetObjectSize))
  (bind _cellundercursor (Variables|/Game/Blueprints/BP_BuildManager.BP_BuildManager_C|GetCellUnderCursor _buildmanager_2))
  (bind _center (Default|GetCenterOfRectangularArea _buildmanager _cellundercursor _objectsize))
  (CallFunction|DrawCursorIndicator)
  (if (and (Variables|Default|GetCanBuild) (not (and (Variables|Settings|GetCheckUnitsInBuildArea) (Variables|Default|GetHasUnitsInBuildArea))))
    (Variables|Default|SetForceUpdatePlaceIndicators true)
    (Game|SpawnActorfromClass (Variables|Default|GetPlaceableObjectClass) (Math|Transform|MakeTransform (Math|Vector|MakeVector (.x _center) (.y _center) (.z (Variables|/Game/Blueprints/BP_BuildManager.BP_BuildManager_C|GetLocationUnderCursor%28Camera%29 _buildmanager))) "0, 0, 0" "1.000000,1.000000,1.000000") "Undefined" "SelectDefaultAtRuntime" 0 (Variables|Default|GetObjectNameInTable) (Utilities|Struct|MakeS_PlaceableObjects_Dynamic_Data true _buildmanager _cellundercursor (Variables|Default|GetBuildDirection)) 0)))

(fn CreateLineOfObjects
  (LocalVariables|SetOneSegmentCostLOCAL (.Value (Utilities|Map|Find (Utilities|Struct|BreakS_ConstructionCost (Utilities|Struct|BreakS_PlaceableObjects_Data (Variables|Default|GetObjectData))) "Stone")))
  (LocalVariables|SetPlayerRecourceAmountLOCAL (.Value (Utilities|Map|Find (.resourcedatatable (Variables|/Game/Blueprints/BP_BuildManager.BP_BuildManager_C|GetPlayerResources (Variables|Default|GetBuildManager))) "Stone")))
  (bind _pathcellnumbers (Default|FindLShapedWayonGrid (Variables|Default|GetBuildManager) (Variables|Default|GetBuildStartCell) (Variables|/Game/Blueprints/BP_BuildManager.BP_BuildManager_C|GetCellUnderCursor (Variables|Default|GetBuildManager))))
  (bind _array_element (Utilities|Array|ForEachLoopwithBreak _pathcellnumbers :!label _label)
    (:LoopBody
      (LocalVariables|SetCellLOCAL _array_element)
      (if (>= (- (LocalVariables|GetPlayerRecourceAmountLOCAL) (+ (LocalVariables|GetCurrentCostLOCAL) (LocalVariables|GetOneSegmentCostLOCAL))) 0)
        (if (not (Default|GetOccupancyData (Variables|Default|GetBuildManager) (LocalVariables|GetCellLOCAL)))
          (if (Variables|Settings|GetCheckUnitsInBuildArea)
            (bind _unitsfound (Default|FindUnitsinRectangularArea (Variables|Default|GetBuildManager) (LocalVariables|GetCellLOCAL) (Utilities|Struct|MakeIntPoint 1 1) "ObjectTypeQuery3" 5e+03))
            (if (not _unitsfound)
              (bind (_location _success) (Default|GetCellLocation (Variables|Default|GetBuildManager) (LocalVariables|GetCellLOCAL) :!label _label_2))
              (if _success
                (Game|SpawnActorfromClass (Variables|Default|GetPlaceableObjectClass) (Math|Transform|MakeTransform _location "0, 0, 0" "1.000000,1.000000,1.000000") "Undefined" "SelectDefaultAtRuntime" 0 (Variables|Default|GetObjectNameInTable) (Utilities|Struct|MakeS_PlaceableObjects_Dynamic_Data true (Variables|Default|GetBuildManager) (LocalVariables|GetCellLOCAL)) 0)
                (LocalVariables|SetCurrentCostLOCAL (+ (LocalVariables|GetCurrentCostLOCAL) (LocalVariables|GetOneSegmentCostLOCAL)))))
            (else
              (goto _label_2))))
        (else
          (goto _label Break))))))