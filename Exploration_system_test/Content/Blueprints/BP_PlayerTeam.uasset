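; Player team pawn that carries up to four heroes in child actor slots and arranges them in a formation.
; On BeginPlay, slot indices select Baird, Sorcerer or Witch classes, then BPTeamTool saves the team info if valid.
; It gathers the spawned heroes, clears all slots, then respawns them compacted into a layout based on hero count.
; HP and movement point bars show only when this is player 0's pawn.
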(event EventBeginPlay
  (bind _heroslot2 (Variables|Default|GetHeroSlot2))
  (bind _heroslot1 (Variables|Default|GetHeroSlot1))
  (bind _heroslot1_2 (Variables|Default|GetHeroSlot1))
  (bind _heroslot1_3 (Variables|Default|GetHeroSlot1))
  (bind _heroslot2_2 (Variables|Default|GetHeroSlot2))
  (bind _heroslot4 (Variables|Default|GetHeroSlot4))
  (bind _heroslot4_2 (Variables|Default|GetHeroSlot4))
  (bind _heroslot3 (Variables|Default|GetHeroSlot3))
  (bind _heroslot2_3 (Variables|Default|GetHeroSlot2))
  (CallFunction|SortHeroSlot)
  (CallFunction|InitializetheHPBarandMovementPointsBar)
  (CallFunction|InitTeamHeroArray)
  (ChildActorComponent|SetChildActorClass (Variables|Default|GetHeroSlot1) 0)
  (switch int (Variables|Default|GetHeroCount)
    (:1
      (ChildActorComponent|SetChildActorClass (Variables|Default|GetHeroSlot1) (Utilities|GetClass (Utilities|Array|Get(acopy) (Variables|Default|GetTeamHeroes))))
      (Transformation|SetRelativeLocation (Variables|Default|GetHeroSlot1) "0.000000,0.000000,-45.000000" false false))
    (:2
      (ChildActorComponent|SetChildActorClass _heroslot1 (Utilities|GetClass (Utilities|Array|Get(acopy) (Variables|Default|GetTeamHeroes))))
      (Transformation|SetRelativeLocation _heroslot1 "70.000000,0.000000,-45.000000" false false)
      (ChildActorComponent|SetChildActorClass _heroslot2 (Utilities|GetClass (Utilities|Array|Get(acopy) (Variables|Default|GetTeamHeroes) 1)))
      (Transformation|SetRelativeLocation _heroslot2 "-70.000000,0.000000,-45.000000" false false))
    (:3
      (ChildActorComponent|SetChildActorClass _heroslot1_2 (Utilities|GetClass (Utilities|Array|Get(acopy) (Variables|Default|GetTeamHeroes))))
      (Transformation|SetRelativeLocation _heroslot1_2 "54.000000,0.000000,-45.000000" false false)
      (ChildActorComponent|SetChildActorClass _heroslot2_2 (Utilities|GetClass (Utilities|Array|Get(acopy) (Variables|Default|GetTeamHeroes) 1)))
      (Transformation|SetRelativeLocation _heroslot2_2 "-16.000000,70.000000,-45.000000" false false)
      (ChildActorComponent|SetChildActorClass _heroslot4 (Utilities|GetClass (Utilities|Array|Get(acopy) (Variables|Default|GetTeamHeroes) 2)))
      (Transformation|SetRelativeLocation _heroslot4 "-16.000000,-70.000000,-45.000000" false false))
    (:4
      (ChildActorComponent|SetChildActorClass _heroslot1_3 (Utilities|GetClass (Utilities|Array|Get(acopy) (Variables|Default|GetTeamHeroes))))
      (Transformation|SetRelativeLocation _heroslot1_3 "70.000000,-50.000000,-45.000000" false false)
      (ChildActorComponent|SetChildActorClass _heroslot2_3 (Utilities|GetClass (Utilities|Array|Get(acopy) (Variables|Default|GetTeamHeroes) 1)))
      (Transformation|SetRelativeLocation _heroslot2_3 "30.000000,50.000000,-45.000000" false false)
      (ChildActorComponent|SetChildActorClass _heroslot3 (Utilities|GetClass (Utilities|Array|Get(acopy) (Variables|Default|GetTeamHeroes) 2)))
      (Transformation|SetRelativeLocation _heroslot3 "-30.000000,-50.000000,-45.000000" false false)
      (ChildActorComponent|SetChildActorClass _heroslot4_2 (Utilities|GetClass (Utilities|Array|Get(acopy) (Variables|Default|GetTeamHeroes) 3)))
      (Transformation|SetRelativeLocation _heroslot4_2 "-70.000000,50.000000,-45.000000" false false))))

(fn ConstructionScript)

(fn InitTeamHeroArray
  (bind _asbase_hero (Utilities|Casting|CastToBaseHero (Variables|/Script/Engine.ChildActorComponent|GetChildActor (Variables|Default|GetHeroSlot1)))
    (:then
      (Utilities|Array|Add (Variables|Default|GetTeamHeroes) _asbase_hero))
    (:CastFailed
      _))
  (bind _asbase_hero_2 (Utilities|Casting|CastToBaseHero (Variables|/Script/Engine.ChildActorComponent|GetChildActor (Variables|Default|GetHeroSlot2)))
    (:then
      (Utilities|Array|Add (Variables|Default|GetTeamHeroes) _asbase_hero_2))
    (:CastFailed
      _))
  (bind _asbase_hero_3 (Utilities|Casting|CastToBaseHero (Variables|/Script/Engine.ChildActorComponent|GetChildActor (Variables|Default|GetHeroSlot3)))
    (:then
      (Utilities|Array|Add (Variables|Default|GetTeamHeroes) _asbase_hero_3))
    (:CastFailed
      _))
  (bind _asbase_hero_4 (Utilities|Casting|CastToBaseHero (Variables|/Script/Engine.ChildActorComponent|GetChildActor (Variables|Default|GetHeroSlot4)))
    (:then
      (Utilities|Array|Add (Variables|Default|GetTeamHeroes) _asbase_hero_4))
    (:CastFailed
      _))
  (Variables|Default|SetHeroCount (Utilities|Array|Length (Variables|Default|GetTeamHeroes))))

(fn InitializetheHPBarandMovementPointsBar
  (bind _returnvalue (Game|Player|GetPlayerPawn 0))
  (bind _self self)
  (bind _returnvalue_2 (== _returnvalue _self))
  (Rendering|SetVisibility (Variables|Default|GetHPbar) _returnvalue_2 false)
  (Rendering|SetVisibility (Variables|Default|GetMovementPointBar) _returnvalue_2 false))

(fn InitialzeHeroSlot
  (params (HeroSlot :type Child%20Actor%20Component%20Object%20Reference) (Selection :type Integer))
  (switch int Selection
    (:0
      _)
    (:1
      (ChildActorComponent|SetChildActorClass HeroSlot "/Game/Blueprints/Heroes/BP_Baird.BP_Baird_C"))
    (:2
      (ChildActorComponent|SetChildActorClass HeroSlot "/Game/Blueprints/Heroes/BP_Sorcerer.BP_Sorcerer_C"))
    (:3
      (ChildActorComponent|SetChildActorClass HeroSlot "/Game/Blueprints/Heroes/BP_Witch.BP_Witch_C")))
  (Development|PrintString (Utilities|GetDisplayName HeroSlot)))

(fn SortHeroSlot
  (bind _bp_teamtool (Variables|Default|GetBP_TeamTool))
  (CallFunction|InitialzeHeroSlot (Variables|Default|GetHeroSlot1) (Variables|Default|GetHeroSlot1Index))
  (CallFunction|InitialzeHeroSlot (Variables|Default|GetHeroSlot2) (Variables|Default|GetHeroSlot2Index))
  (CallFunction|InitialzeHeroSlot (Variables|Default|GetHeroSlot3) (Variables|Default|GetHeroSlot3Index))
  (CallFunction|InitialzeHeroSlot (Variables|Default|GetHeroSlot4) (Variables|Default|GetHeroSlot4Index))
  (Utilities|IsValid _bp_teamtool
    (:Is%20Valid
      (Default|SaveTeamInfo _bp_teamtool))))