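; Base class for the building placement preview actor, with an empty BuildObject.
; On BeginPlay it finds BP_BuildManager, loads class, size and height limit from a data table row, and binds to resource updates.
; The preview mesh material shows whether construction is affordable; rotation turns it 90 degrees, swapping footprint axes and cycling build direction.
; Place indicator meshes are created on demand and reused, with accepted or rejected materials per free or blocked spot.
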(event Custom|UpdateResourceAmount
  (params (NewResourcesAmount :type S%20Construction%20Cost%20Structure))
  ;[0 0.5885 0.04905 0.1 16] If there are not enough resources to build, the building material will turn red
  (ParentFunctions|UpdateMeshMatDependingAmountOfResources))

(event EventBeginPlay
  (ParentFunctions|SetupObjectPlacer)
  ;[0 0.5885 0.04905 0.1 16] If there are not enough resources to build, the building material will turn red
  (EventDispatchers|BindEventtoEventUpdateResourceAmount (Variables|Default|GetBuildManager) (delegate Custom|UpdateResourceAmount))
  (ParentFunctions|UpdateMeshMatDependingAmountOfResources))

(fn ConstructionScript)

(fn SetupObjectPlacer
  (bind _objectnameintable (Variables|Settings|GetObjectNameInTable))
  (bind _returnvalue (Actor|GetActorOfClass "/Game/Blueprints/BP_BuildManager.BP_BuildManager_C"))
  (Variables|Default|SetBuildManager _returnvalue)
  (bind _returnvalue_2 (Utilities|GetDataTableRow (.datatable _objectnameintable) (.rowname _objectnameintable))
    (:then
      (Variables|Default|SetObjectData _returnvalue_2)
      (Variables|Default|SetPlaceableObjectClass (.PlaceableObjectClass (Utilities|Struct|BreakS_PlaceableObjects_Data (Variables|Default|GetObjectData))))
      (Variables|Default|SetObjectSize (Utilities|Struct|MakeIntPoint (Math|Integer|Clamp(Integer) (.X (Utilities|Struct|BreakIntPoint (.ObjectSize (Utilities|Struct|BreakS_PlaceableObjects_Data (Variables|Default|GetObjectData))))) 1 (.X (Utilities|Struct|BreakIntPoint (.ObjectSize (Utilities|Struct|BreakS_PlaceableObjects_Data (Variables|Default|GetObjectData)))))) (Math|Integer|Clamp(Integer) (.Y (Utilities|Struct|BreakIntPoint (.ObjectSize (Utilities|Struct|BreakS_PlaceableObjects_Data (Variables|Default|GetObjectData))))) 1 (.Y (Utilities|Struct|BreakIntPoint (.ObjectSize (Utilities|Struct|BreakS_PlaceableObjects_Data (Variables|Default|GetObjectData))))))))
      (Variables|Default|SetMaxHeightDifferenceForConstruction (.MaxHeightDifferenceForConstruction (Utilities|Struct|BreakS_PlaceableObjects_Data (Variables|Default|GetObjectData)))))))

(fn ActivateObjectPlacer
  (Actor|Tick|SetActorTickEnabled true)
  (Rendering|SetVisibility (Variables|Default|GetObectMesh) true true))

(fn DeactivateObjectPlacer
  (Actor|DestroyActor))

(fn BuildObject)

(fn RotateObjectPlacer
  (params (Left :type Boolean))
  (Variables|Default|SetObjectSize (Utilities|Struct|MakeIntPoint (.y (Variables|Default|GetObjectSize)) (.x (Variables|Default|GetObjectSize))))
  (Transformation|AddRelativeRotation (Variables|Default|GetObectMesh) (Math|Rotator|MakeRotator 0.0 0.0 (Math|Float|SelectFloat -9e+01 9e+01 Left)) false false)
  (Variables|Default|SetBuildDirection (Math|Integer|SelectInt 0 (Math|Integer|SelectInt 3 (+ (Math|Integer|SelectInt -1 1 Left) (Variables|Default|GetBuildDirection)) (< (+ (Math|Integer|SelectInt -1 1 Left) (Variables|Default|GetBuildDirection)) 0)) (> (+ (Math|Integer|SelectInt -1 1 Left) (Variables|Default|GetBuildDirection)) 3))))

(fn HIdePlaceIndicators
  (for _array_element (Variables|Default|GetPlaceIndicators)
    (Rendering|SetVisibility _array_element false false))
  (Variables|Default|SetPlaceMeshUsingAmount 0))

(fn GetReusableMesh
  (params (MeshesArray :type Array%20of%20Static%20Mesh%20Component%20Object%20References) (Index :type Integer%20%28by%20ref%29) (Mesh :type Static%20Mesh%20Object%20Reference) (FreePlace :type Boolean))
  (bind _placeacceptedmaterial (Variables|Settings|GetPlaceAcceptedMaterial))
  (bind _placerejectedmaterial (Variables|Settings|GetPlaceRejectedMaterial))
  (bind _returnvalue (select FreePlace _placeacceptedmaterial _placerejectedmaterial))
  (if (> (Utilities|Array|Length MeshesArray) Index)
    ;[0 0.2956 0.7448 0.1 16] Return already created mesh
    (Math|Integer|IncrementInt Index
      (:%20%20
        (LocalVariables|SetMeshLOCAL (Utilities|Array|Get(acopy) MeshesArray (- Index 1)))
        (if (!= (Rendering|Material|GetMaterial (LocalVariables|GetMeshLOCAL) 0) _returnvalue)
          (Rendering|Material|SetMaterial (LocalVariables|GetMeshLOCAL) 0 _returnvalue)
          (Rendering|SetVisibility (LocalVariables|GetMeshLOCAL) true false)
          (return (LocalVariables|GetMeshLOCAL))
          (else
            (Rendering|SetVisibility (LocalVariables|GetMeshLOCAL) true false)
            (return (LocalVariables|GetMeshLOCAL))))))
    (else
      ;[0 0.2956 0.7448 0.1 16] Create, setup and return new mesh
      (bind _returnvalue_2 (AddComponent|AddStaticMeshComponent false))
      (Utilities|Array|Add MeshesArray _returnvalue_2)
      (Components|StaticMesh|SetStaticMesh _returnvalue_2 Mesh)
      (Math|Integer|IncrementInt Index
        (:%20%20
          (Rendering|Material|SetMaterial _returnvalue_2 0 _returnvalue)
          (Rendering|SetVisibility _returnvalue_2 true false)
          (return _returnvalue_2))))))

(fn UpdateMeshMatDependingAmountOfResources
  (if (Default|CheckifEnoughResources (Variables|Default|GetBuildManager) (Utilities|Struct|MakeS_ConstructionCost (Utilities|Struct|BreakS_PlaceableObjects_Data (Variables|Default|GetObjectData))))
    (Rendering|Material|SetMaterial (Variables|Default|GetObectMesh) 0 (Variables|Settings|GetBuildingAcceptedMaterial))
    (else
      (Rendering|Material|SetMaterial (Variables|Default|GetObectMesh) 0 (Variables|Settings|GetBuildingRejectedMaterial)))))