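; BP_AttackN is an anim notify that adds impact feedback to attack animations in the turn-based JRPG combat.
; It plays a sound at the mesh owner's location for any owner.
; For player combat units only, it spawns a Niagara splash atop the battle controller's current target, offset by its bounds' half-height, and shakes the first player's camera.
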(fn ReceivedNotify
  (params (MeshComp :type Skeletal%20Mesh%20Component%20Object%20Reference) (Animation :type Anim%20Sequence%20Base%20Object%20Reference) (EventReference :type Anim%20Notify%20Event%20Reference%20Structure%20%28by%20ref%29))
  (bind _returnvalue (Components|GetOwner MeshComp))
  (Audio|PlaySoundatLocation "/Engine/EditorSounds/GamePreview/PossessPlayer.PossessPlayer" (.location (Transformation|GetActorTransform _returnvalue)) "0, 0, 0" 1.0 1.0 0.0 0 0 0 0)
  (bind _asbp_combat_player_unit_base (Utilities|Casting|CastToBP_CombatPlayerUnitBase _returnvalue))
  (Niagara|SpawnSystematLocation "/Game/Combat/Nigara/NS_Splash.NS_Splash" (Math|Vector|MakeVector (.x (Transformation|GetActorLocation (Variables|/Game/TurnBasedJRPGTemplate/Blueprints/Battle/BP_BattleController.BP_BattleController_C|GetcurrentTargetUnit (Variables|/Game/TurnBasedJRPGTemplate/Blueprints/Units/BP_UnitBase.BP_UnitBase_C|GetbattleController _asbp_combat_player_unit_base)))) (.y (Transformation|GetActorLocation (Variables|/Game/TurnBasedJRPGTemplate/Blueprints/Battle/BP_BattleController.BP_BattleController_C|GetcurrentTargetUnit (Variables|/Game/TurnBasedJRPGTemplate/Blueprints/Units/BP_UnitBase.BP_UnitBase_C|GetbattleController _asbp_combat_player_unit_base)))) (+ (.z (Transformation|GetActorLocation (Variables|/Game/TurnBasedJRPGTemplate/Blueprints/Battle/BP_BattleController.BP_BattleController_C|GetcurrentTargetUnit (Variables|/Game/TurnBasedJRPGTemplate/Blueprints/Units/BP_UnitBase.BP_UnitBase_C|GetbattleController _asbp_combat_player_unit_base)))) (.z (.BoxExtent (Collision|GetActorBounds (Variables|/Game/TurnBasedJRPGTemplate/Blueprints/Battle/BP_BattleController.BP_BattleController_C|GetcurrentTargetUnit (Variables|/Game/TurnBasedJRPGTemplate/Blueprints/Units/BP_UnitBase.BP_UnitBase_C|GetbattleController _asbp_combat_player_unit_base)) false false))))))
  (CameraShakes|StartCameraShake (Variables|/Script/Engine.PlayerController|GetPlayerCameraManager (Game|GetPlayerController 0)) "/Game/Combat/Blueprints/Skills/BP_AttackCameraShake.BP_AttackCameraShake_C" 1.0 "CameraLocal" "0, 0, 0")
  (return false))