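; Combat player controller that builds the player's party from saved game data and offers helpers for acting on units by battle position.
; The GameInstance's team save and UUID-to-class mapping fill the party list, which can be selection-sorted by saved Speed, highest first.
; Saved hero HP/MP seeds unit stats.
; Position helpers swap or slide enemies between spawn slots and route damage to the matching unit through BP_CombatController.
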(event EventBeginPlay
  (|CallParentFunction)
  (CallFunction|SetPartyMembersbyGameInstance))

(event EventTick
  (params (DeltaSeconds :type Float%20%28single-precision%29)))

(event EventSetUnitsStartingStats
  (bind _keys (Utilities|Map|Keys (Variables|Default|GetplayerUnits)))
  (for _array_element _keys
    (bind _asbp_shared_data_game_instance (Utilities|Casting|CastToBP_SharedDataGameInstance (Game|GetGameInstance)))
    (bind _asbp_combat_player_unit_base (Utilities|Casting|CastToBP_CombatPlayerUnitBaseClass _array_element))
    (bind _structout (Utilities|Struct|SetmembersinS_PlayerUnitData (.Value (Utilities|Map|Find (Variables|Default|GetplayerUnits) _asbp_combat_player_unit_base)) (.currentHP (Utilities|Struct|BreakS_CombatUnitData (.Value (Utilities|Map|Find (Variables|/Game/Combat/Blueprints/SaveGame/BP_CombatSaveGame_HeroData.BP_CombatSaveGame_HeroData_C|GetHeroData (Variables|/Game/Maps/BP_SharedDataGameInstance.BP_SharedDataGameInstance_C|GetHero%20Data%20SaveGame _asbp_shared_data_game_instance)) (.Value (Utilities|Map|Find (Variables|Default|GetParty%20Member%20UUIDs) _asbp_combat_player_unit_base)))))) (.currentMP (Utilities|Struct|BreakS_CombatUnitData (.Value (Utilities|Map|Find (Variables|/Game/Combat/Blueprints/SaveGame/BP_CombatSaveGame_HeroData.BP_CombatSaveGame_HeroData_C|GetHeroData (Variables|/Game/Maps/BP_SharedDataGameInstance.BP_SharedDataGameInstance_C|GetHero%20Data%20SaveGame _asbp_shared_data_game_instance)) (.Value (Utilities|Map|Find (Variables|Default|GetParty%20Member%20UUIDs) _asbp_combat_player_unit_base))))))))
    (Utilities|Map|Add (Variables|Default|GetplayerUnits) _asbp_combat_player_unit_base _structout)))

(fn ConstructionScript
  (|CallParentFunction)
  (bind _asbp_shared_data_game_instance (Utilities|Casting|CastToBP_SharedDataGameInstance (Game|GetGameInstance)))
  (Default|LoadHeroDatas _asbp_shared_data_game_instance))

(fn SortPartyMemberbySpeed
  (bind _partymembers (Variables|Default|GetpartyMembers))
  (bind _returnvalue (Utilities|Array|Length _partymembers))
  (bind _returnvalue_2 (- _returnvalue 1))
  (Utilities|FlowControl|Sequence
    (:then_0
      (for _array_element (Variables|Default|GetpartyMembers) :!label _label
        (Development|PrintString (Utilities|String|Append "B/A Swap           " (Utilities|GetClassDisplayName _array_element)) true true "(R=1.000000,G=0.396826,B=0.000000,A=1.000000)" 15.0))
      (Development|PrintString "============" true true "(R=1.000000,G=0.396826,B=0.000000,A=1.000000)" 15.0))
    (:then_1
      (bind _asbp_shared_data_game_instance (Utilities|Casting|CastToBP_SharedDataGameInstance (Game|GetGameInstance)))
      (LocalVariables|SetHero%20Data (Variables|/Game/Combat/Blueprints/SaveGame/BP_CombatSaveGame_HeroData.BP_CombatSaveGame_HeroData_C|GetHeroData (Variables|/Game/Maps/BP_SharedDataGameInstance.BP_SharedDataGameInstance_C|GetHero%20Data%20SaveGame _asbp_shared_data_game_instance)))
      (for _index (range 0 _returnvalue_2)
        (for _index_2 (range _index _returnvalue_2)
          (bind _asbp_combat_player_unit_base (Utilities|Casting|CastToBP_CombatPlayerUnitBaseClass (Utilities|Array|Get(acopy) (Variables|Default|GetpartyMembers) _index_2)))
          (if (>= (.Speed (Utilities|Struct|BreakS_CombatUnitData (.Value (Utilities|Map|Find (LocalVariables|GetHero%20Data) (.Value (Utilities|Map|Find (Variables|Default|GetParty%20Member%20UUIDs) _asbp_combat_player_unit_base)))))) (LocalVariables|GetmaxSpeed))
            (LocalVariables|SetmaxSpeed (.Speed (Utilities|Struct|BreakS_CombatUnitData (.Value (Utilities|Map|Find (LocalVariables|GetHero%20Data) (.Value (Utilities|Map|Find (Variables|Default|GetParty%20Member%20UUIDs) _asbp_combat_player_unit_base)))))))
            (LocalVariables|SetmaxIndex _index_2)))
        ;[1 1 1] swap(hero[max], hero[i]); reset maxSpeed, maxIndex
        (Utilities|Array|Swap (Variables|Default|GetpartyMembers) _index (LocalVariables|GetmaxIndex))
        (LocalVariables|SetmaxSpeed 0)
        (LocalVariables|SetmaxIndex -1)))
    (:then_2
      (goto _label))))

(fn SetPartyMembersbyGameInstance
  (bind _asbp_shared_data_game_instance (Utilities|Casting|CastToBP_SharedDataGameInstance (Game|GetGameInstance)))
  (Default|LoadTeamMembers _asbp_shared_data_game_instance)
  (Utilities|Map|Clear (Variables|Default|GetParty%20Member%20UUIDs))
  (Utilities|Array|Clear (Variables|Default|GetpartyMembers))
  (LocalVariables|SetgameInstance _asbp_shared_data_game_instance)
  (for _array_element (Variables|/Game/Combat/Blueprints/SaveGame/BP_CombatSaveGame_TeamMembers.BP_CombatSaveGame_TeamMembers_C|GetTeam%20Member%20UUID%20List (Variables|/Game/Maps/BP_SharedDataGameInstance.BP_SharedDataGameInstance_C|GetTeam%20Members%20SaveGame (LocalVariables|GetgameInstance)))
    (if (.ReturnValue (Utilities|Map|Find (Utilities|Struct|BreakS_CombatUnitMappingDatas (Variables|/Game/Maps/BP_SharedDataGameInstance.BP_SharedDataGameInstance_C|GetCombat%20Unit%20Mapping%20Datas (LocalVariables|GetgameInstance))) _array_element))
      (Utilities|Array|Add (Variables|Default|GetpartyMembers) (.class (Utilities|Struct|BreakS_CombatUnitData (.Value (Utilities|Map|Find (Utilities|Struct|BreakS_CombatUnitMappingDatas (Variables|/Game/Maps/BP_SharedDataGameInstance.BP_SharedDataGameInstance_C|GetCombat%20Unit%20Mapping%20Datas (LocalVariables|GetgameInstance))) _array_element)))))
      (Utilities|Map|Add (Variables|Default|GetParty%20Member%20UUIDs) (.class (Utilities|Struct|BreakS_CombatUnitData (.Value (Utilities|Map|Find (Utilities|Struct|BreakS_CombatUnitMappingDatas (Variables|/Game/Maps/BP_SharedDataGameInstance.BP_SharedDataGameInstance_C|GetCombat%20Unit%20Mapping%20Datas (LocalVariables|GetgameInstance))) _array_element)))) _array_element)
      (Development|PrintString (Utilities|String|Append "Add Player " (Utilities|GetClassDisplayName (.class (Utilities|Struct|BreakS_CombatUnitData (.Value (Utilities|Map|Find (Utilities|Struct|BreakS_CombatUnitMappingDatas (Variables|/Game/Maps/BP_SharedDataGameInstance.BP_SharedDataGameInstance_C|GetCombat%20Unit%20Mapping%20Datas (LocalVariables|GetgameInstance))) _array_element)))))) true true "(R=1.000000,G=0.542845,B=0.000000,A=1.000000)")
      (else
        (Class|AutomationBlueprintFunctionLibrary|AddExpectedLogError "No Mapping Data")))))

(fn SwapEnemyPosition
  (params (Source :type Integer) (Target :type Integer))
  (if (not (== Source Target))
    (Variables|Default|SetSwapSourceEnemy 0)
    (Variables|Default|SetSwapTargetEnemy 0)
    ;[1 1 1] Find Source and Target Enemy Unit
    (bind _array_element (Utilities|Array|ForEachLoopwithBreak (Variables|/Game/TurnBasedJRPGTemplate/Blueprints/Battle/BP_BattleBase.BP_BattleBase_C|GetenemyUnits (Variables|/Game/TurnBasedJRPGTemplate/Blueprints/Battle/BP_BattleController.BP_BattleController_C|GetcurrentBattle (CallFunction|GetBattleController))))
      (:LoopBody
        (bind _asbp_combat_enemy_unit_base (Utilities|Casting|CastToBP_CombatEnemyUnitBase _array_element))
        (Utilities|IsValid _asbp_combat_enemy_unit_base
          (:Is%20Valid
            (if (== (Variables|/Game/Combat/Blueprints/Unit/EnemyUnits/BP_CombatEnemyUnitBase.BP_CombatEnemyUnitBase_C|GetcurrentPosition _asbp_combat_enemy_unit_base) Source)
              (Variables|Default|SetSwapSourceEnemy _asbp_combat_enemy_unit_base)
              (elif (== (Variables|/Game/Combat/Blueprints/Unit/EnemyUnits/BP_CombatEnemyUnitBase.BP_CombatEnemyUnitBase_C|GetcurrentPosition _asbp_combat_enemy_unit_base) Target)
                (Variables|Default|SetSwapTargetEnemy _asbp_combat_enemy_unit_base))))))
      (:Completed
        (Utilities|IsValid (Variables|Default|GetSwapTargetEnemy)
          (:Is%20Valid
            (Default|SwapPositionwith (Variables|Default|GetSwapSourceEnemy) (Variables|Default|GetSwapTargetEnemy))
            (Development|PrintString (Utilities|String|Append (Utilities|String|Append (Utilities|String|Append (Utilities|String|Append "Enemy at position [" (Utilities|String|ToString(Integer) (Variables|/Game/Combat/Blueprints/Unit/EnemyUnits/BP_CombatEnemyUnitBase.BP_CombatEnemyUnitBase_C|GetcurrentPosition (Variables|Default|GetSwapSourceEnemy)))) "]  Swap with enemy at [") (Utilities|String|ToString(Integer) (Variables|/Game/Combat/Blueprints/Unit/EnemyUnits/BP_CombatEnemyUnitBase.BP_CombatEnemyUnitBase_C|GetcurrentPosition (Variables|Default|GetSwapTargetEnemy)))) "]")))
          (:Is%20Not%20Valid
            (Default|MovetoTargetwithRoot (Variables|Default|GetSwapSourceEnemy) (Transformation|GetActorLocation (Utilities|Array|Get(acopy) (Variables|/Game/TurnBasedJRPGTemplate/Blueprints/Battle/BP_BattleBase.BP_BattleBase_C|GetenemySpawnLocations (Variables|/Game/TurnBasedJRPGTemplate/Blueprints/Battle/BP_BattleController.BP_BattleController_C|GetcurrentBattle (Variables|Default|GetbattleController))) Target)) false 7e+02)
            (Variables|/Game/Combat/Blueprints/Unit/EnemyUnits/BP_CombatEnemyUnitBase.BP_CombatEnemyUnitBase_C|SetcurrentPosition (Variables|Default|GetSwapSourceEnemy) Target)))))))

(fn CallDealDamageto
  (params (pure%20Damage :type Integer) (damage%20Multiplier :type Float%20%28double-precision%29) (playerOrEnemy :type Boolean) (position :type Integer))
  (if playerOrEnemy
    (Development|PrintString "Target To Player" true true "(R=1.000000,G=0.000000,B=0.000000,A=1.000000)")
    (bind _returnvalue (Actor|GetActorOfClass "/Game/Combat/Blueprints/Battle/BP_CombatController.BP_CombatController_C"))
    (bind _array_element (Utilities|Array|ForEachLoopwithBreak (Variables|/Game/TurnBasedJRPGTemplate/Blueprints/Battle/BP_BattleBase.BP_BattleBase_C|GetplayerUnits (Variables|/Game/TurnBasedJRPGTemplate/Blueprints/Battle/BP_BattleController.BP_BattleController_C|GetcurrentBattle _returnvalue)) :!label _label)
      (:LoopBody
        (bind _asbp_combat_player_unit_base (Utilities|Casting|CastToBP_CombatPlayerUnitBase _array_element))
        (if (== (Variables|/Game/Combat/Blueprints/Unit/PlayerUnits/BP_CombatPlayerUnitBase.BP_CombatPlayerUnitBase_C|GetcurrentPosition _asbp_combat_player_unit_base) position)
          (Default|DealDamageto _returnvalue pure%20Damage damage%20Multiplier _asbp_combat_player_unit_base)
          (goto _label Break))))
    (else
      (Development|PrintString "Target To Enemy" true true "(R=1.000000,G=0.000000,B=0.000000,A=1.000000)")
      (bind _returnvalue_2 (Actor|GetActorOfClass "/Game/Combat/Blueprints/Battle/BP_CombatController.BP_CombatController_C"))
      (bind _array_element_2 (Utilities|Array|ForEachLoopwithBreak (Variables|/Game/TurnBasedJRPGTemplate/Blueprints/Battle/BP_BattleBase.BP_BattleBase_C|GetenemyUnits (Variables|/Game/TurnBasedJRPGTemplate/Blueprints/Battle/BP_BattleController.BP_BattleController_C|GetcurrentBattle _returnvalue_2)) :!label _label_2)
        (:LoopBody
          (bind _asbp_combat_enemy_unit_base (Utilities|Casting|CastToBP_CombatEnemyUnitBase _array_element_2))
          (if (== (Variables|/Game/Combat/Blueprints/Unit/EnemyUnits/BP_CombatEnemyUnitBase.BP_CombatEnemyUnitBase_C|GetcurrentPosition _asbp_combat_enemy_unit_base) position)
            (Default|DealDamageto _returnvalue_2 pure%20Damage damage%20Multiplier _asbp_combat_enemy_unit_base)
            (goto _label_2 Break)))))))