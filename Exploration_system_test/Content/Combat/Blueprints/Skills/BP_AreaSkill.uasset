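; BP_AreaSkill is a combat skill Blueprint that resolves a set of battlefield positions into the enemy units standing on them.
; AreaSkill compares each given position with the CurrentPosition of every enemy in the current battle, inserting matches at that position's index.
; GenerateArray supplies the index list for the enemy loop.
; The skill use, notify and animation-end events are empty, so no effect is applied here.
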(event EventUseSkillonNotify)

(event EventOnSkillAnimationEnded)

(event EventUseSkill)

(fn ConstructionScript
  (|CallParentFunction))

(fn AreaSkill
  (params (unitPositions :type Array%20of%20Integers))
  (bind _battlecontroller (Variables|Default|GetbattleController))
  (bind _currentbattle (Variables|/Game/TurnBasedJRPGTemplate/Blueprints/Battle/BP_BattleController.BP_BattleController_C|GetcurrentBattle _battlecontroller))
  (bind _enemyunits (Variables|/Game/TurnBasedJRPGTemplate/Blueprints/Battle/BP_BattleBase.BP_BattleBase_C|GetenemyUnits _currentbattle))
  (bind _returnarray (CallFunction|GenerateArray (Utilities|Array|LastIndex _enemyunits)))
  (for (_array_element _array_index) unitPositions
    (for _array_element_2 _returnarray
      (bind _asbp_combat_enemy_unit_base (Utilities|Casting|CastToBP_CombatEnemyUnitBase (Utilities|Array|Get(acopy) _enemyunits _array_element_2)))
      (if (== _array_element (Variables|/Game/Combat/Blueprints/Unit/EnemyUnits/BP_CombatEnemyUnitBase.BP_CombatEnemyUnitBase_C|GetcurrentPosition _asbp_combat_enemy_unit_base))
        (Utilities|Array|Insert (Variables|Default|GetOutput) _asbp_combat_enemy_unit_base _array_index))))
  (return (Variables|Default|GetOutput)))

(fn GenerateArray
  (params (ArrayLength :type Integer))
  (for _index (range 0 ArrayLength)
    (Utilities|Array|Add (Variables|Default|GetOutputArray) _index))
  (return (Variables|Default|GetOutputArray)))