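; Base Blueprint for combat buffs that last a number of turns on a target unit.
; Initialization copies the turn duration from the buff init data into DurationTurn.
; The apply, per-turn effect and end events only print debug messages naming the buff, target unit and turn counts.
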(event EventProcessTurnEffect
  (Development|PrintString (Utilities|String|Append (Utilities|GetObjectName self) "applied effect for 1 turn on unit :" (Utilities|GetObjectName (Variables|Default|GettargetUnit)) ". Turn left : " (Utilities|String|ToString(Integer) (Variables|Default|GetturnLeft)))))

(event EventApplyBuff
  (Development|PrintString (Utilities|String|Append (Utilities|GetObjectName self) " applied on target : " (Utilities|GetObjectName (Variables|Default|GettargetUnit)) " for " (Utilities|String|ToString(Integer) (Variables|Default|GetdurationTurn)) " turns.")))

(event EventOnBuffEnded
  (Development|PrintString (Utilities|String|Append (Utilities|GetObjectName self) " has been removed from unit : " (Utilities|GetObjectName (Variables|Default|GettargetUnit)))))

(fn ConstructionScript
  (|CallParentFunction))

(fn Initialization
  (params (buffInitData :type Buff%20Init%20Data%20Structure))
  (Variables|Default|SetdurationTurn (.turnDuration (Utilities|Struct|BreakBuffInitData buffInitData))))