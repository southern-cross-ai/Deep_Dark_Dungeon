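; Burn status effect for turn-based combat, a child combat buff that damages its target unit as each turn effect is processed.
; Initialization takes the damage from the buff init data, and turn processing passes it to the combat controller as pure damage with a zero multiplier.
; While active, it tints the unit's skeletal mesh through a LOD 0 vertex color override, which it clears when the buff ends.
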(event EventProcessTurnEffect
  (bind _targetunit (Variables|Default|GettargetUnit))
  (|CallParentFunction)
  ;[1 1 1] Apply Damage
  (bind _asbp_combat_controller (Utilities|Casting|CastToBP_CombatController (Variables|Default|GetbattleController)))
  (Default|DealDamageto _asbp_combat_controller (Variables|Default|Getdamage) 0.0 _targetunit)
  (Development|PrintString (Utilities|String|Append (Utilities|GetObjectName _targetunit) " is burned!")))

(event EventApplyBuff
  (bind _targetunit (Variables|Default|GettargetUnit))
  (|CallParentFunction)
  ;[1 1 1] 变成红色
  (Class|SkinnedMeshComponent|SetVertexColorOverrideLinearColor (Variables|/Game/TurnBasedJRPGTemplate/Blueprints/Units/BP_UnitBase.BP_UnitBase_C|GetSkeletalMesh _targetunit) 0 (Utilities|Array|MakeArray (Variables|Default|GetTargetTintColor)))
  (Development|PrintString (Utilities|String|Append "Burning Buff applied to unit " (Utilities|GetObjectName _targetunit))))

(event EventOnBuffEnded
  (|CallParentFunction)
  ;[1 1 1] 变回角色原有颜色
  (Class|SkinnedMeshComponent|ClearVertexColorOverride (Variables|/Game/TurnBasedJRPGTemplate/Blueprints/Units/BP_UnitBase.BP_UnitBase_C|GetSkeletalMesh (Variables|Default|GettargetUnit))))

(fn ConstructionScript
  (|CallParentFunction))

(fn Initialization
  (params (buffInitData :type Buff%20Init%20Data%20Structure))
  (|CallParentFunction buffInitData)
  (Variables|Default|Setdamage (.modifierdamage (Utilities|Struct|BreakBuffInitData buffInitData))))