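; Scorching Strike combat skill that damages the current target and applies a debuff, noted as armor-reducing, to that target whether or not the hit lands.
; Using it plays the skill animation and, for a Pyromaniac attacker, flags Pyro skill use in the shared-data GameInstance.
; The notify event deals multiplier-scaled damage through the BattleController, applies the debuff and sets the buff-applied flag.
; Animation end signals that the skill is used.
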(event EventUseSkill
  (CallFunction|PlaySkillAnimation)
  (bind _asbp_combat_player_unit_pyromaniac (Utilities|Casting|CastToBP_Combat_PlayerUnit_Pyromaniac (Variables|/Game/TurnBasedJRPGTemplate/Blueprints/Battle/BP_BattleController.BP_BattleController_C|GetcurrentAttackingUnit (Variables|Default|GetbattleController))))
  (Utilities|IsValid _asbp_combat_player_unit_pyromaniac
    (:Is%20Valid
      (bind _asbp_shared_data_game_instance (Utilities|Casting|CastToBP_SharedDataGameInstance (Game|GetGameInstance)))
      (Default|SetHasPyroUseSkill _asbp_shared_data_game_instance true))))

(event EventUseSkillonNotify
  (Default|DealDamage (Variables|Default|GetbattleController) 0 (Variables|Default|GetdamageMultiplier))
  ;[1 1 1] Hit or not, apply an armor reducing debuff to the user
  (CallFunction|ApplyBuffs (Utilities|Array|MakeArray (Variables|/Game/TurnBasedJRPGTemplate/Blueprints/Battle/BP_BattleController.BP_BattleController_C|GetcurrentTargetUnit (Variables|Default|GetbattleController))))
  (bind _asbp_shared_data_game_instance (Utilities|Casting|CastToBP_SharedDataGameInstance (Game|GetGameInstance)))
  (Default|SetIsBuffApplied _asbp_shared_data_game_instance true))

(event EventOnSkillAnimationEnded
  (Default|CallOnSkillUsed))

(fn ConstructionScript
  (|CallParentFunction))