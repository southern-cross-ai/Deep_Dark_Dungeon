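; Fanatical Charge is a combat skill that deals multiplied damage to its target and, hit or miss, applies an armor-reducing debuff to the attacker.
; On use it plays the skill animation and, when the attacker is a Zealot, flags the skill as used in the shared game instance.
; An animation notify triggers damage through the BattleController and the self-debuff, and the animation's end reports the skill as used.
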(event EventUseSkill
  (CallFunction|PlaySkillAnimation)
  (bind _asbp_combat_player_unit_zealot (Utilities|Casting|CastToBP_Combat_PlayerUnit_Zealot (Variables|/Game/TurnBasedJRPGTemplate/Blueprints/Battle/BP_BattleController.BP_BattleController_C|GetcurrentAttackingUnit (Variables|Default|GetbattleController))))
  (Utilities|IsValid _asbp_combat_player_unit_zealot
    (:Is%20Valid
      (bind _asbp_shared_data_game_instance (Utilities|Casting|CastToBP_SharedDataGameInstance (Game|GetGameInstance)))
      (Default|SetHasZealotUseSkill _asbp_shared_data_game_instance true))))

(event EventUseSkillonNotify
  (Default|DealDamage (Variables|Default|GetbattleController) 0 (Variables|Default|GetdamageMutiplier))
  ;[1 1 1] Hit or not, apply an armor reducing debuff to the user
  (CallFunction|ApplyBuffs (Utilities|Array|MakeArray (Variables|/Game/TurnBasedJRPGTemplate/Blueprints/Battle/BP_BattleController.BP_BattleController_C|GetcurrentAttackingUnit (Variables|Default|GetbattleController)))))

(event EventOnSkillAnimationEnded
  (Default|CallOnSkillUsed))

(fn ConstructionScript
  (|CallParentFunction))