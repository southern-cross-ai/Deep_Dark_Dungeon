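; Grip of the Dead combat skill that damages the current target and applies its buffs to that unit.
; Using the skill plays its animation, whose notify calls the BattleController to deal multiplier-based damage with no pure damage.
; Buffs are applied only if the damage call returns true, and the end of the animation signals that the skill has been used.
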(event EventUseSkill
  (CallFunction|PlaySkillAnimation))

(event EventUseSkillonNotify
  (bind _ishit (Default|DealDamage (Variables|Default|GetbattleController) 0 (Variables|Default|GetdamageMultiplier)))
  (if _ishit
    (CallFunction|ApplyBuffs (Utilities|Array|MakeArray (Variables|/Game/TurnBasedJRPGTemplate/Blueprints/Battle/BP_BattleController.BP_BattleController_C|GetcurrentTargetUnit (Variables|Default|GetbattleController))))))

(event EventOnSkillAnimationEnded
  (Default|CallOnSkillUsed))

(fn ConstructionScript
  (|CallParentFunction))