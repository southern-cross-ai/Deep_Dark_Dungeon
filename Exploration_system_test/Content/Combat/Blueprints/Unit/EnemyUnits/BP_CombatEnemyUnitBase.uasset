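; Base Blueprint for enemy combat units, handling animated movement and position swaps between enemies in battle.
; MoveToTargetWithRoot plays a forward or backward dash montage and lerps location on a timeline, with play rate scaled by speed over distance.
; On finish it returns to idle, fires OnMovedToTarget, then unbinds its listeners.
; SwapPositionWith exchanges slot indices, sending this unit to its new spawn point and the other to this unit's location.
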(event Custom|Move%20To%20Target%20With%20Root
  (params (targetLocation :type Vector) (isForward :type Boolean) (speed :type Float%20%28double-precision%29))
  ;[1 1 1] Move to target location
  (Variables|Default|SettargetLocation targetLocation)
  (Variables|Default|SetstartLocation (Transformation|GetActorLocation))
  (CallFunction|PlayAnimationMontage (select isForward (Variables|Default|GetdashForwardAnimation) (Variables|Default|GetdashBackwardAnimation)))
  (Components|Timeline|SetPlayRate (Variables|Default|GetMoveOverTime) (/ speed (Math|Vector|VectorLength (- (Variables|Default|GettargetLocation) (Variables|Default|GetstartLocation)))))
  (bind _alpha (Timeline|Timeline PlayFromStart)
    (:Update
      (Transformation|SetActorLocation (Math|Vector|Lerp(Vector) (Variables|Default|GetstartLocation) (Variables|Default|GettargetLocation) _alpha) false false))
    (:Finished
      (CallFunction|PlayAnimationMontage (Variables|Default|GetIdleAnimationMontage))
      (Default|CallOnMovedtoTarget)
      (EventDispatchers|UnbindallEventsfromOnMovedtoTarget))))

(fn ConstructionScript
  (|CallParentFunction))

(fn SwapPositionwith
  (params (toSwap :type BP%20Combat%20Enemy%20Unit%20Base%20Object%20Reference))
  (Utilities|FlowControl|Sequence
    (:then_0
      (LocalVariables|SetpositionTemp (Variables|BP_CombatEnemyUnitBase_C|GetcurrentPosition toSwap))
      (Variables|BP_CombatEnemyUnitBase_C|SetcurrentPosition toSwap (Variables|Default|GetcurrentPosition))
      (Variables|Default|SetcurrentPosition (LocalVariables|GetpositionTemp)))
    (:then_1
      (CallFunction|MovetoTargetwithRoot (Transformation|GetActorLocation (Utilities|Array|Get(acopy) (Variables|/Game/TurnBasedJRPGTemplate/Blueprints/Battle/BP_BattleBase.BP_BattleBase_C|GetenemySpawnLocations (Variables|/Game/TurnBasedJRPGTemplate/Blueprints/Battle/BP_BattleController.BP_BattleController_C|GetcurrentBattle (Variables|Default|GetbattleController))) (Variables|Default|GetcurrentPosition))) false 7e+02)
      (CallFunction|MovetoTargetwithRoot toSwap (Transformation|GetActorLocation) false 7e+02))))