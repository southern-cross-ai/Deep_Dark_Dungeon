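; Game instance that saves and restores placed grid-building objects through the "gridScene" save slot and keeps a background music player.
; Save records actors with configured tags as building data, handling indoor and regular grid objects separately.
; Load respawns them, relinks their build manager and runs their setup.
; Theme functions store layouts as indexed scenario slots keyed by level name, with functions to add or remove slots.
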(event Custom|Save
  (Utilities|FlowControl|Sequence
    (:then_0
      (Utilities|IsValid (Variables|Default|GetSaveGameInstance)
        (:Is%20Valid
          _)
        (:Is%20Not%20Valid
          (bind _returnvalue (SaveGame|CreateSaveGameObject "/Game/Data/BP_SaveGameData.BP_SaveGameData_C"))
          (Variables|Default|SetSaveGameInstance _returnvalue)))
      (CallFunction|SaveNewPlaceableObject)
      (SaveGame|SaveGametoSlot (Variables|Default|GetSaveGameInstance) "gridScene"))))

(event Custom|Load
  (Utilities|FlowControl|Sequence
    (:then_0
      (bind _returnvalue (SaveGame|DoesSaveGameExist "gridScene"))
      (if _returnvalue
        (bind _returnvalue_2 (SaveGame|LoadGamefromSlot "gridScene"))
        (bind _asbp_save_game_data (Utilities|Casting|CastToBP_SaveGameData _returnvalue_2))
        (Variables|Default|SetSaveGameInstance _asbp_save_game_data)
        (else
          (bind _returnvalue_3 (SaveGame|CreateSaveGameObject "/Game/Data/BP_SaveGameData.BP_SaveGameData_C"))
          (Variables|Default|SetSaveGameInstance _returnvalue_3)))
      (CallFunction|GenerateActors))))

(event Custom|SaveThemeData
  (params (storeArrayIndex :type Integer))
  (CallFunction|Save)
  (Utilities|FlowControl|Sequence
    (:then_0
      (Utilities|IsValid (Variables|Default|GetSaveGameInstance)
        (:Is%20Valid
          _)
        (:Is%20Not%20Valid
          (bind _returnvalue (SaveGame|CreateSaveGameObject "/Game/Data/BP_SaveGameData.BP_SaveGameData_C"))
          (Variables|Default|SetSaveGameInstance _returnvalue)))
      (CallFunction|StoreBuildingDataIntoThemeData storeArrayIndex)
      (SaveGame|SaveGametoSlot (Variables|Default|GetSaveGameInstance) "gridScene"))))

(event Custom|PlayBGM
  (params (Sound :type Sound%20Base%20Object%20Reference))
  ;[1 1 1] Play Background Music
  (Utilities|IsValid (Variables|Default|GetBGM)
    (:Is%20Valid
      (Audio|Components|Audio|SetSound (Variables|Default|GetBGM) Sound))
    (:Is%20Not%20Valid
      (bind _returnvalue (Audio|SpawnSound2D Sound 1.0 1.0 0.0 0 true))
      (Variables|Default|SetBGM _returnvalue))))

(event EventInit)

(fn SaveNewPlaceableObject
  (bind _output_get (Variables|/Game/Data/BP_SaveGameData.BP_SaveGameData_C|SetBuildingData (Variables|Default|GetSaveGameInstance) (Utilities|Array|MakeArray (Utilities|Struct|MakeS_SavedBuildingData 0 "0.000000,0.000000,0.000000|0.000000,0.000000,0.000000|1.000000,1.000000,1.000000"))))
  (bind _outactors (Actor|GetAllActorsOfClass "/Script/Engine.Actor"))
  (for _array_element _outactors
    ;[1 1 1] Add Mapping Tag Actors into SaveGameInstance
    (bind _bfounded (CallFunction|FoundMappingTag _array_element (Variables|Default|GetPlaceableObjectTagToSave)))
    (if _bfounded
      (bind _asbp_indoor_grid_new_placeable_object (Utilities|Casting|CastToBP_IndoorGrid_NewPlaceableObject _array_element :!pinned true) ; if its an indoor object then GO UP /// otherwise GO RIGHT
        (:then
          (Utilities|Array|Add _output_get (Utilities|Struct|MakeS_SavedBuildingData (Utilities|GetClass _array_element) (Transformation|GetActorTransform _array_element) (Math|Rotator|GetRotationXVector (Transformation|GetWorldRotation (Actor|GetComponentbyClass _array_element "/Script/Engine.StaticMeshComponent"))) (Variables|/Game/Blueprints/GridBuildingOutdoor/BP_Grid_NewPlaceableObject.BP_Grid_NewPlaceableObject_C|GetcurrentLevel _asbp_indoor_grid_new_placeable_object) (Variables|/Game/Blueprints/GridBuildingOutdoor/BP_Grid_NewPlaceableObject.BP_Grid_NewPlaceableObject_C|GetbuildingComplete _asbp_indoor_grid_new_placeable_object) (Variables|/Game/Blueprints/GridBuildingOutdoor/BP_Grid_NewPlaceableObject.BP_Grid_NewPlaceableObject_C|GetspawnedTime _asbp_indoor_grid_new_placeable_object) (Variables|/Game/Blueprints/BP_PlaceableObject_Base_Class.BP_PlaceableObject_Base_Class_C|GetObjectNameInTable _asbp_indoor_grid_new_placeable_object) (Variables|/Game/Blueprints/BP_PlaceableObject_Base_Class.BP_PlaceableObject_Base_Class_C|GetObjectSide _asbp_indoor_grid_new_placeable_object) (Variables|/Game/Blueprints/BP_PlaceableObject_Base_Class.BP_PlaceableObject_Base_Class_C|GetStartingHealthPercent _asbp_indoor_grid_new_placeable_object) (Variables|/Game/Blueprints/BP_PlaceableObject_Base_Class.BP_PlaceableObject_Base_Class_C|GetObjectDynamicData _asbp_indoor_grid_new_placeable_object) (Variables|/Game/Blueprints/GridBuildingIndoor/BP_IndoorGrid_NewPlaceableObject.BP_IndoorGrid_NewPlaceableObject_C|GetbuildingLayerIndex _asbp_indoor_grid_new_placeable_object))))
        (:CastFailed
          (bind _asbp_grid_new_placeable_object (Utilities|Casting|CastToBP_Grid_NewPlaceableObject _array_element)
            (:then
              (Utilities|Array|Add _output_get (Utilities|Struct|MakeS_SavedBuildingData (Utilities|GetClass _array_element) (Transformation|GetActorTransform _array_element) (Math|Rotator|GetRotationXVector (Transformation|GetWorldRotation (Actor|GetComponentbyClass _array_element "/Script/Engine.StaticMeshComponent"))) (Variables|/Game/Blueprints/GridBuildingOutdoor/BP_Grid_NewPlaceableObject.BP_Grid_NewPlaceableObject_C|GetcurrentLevel _asbp_grid_new_placeable_object) (Variables|/Game/Blueprints/GridBuildingOutdoor/BP_Grid_NewPlaceableObject.BP_Grid_NewPlaceableObject_C|GetbuildingComplete _asbp_grid_new_placeable_object) (Variables|/Game/Blueprints/GridBuildingOutdoor/BP_Grid_NewPlaceableObject.BP_Grid_NewPlaceableObject_C|GetspawnedTime _asbp_grid_new_placeable_object) (Variables|/Game/Blueprints/BP_PlaceableObject_Base_Class.BP_PlaceableObject_Base_Class_C|GetObjectNameInTable _asbp_grid_new_placeable_object) (Variables|/Game/Blueprints/BP_PlaceableObject_Base_Class.BP_PlaceableObject_Base_Class_C|GetObjectSide _asbp_grid_new_placeable_object) (Variables|/Game/Blueprints/BP_PlaceableObject_Base_Class.BP_PlaceableObject_Base_Class_C|GetStartingHealthPercent _asbp_grid_new_placeable_object) (Variables|/Game/Blueprints/BP_PlaceableObject_Base_Class.BP_PlaceableObject_Base_Class_C|GetObjectDynamicData _asbp_grid_new_placeable_object))))
            (:CastFailed
              (Development|PrintString "Failed to cast NewPlaceableObject")))))))
  (Development|PrintString (Utilities|String|Append "[GameInstance] Saved Objects Amount: " (Utilities|String|ToString(Integer) (Utilities|Array|Length _output_get))) true true "(R=0.000000,G=0.117245,B=1.000000,A=1.000000)"))

(fn FoundMappingTag
  (params (Actor :type Actor%20Object%20Reference) (Tags :type Array%20of%20Strings))
  (for _array_element Tags
    (if (Actor|ActorHasTag Actor (Utilities|String|StringToName _array_element))
      (return true)))
  (return false))

(fn GenerateActorsfromBuildngDatas
  (params (Array :type Array%20of%20S%20Saved%20Building%20Data%20Structures))
  ;[1 1 1] Generate Actors
  (for _array_element Array
    (bind _returnvalue (Game|SpawnActorfromClass (.ActorClass (Utilities|Struct|BreakS_SavedBuildingData _array_element)) (.ActorTransform (Utilities|Struct|BreakS_SavedBuildingData _array_element)) "Undefined" "MultiplyWithRoot" 0 0))
    (bind _asbp_indoor_grid_new_placeable_object (Utilities|Casting|CastToBP_IndoorGrid_NewPlaceableObject _returnvalue :!pinned true) ; if its an indoor object then GO UP /// otherwise GO DOWN
      (:then
        (Utilities|FlowControl|Sequence
          (:then_0
            (Transformation|SetWorldRotation (Actor|GetComponentbyClass _asbp_indoor_grid_new_placeable_object "/Script/Engine.StaticMeshComponent") (Math|Conversions|RotationFromXVector (.MeshRotation (Utilities|Struct|BreakS_SavedBuildingData _array_element))) false false))
          (:then_1
            (Variables|/Game/Blueprints/GridBuildingOutdoor/BP_Grid_NewPlaceableObject.BP_Grid_NewPlaceableObject_C|SetcurrentLevel _asbp_indoor_grid_new_placeable_object (.LevelData (Utilities|Struct|BreakS_SavedBuildingData _array_element))))
          (:then_2
            (Variables|/Game/Blueprints/GridBuildingOutdoor/BP_Grid_NewPlaceableObject.BP_Grid_NewPlaceableObject_C|SetbuildingComplete _asbp_indoor_grid_new_placeable_object (.bHasBeenBuilt (Utilities|Struct|BreakS_SavedBuildingData _array_element))))
          (:then_3
            (Variables|/Game/Blueprints/GridBuildingOutdoor/BP_Grid_NewPlaceableObject.BP_Grid_NewPlaceableObject_C|SetspawnedTime _asbp_indoor_grid_new_placeable_object (.SpawnedTime (Utilities|Struct|BreakS_SavedBuildingData _array_element))))
          (:then_4
            (Variables|/Game/Blueprints/BP_PlaceableObject_Base_Class.BP_PlaceableObject_Base_Class_C|SetObjectNameInTable _asbp_indoor_grid_new_placeable_object (.Component_ObjectNameInTable (Utilities|Struct|BreakS_SavedBuildingData _array_element))))
          (:then_5
            (Variables|/Game/Blueprints/BP_PlaceableObject_Base_Class.BP_PlaceableObject_Base_Class_C|SetObjectSide _asbp_indoor_grid_new_placeable_object (.Component_ObjectSide (Utilities|Struct|BreakS_SavedBuildingData _array_element))))
          (:then_6
            (Variables|/Game/Blueprints/BP_PlaceableObject_Base_Class.BP_PlaceableObject_Base_Class_C|SetStartingHealthPercent _asbp_indoor_grid_new_placeable_object (.Component_StartingHealthPercent (Utilities|Struct|BreakS_SavedBuildingData _array_element))))
          (:then_7
            (bind _returnvalue_2 (Actor|GetActorOfClass "/Game/Blueprints/BP_IndoorBuildMananger.BP_IndoorBuildMananger_C"))
            (Variables|/Game/Blueprints/BP_PlaceableObject_Base_Class.BP_PlaceableObject_Base_Class_C|SetObjectDynamicData _asbp_indoor_grid_new_placeable_object (Utilities|Struct|MakeS_PlaceableObjects_Dynamic_Data (.HasData (Utilities|Struct|BreakS_PlaceableObjects_Dynamic_Data (.Component_ObjectDynamicData (Utilities|Struct|BreakS_SavedBuildingData _array_element)))) _returnvalue_2 (.ObjectCenterCell (Utilities|Struct|BreakS_PlaceableObjects_Dynamic_Data (.Component_ObjectDynamicData (Utilities|Struct|BreakS_SavedBuildingData _array_element)))) (.DIrection (Utilities|Struct|BreakS_PlaceableObjects_Dynamic_Data (.Component_ObjectDynamicData (Utilities|Struct|BreakS_SavedBuildingData _array_element)))) (.Height (Utilities|Struct|BreakS_PlaceableObjects_Dynamic_Data (.Component_ObjectDynamicData (Utilities|Struct|BreakS_SavedBuildingData _array_element)))) (.Side (Utilities|Struct|BreakS_PlaceableObjects_Dynamic_Data (.Component_ObjectDynamicData (Utilities|Struct|BreakS_SavedBuildingData _array_element)))))))
          (:then_8
            (Variables|/Game/Blueprints/GridBuildingIndoor/BP_IndoorGrid_NewPlaceableObject.BP_IndoorGrid_NewPlaceableObject_C|SetbuildingLayerIndex _asbp_indoor_grid_new_placeable_object (.buildingLayer (Utilities|Struct|BreakS_SavedBuildingData _array_element))))
          (:then_9
            (Default|SetupPlaceableObject _asbp_indoor_grid_new_placeable_object))))
      (:CastFailed
        ;;[1 1 1] Set Actor Component Data
        (bind _asbp_grid_new_placeable_object (Utilities|Casting|CastToBP_Grid_NewPlaceableObject _returnvalue))
        (Utilities|FlowControl|Sequence
          (:then_0
            (Transformation|SetWorldRotation (Actor|GetComponentbyClass _asbp_grid_new_placeable_object "/Script/Engine.StaticMeshComponent") (Math|Conversions|RotationFromXVector (.MeshRotation (Utilities|Struct|BreakS_SavedBuildingData _array_element))) false false))
          (:then_1
            (Variables|/Game/Blueprints/GridBuildingOutdoor/BP_Grid_NewPlaceableObject.BP_Grid_NewPlaceableObject_C|SetcurrentLevel _asbp_grid_new_placeable_object (.LevelData (Utilities|Struct|BreakS_SavedBuildingData _array_element))))
          (:then_2
            (Variables|/Game/Blueprints/GridBuildingOutdoor/BP_Grid_NewPlaceableObject.BP_Grid_NewPlaceableObject_C|SetbuildingComplete _asbp_grid_new_placeable_object (.bHasBeenBuilt (Utilities|Struct|BreakS_SavedBuildingData _array_element))))
          (:then_3
            (Variables|/Game/Blueprints/GridBuildingOutdoor/BP_Grid_NewPlaceableObject.BP_Grid_NewPlaceableObject_C|SetspawnedTime _asbp_grid_new_placeable_object (.SpawnedTime (Utilities|Struct|BreakS_SavedBuildingData _array_element))))
          (:then_4
            (Variables|/Game/Blueprints/BP_PlaceableObject_Base_Class.BP_PlaceableObject_Base_Class_C|SetObjectNameInTable _asbp_grid_new_placeable_object (.Component_ObjectNameInTable (Utilities|Struct|BreakS_SavedBuildingData _array_element))))
          (:then_5
            (Variables|/Game/Blueprints/BP_PlaceableObject_Base_Class.BP_PlaceableObject_Base_Class_C|SetObjectSide _asbp_grid_new_placeable_object (.Component_ObjectSide (Utilities|Struct|BreakS_SavedBuildingData _array_element))))
          (:then_6
            (Variables|/Game/Blueprints/BP_PlaceableObject_Base_Class.BP_PlaceableObject_Base_Class_C|SetStartingHealthPercent _asbp_grid_new_placeable_object (.Component_StartingHealthPercent (Utilities|Struct|BreakS_SavedBuildingData _array_element))))
          (:then_7
            (bind _returnvalue_3 (Actor|GetActorOfClass "/Game/Blueprints/BP_BuildManager.BP_BuildManager_C"))
            (Variables|/Game/Blueprints/BP_PlaceableObject_Base_Class.BP_PlaceableObject_Base_Class_C|SetObjectDynamicData _asbp_grid_new_placeable_object (Utilities|Struct|MakeS_PlaceableObjects_Dynamic_Data (.HasData (Utilities|Struct|BreakS_PlaceableObjects_Dynamic_Data (.Component_ObjectDynamicData (Utilities|Struct|BreakS_SavedBuildingData _array_element)))) _returnvalue_3 (.ObjectCenterCell (Utilities|Struct|BreakS_PlaceableObjects_Dynamic_Data (.Component_ObjectDynamicData (Utilities|Struct|BreakS_SavedBuildingData _array_element)))) (.DIrection (Utilities|Struct|BreakS_PlaceableObjects_Dynamic_Data (.Component_ObjectDynamicData (Utilities|Struct|BreakS_SavedBuildingData _array_element)))) (.Height (Utilities|Struct|BreakS_PlaceableObjects_Dynamic_Data (.Component_ObjectDynamicData (Utilities|Struct|BreakS_SavedBuildingData _array_element)))) (.Side (Utilities|Struct|BreakS_PlaceableObjects_Dynamic_Data (.Component_ObjectDynamicData (Utilities|Struct|BreakS_SavedBuildingData _array_element)))))))
          (:then_9
            (Default|SetupPlaceableObject _asbp_grid_new_placeable_object)))))))

(fn GenerateActors
  (bind _savegameinstance (Variables|Default|GetSaveGameInstance))
  (bind _buildingdata (Variables|/Game/Data/BP_SaveGameData.BP_SaveGameData_C|GetBuildingData _savegameinstance))
  (Development|PrintString (Utilities|String|Append "[GameInstance] Try place buildings amount: " (Utilities|String|ToString(Integer) (Utilities|Array|Length _buildingdata))))
  (CallFunction|GenerateActorsfromBuildngDatas _buildingdata))

(fn ClearActorswithTag
  ;[1 1 1] Clear all actor with Tag
  (bind _outactors (Actor|GetAllActorsOfClass "/Script/Engine.Actor"))
  (for _array_element _outactors
    (bind _bfounded (CallFunction|FoundMappingTag _array_element (Variables|Default|GetPlaceableObjectTagToSave)))
    (if _bfounded
      (Actor|DestroyActor _array_element))))

(fn StoreBuildingDataIntoThemeData
  (params (arrayIndex :type Integer))
  (bind _s_savegamedata_array (Utilities|Struct|MakeS_SaveGameData_Array))
  (bind _savegameinstance (Variables|Default|GetSaveGameInstance))
  (bind _savegameinstance_2 (Variables|Default|GetSaveGameInstance))
  (bind _membervar_0 (Utilities|Struct|BreakS_SaveGameData_Array _s_savegamedata_array))
  (bind _indoorscenesscenariosdata (Variables|/Game/Data/BP_SaveGameData.BP_SaveGameData_C|GetIndoorScenesScenariosData _savegameinstance))
  (bind _buildingdata (Variables|/Game/Data/BP_SaveGameData.BP_SaveGameData_C|GetBuildingData _savegameinstance_2))
  (bind _s_savegamedata (Utilities|Struct|MakeS_SaveGameData _buildingdata))
  (bind _returnvalue (Game|GetCurrentLevelName true))
  (if (.ReturnValue (Utilities|Map|Find _indoorscenesscenariosdata _returnvalue)) ; if find mapping array [Set element]→ /// otherwise [create new array add to Map]↓
    (Utilities|Array|SetArrayElem (Utilities|Struct|BreakS_SaveGameData_Array (.Value (Utilities|Map|Find _indoorscenesscenariosdata _returnvalue))) arrayIndex _s_savegamedata true)
    (Utilities|Map|Add _indoorscenesscenariosdata _returnvalue (Utilities|Struct|MakeS_SaveGameData_Array (Utilities|Struct|BreakS_SaveGameData_Array (.Value (Utilities|Map|Find _indoorscenesscenariosdata _returnvalue)))))
    (else
      ;[1 1 1] Create New Array
      (Utilities|Array|SetArrayElem _membervar_0 arrayIndex _s_savegamedata true)
      (Utilities|Map|Add _indoorscenesscenariosdata _returnvalue (Utilities|Struct|MakeS_SaveGameData_Array _membervar_0)))))

(fn AddNewThemeDataSlot
  (bind _savegameinstance (Variables|Default|GetSaveGameInstance))
  (bind _indoorscenesscenariosdata (Variables|/Game/Data/BP_SaveGameData.BP_SaveGameData_C|GetIndoorScenesScenariosData _savegameinstance))
  (bind _returnvalue (Game|GetCurrentLevelName true))
  (if (.ReturnValue (Utilities|Map|Find _indoorscenesscenariosdata _returnvalue))
    (LocalVariables|SetTempSaveGameArray (Utilities|Struct|BreakS_SaveGameData_Array (.Value (Utilities|Map|Find _indoorscenesscenariosdata _returnvalue))))
    (bind _returnvalue_2 (Utilities|Array|Add :TargetArray (LocalVariables|GetTempSaveGameArray)))
    (Utilities|Map|Add (Variables|/Game/Data/BP_SaveGameData.BP_SaveGameData_C|GetIndoorScenesScenariosData (Variables|Default|GetSaveGameInstance)) _returnvalue (Utilities|Struct|MakeS_SaveGameData_Array (LocalVariables|GetTempSaveGameArray)))
    (Development|PrintString (Utilities|String|ToString(Integer) _returnvalue_2) true true "(R=0.000000,G=0.018010,B=1.000000,A=1.000000)")
    (SaveGame|SaveGametoSlot (Variables|Default|GetSaveGameInstance) "gridScene")
    (else
      (Utilities|Map|Add _indoorscenesscenariosdata _returnvalue (Utilities|Struct|MakeS_SaveGameData_Array (Utilities|Array|MakeArray (Utilities|Struct|MakeS_SaveGameData "(())")))))))

(fn RemoveLatestThemeDataSlot
  (bind _savegameinstance (Variables|Default|GetSaveGameInstance))
  (bind _indoorscenesscenariosdata (Variables|/Game/Data/BP_SaveGameData.BP_SaveGameData_C|GetIndoorScenesScenariosData _savegameinstance))
  (bind _returnvalue (Game|GetCurrentLevelName true))
  (if (.ReturnValue (Utilities|Map|Find _indoorscenesscenariosdata _returnvalue))
    (bind _output_get (LocalVariables|SetTempSaveGameArray (Utilities|Struct|BreakS_SaveGameData_Array (.Value (Utilities|Map|Find _indoorscenesscenariosdata _returnvalue)))))
    (Utilities|Array|RemoveIndex (LocalVariables|GetTempSaveGameArray) (- (Utilities|Array|Length _output_get) 1))
    (Utilities|Map|Add _indoorscenesscenariosdata _returnvalue (Utilities|Struct|MakeS_SaveGameData_Array (LocalVariables|GetTempSaveGameArray)))
    (Development|PrintString (Utilities|String|ToString(Integer) (- (Utilities|Array|Length _output_get) 1)) true true "(R=0.000000,G=0.018010,B=1.000000,A=1.000000)")
    (SaveGame|SaveGametoSlot (Variables|Default|GetSaveGameInstance) "gridScene")
    (else
      ;[1 1 1] Create Empty Array
      (Utilities|Map|Add _indoorscenesscenariosdata _returnvalue (Utilities|Struct|MakeS_SaveGameData_Array)))))