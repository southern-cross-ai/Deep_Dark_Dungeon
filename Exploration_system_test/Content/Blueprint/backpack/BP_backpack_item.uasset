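; BP_backpack_item is a backpack item actor whose properties and appearance come from a data table.
; The construction script looks up RowName in Data_item, stores the row as ItemProperty and applies its mesh to the StaticMesh component.
; The highlight event spawns a scaled-down BP_3D_Arrow_InScreen above the mesh, and undohighlight destroys it.
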(event Custom|undo%20high%20light
  (Actor|DestroyActor (Variables|Default|Gethighlight)))

(event Custom|high%20light
  (bind _returnvalue (Game|SpawnActorfromClass "/Game/Tutorial/Blueprints/BP_3D_Arrow_InScreen.BP_3D_Arrow_InScreen_C" (Math|Transform|MakeTransform (+ (+ (Transformation|GetActorLocation) (Variables|/Script/Engine.SceneComponent|GetRelativeLocation (Variables|Default|GetStaticMesh))) "0.000000,0.000000,60.000000") "0, 0, 0" "0.300000,0.300000,0.300000") "Undefined" "MultiplyWithRoot" 0 0))
  (Variables|Default|Sethighlight _returnvalue))

(event EventBeginPlay)

(event Collision|EventActorBeginOverlap
  (params (OtherActor :type Actor%20Object%20Reference)))

(event EventTick
  (params (DeltaSeconds :type Float%20%28single-precision%29)))

(fn ConstructionScript
  (bind _returnvalue (Utilities|GetDataTableRow "/Game/Blueprint/backpack/Data_item.Data_item" (Variables|Default|GetRow%20Name))
    (:then
      (Variables|Default|SetItem_Property _returnvalue))
    (:RowNotFound
      _))
  (Components|StaticMesh|SetStaticMesh (Variables|Default|GetStaticMesh) (.Item_mesh (Utilities|Struct|BreakS_item_properies (Variables|Default|GetItem_Property)))))