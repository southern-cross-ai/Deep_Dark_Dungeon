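; Backpack inventory component for the owning character, handling item pickup, stacking, dropping, swapping and number-key selection.
; Tick sphere-traces around the character to highlight a nearby BP_backpack_item, which F stores by stacking or filling an empty slot.
; G drops one item from slot CurrentIndex - 1, respawning it as a world actor.
; Pickups and drops refresh the WB_Dungeon backpack UI and save to BPCSave, loaded at BeginPlay.
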(event Custom|Init%20Backpack
  (for _index (range 0 (- (Variables|Default|Getbackpack_capacity) 1))
    (Utilities|Array|Add (Variables|Default|GetItems_in_backpack) (Variables|Default|Getempty_item))))

(event Custom|Pickup%20Item
  (bind _pickable_item (Variables|Default|GetPickable_Item))
  (Utilities|IsValid _pickable_item
    (:Is%20Valid
      (CallFunction|AddtoBackpack (Variables|/Game/Blueprint/backpack/BP_backpack_item.BP_backpack_item_C|GetItem_Property _pickable_item))
      (Default|RefreshBackpackUI (Variables|/Game/Blueprint/backpack/WB_Dungeon.WB_Dungeon_C|GetWB_backpack (Variables|Default|Getwidget)))
      (CallFunction|SaveBPC))))

(event Custom|delete%20item
  (params (item :type BP%20Backpack%20Item%20Object%20Reference))
  (Utilities|IsValid item
    (:Is%20Valid
      (Default|UndoHighLight item))
    (:Is%20Not%20Valid
      _))
  (Actor|DestroyActor item))

(event Custom|Giveup%20Item
  (params (Remove_Location :type Integer) (Remove_Quantity :type Integer))
  (CallFunction|RemoveItem Remove_Location Remove_Quantity)
  (Default|RefreshBackpackUI (Variables|/Game/Blueprint/backpack/WB_Dungeon.WB_Dungeon_C|GetWB_backpack (Variables|Default|Getwidget)))
  (CallFunction|SaveBPC))

(event Custom|Swap%20Items
  (params (FirstIndex :type Integer) (SecondIndex :type Integer))
  (Utilities|Array|Swap (Variables|Default|GetItems_in_backpack) FirstIndex SecondIndex))

(event Custom|Add%20to%20Backpack
  (params (New%20Item :type S%20Item%20Properies%20Structure))
  (bind (_item_id _item_name _item_quantity _item_description _item_img _item_stackable) (Utilities|Struct|BreakS_item_properies New%20Item))
  (bind _items_in_backpack (Variables|Default|GetItems_in_backpack))
  (bind _empty_item (Variables|Default|Getempty_item))
  (bind _returnvalue (Utilities|Array|FindItem _items_in_backpack _empty_item))
  (if _item_stackable
    (bind _array_index (Utilities|Array|ForEachLoopwithBreak (Variables|Default|GetItems_in_backpack) :!label _label)
      (:LoopBody
        (if (and (== (.item_id (Utilities|Struct|BreakS_item_properies (Utilities|Array|Get(acopy) (Variables|Default|GetItems_in_backpack) _array_index))) _item_id) (<= (+ (.Item_quantity (Utilities|Struct|BreakS_item_properies (Utilities|Array|Get(acopy) (Variables|Default|GetItems_in_backpack) _array_index))) _item_quantity) (.Item_max_stack (Utilities|Struct|BreakS_item_properies (Utilities|Array|Get(acopy) (Variables|Default|GetItems_in_backpack) _array_index)))))
          (Utilities|Struct|SetmembersinS_item_properies (Utilities|Array|Get(acopy) (Variables|Default|GetItems_in_backpack) _array_index) (+ (.Item_quantity (Utilities|Struct|BreakS_item_properies (Utilities|Array|Get(acopy) (Variables|Default|GetItems_in_backpack) _array_index))) _item_quantity))
          (Variables|Default|SetItem_found true)
          (CallFunction|DeleteItem (Variables|Default|GetPickable_Item))
          (goto _label Break)))
      (:Completed
        (if (Variables|Default|GetItem_found)
          (Variables|Default|SetItem_found false)
          (else
            (if (== _returnvalue -1) :!label _label_2
              (Development|PrintString "Backpack is full")
              (else
                (|SetBy-RefVar (Utilities|Array|Get(acopy) (Variables|Default|GetItems_in_backpack) _returnvalue) New%20Item)
                (Development|PrintString (Utilities|String|ToString(Integer) (.item_id (Utilities|Struct|BreakS_item_properies New%20Item))))
                (CallFunction|DeleteItem (Variables|Default|GetPickable_Item))))))))
    (else
      (goto _label_2))))

(event Custom|Remove%20Item
  (params (Remove_Location :type Integer) (Remove_Quantity :type Integer))
  (bind _items_in_backpack (Variables|Default|GetItems_in_backpack))
  (bind _output (Utilities|Array|Get(acopy) _items_in_backpack Remove_Location))
  (bind (_item_id _item_name _item_quantity _item_description _item_img _item_stackable _item_max_stack _item_type _item_mesh) (Utilities|Struct|BreakS_item_properies _output))
  (if (== (.Item_quantity (Utilities|Struct|BreakS_item_properies (Utilities|Array|Get(acopy) (Variables|Default|GetItems_in_backpack) Remove_Location))) 0)
    (Development|PrintString "no object")
    (elif (> Remove_Quantity 0)
      (if (>= Remove_Quantity _item_quantity)
        (CallFunction|SpawnItem _output)
        (|SetBy-RefVar _output (Variables|Default|Getempty_item))
        (Development|PrintString "removed")
        (else
          (Utilities|Struct|SetmembersinS_item_properies _output (- _item_quantity Remove_Quantity))
          (CallFunction|SpawnItem (Utilities|Struct|MakeS_item_properies _item_id _item_name Remove_Quantity _item_description _item_img _item_stackable _item_max_stack _item_type _item_mesh))
          (Development|PrintString "spawned"))))))

(event Custom|Spawn%20Item
  (params (Spawn_Item_Property :type S%20Item%20Properies%20Structure))
  (bind _as角色 (Variables|Default|GetAs角色))
  (Development|PrintString (Utilities|String|ToString(Integer) (.item_id (Utilities|Struct|BreakS_item_properies Spawn_Item_Property))))
  (Game|SpawnActorfromClass "/Game/Blueprint/backpack/BP_backpack_item.BP_backpack_item_C" (Math|Transform|MakeTransform (- (+ (Transformation|GetActorLocation _as角色) (* (Transformation|GetActorForwardVector _as角色) 6e+01)) "0.000000,0.000000,100.000000") "0, 0, 0" "1.000000,1.000000,1.000000") "Undefined" "MultiplyWithRoot" 0 "0" Spawn_Item_Property 0))

(event Custom|Set%20Current%20Item
  (Variables|Default|Setcurrent_item (Utilities|Array|Get(acopy) (Variables|Default|GetItems_in_backpack) (Variables|Default|Getcurrent_index)))
  (Default|RefreshBackpackUI (Variables|/Game/Blueprint/backpack/WB_Dungeon.WB_Dungeon_C|GetWB_backpack (Variables|Default|Getwidget))))

(event Custom|LoadBPC
  (bind _returnvalue (SaveGame|DoesSaveGameExist "BPCSave"))
  (if _returnvalue
    (bind _returnvalue_2 (SaveGame|LoadGamefromSlot "BPCSave"))
    (bind _asbp_bpcsave (Utilities|Casting|CastToBP_BPCSave _returnvalue_2))
    (Variables|Default|SetBPCSave _asbp_bpcsave)
    (Variables|Default|SetItems_in_backpack (Variables|/Game/Blueprint/backpack/BP_BPCSave.BP_BPCSave_C|GetItems%20in%20backpack (Variables|Default|GetBPCSave)) :!label _label)
    (Variables|Default|Setbackpack_capacity (Variables|/Game/Blueprint/backpack/BP_BPCSave.BP_BPCSave_C|Getbackpack%20capacity (Variables|Default|GetBPCSave)))
    (Default|RefreshBackpackUI (Variables|/Game/Blueprint/backpack/WB_Dungeon.WB_Dungeon_C|GetWB_backpack (Variables|Default|Getwidget)))
    (else
      (bind _returnvalue_3 (SaveGame|CreateSaveGameObject "/Game/Blueprint/backpack/BP_BPCSave.BP_BPCSave_C"))
      (Variables|Default|SetBPCSave _returnvalue_3)
      (Utilities|FlowControl|Sequence
        (:then_0
          (goto _label))
        (:then_1
          (CallFunction|InitBackpack)
          (Default|RefreshBackpackUI (Variables|/Game/Blueprint/backpack/WB_Dungeon.WB_Dungeon_C|GetWB_backpack (Variables|Default|Getwidget))))))))

(event Custom|SaveBPC
  (Utilities|IsValid (Variables|Default|GetBPCSave)
    (:Is%20Valid
      _)
    (:Is%20Not%20Valid
      (bind _returnvalue (SaveGame|CreateSaveGameObject "/Game/Blueprint/backpack/BP_BPCSave.BP_BPCSave_C"))
      (Variables|Default|SetBPCSave _returnvalue)))
  (Variables|/Game/Blueprint/backpack/BP_BPCSave.BP_BPCSave_C|SetItems%20in%20backpack (Variables|Default|GetBPCSave) (Variables|Default|GetItems_in_backpack))
  (Variables|/Game/Blueprint/backpack/BP_BPCSave.BP_BPCSave_C|Setbackpack%20capacity (Variables|Default|GetBPCSave) (Variables|Default|Getbackpack_capacity))
  (SaveGame|SaveGametoSlot (Variables|Default|GetBPCSave) "BPCSave"))

(event EventBeginPlay
  (Utilities|FlowControl|Sequence
    (:then_0
      (bind _as角色 (Utilities|Casting|CastToCharacter (Components|GetOwner)))
      (bind _output_get (Variables|Default|SetAs角色 _as角色))
      (bind _as玩家控制器 (Utilities|Casting|CastToPlayerController (Pawn|GetController _output_get)))
      (Variables|Default|SetAs玩家控制器 _as玩家控制器)
      (CallFunction|InitBackpack))
    (:then_1
      (bind _returnvalue (UserInterface|CreateWidget "/Game/Blueprint/backpack/WB_Dungeon.WB_Dungeon_C" (Variables|Default|GetAs玩家控制器)))
      (bind _output_get_2 (Variables|Default|Setwidget _returnvalue))
      (UserInterface|Viewport|AddtoViewport _output_get_2 0)
      (CallFunction|LoadBPC))))

(event EventTick
  (params (DeltaSeconds :type Float%20%28single-precision%29))
  (bind _as角色 (Variables|Default|GetAs角色))
  (bind _returnvalue (Transformation|GetActorLocation _as角色))
  (bind _outhit (Collision|SphereTraceForObjects _returnvalue (+ _returnvalue "1.000000,0.000000,0.000000") 1.5e+02 (Utilities|Array|MakeArray "ObjectTypeQuery2") false 0 "None"))
  (bind _asbp_backpack_item (Utilities|Casting|CastToBP_backpack_item (.HitActor (Collision|BreakHitResult _outhit))))
  (Utilities|IsValid (Variables|Default|GetPickable_Item)
    (:Is%20Valid
      (Default|UndoHighLight (Variables|Default|GetPickable_Item)))
    (:Is%20Not%20Valid
      _))
  (bind _output_get (Variables|Default|SetPickable_Item _asbp_backpack_item))
  (Default|HighLight _output_get))

(event Input|KeyboardEvents|F
  (params (Key :type Key%20Structure :default "None"))
  (:Pressed
    (CallFunction|PickupItem)))

(event Input|KeyboardEvents|G
  (params (Key :type Key%20Structure :default "None"))
  (:Pressed
    (CallFunction|GiveupItem (- (Variables|Default|Getcurrent_index) 1) 1)))

(event Input|KeyboardEvents|7
  (params (Key :type Key%20Structure :default "None"))
  (:Pressed
    (Variables|Default|Setcurrent_index 7)
    (CallFunction|SetCurrentItem)))

(event Input|KeyboardEvents|8
  (params (Key :type Key%20Structure :default "None"))
  (:Pressed
    (Variables|Default|Setcurrent_index 8)
    (CallFunction|SetCurrentItem)))

(event Input|KeyboardEvents|9
  (params (Key :type Key%20Structure :default "None"))
  (:Pressed
    (Variables|Default|Setcurrent_index 9)
    (CallFunction|SetCurrentItem)))

(event Input|KeyboardEvents|0
  (params (Key :type Key%20Structure :default "None"))
  (:Pressed
    (Variables|Default|Setcurrent_index 0)
    (CallFunction|SetCurrentItem)))

(event Input|KeyboardEvents|1
  (params (Key :type Key%20Structure :default "None"))
  (:Pressed
    (Variables|Default|Setcurrent_index 1)
    (CallFunction|SetCurrentItem)))

(event Input|KeyboardEvents|2
  (params (Key :type Key%20Structure :default "None"))
  (:Pressed
    (Variables|Default|Setcurrent_index 2)
    (CallFunction|SetCurrentItem)))

(event Input|KeyboardEvents|3
  (params (Key :type Key%20Structure :default "None"))
  (:Pressed
    (Variables|Default|Setcurrent_index 3)
    (CallFunction|SetCurrentItem)))

(event Input|KeyboardEvents|4
  (params (Key :type Key%20Structure :default "None"))
  (:Pressed
    (Variables|Default|Setcurrent_index 4)
    (CallFunction|SetCurrentItem)))

(event Input|KeyboardEvents|5
  (params (Key :type Key%20Structure :default "None"))
  (:Pressed
    (Variables|Default|Setcurrent_index 5)
    (CallFunction|SetCurrentItem)))

(event Input|KeyboardEvents|6
  (params (Key :type Key%20Structure :default "None"))
  (:Pressed
    (Variables|Default|Setcurrent_index 6)
    (CallFunction|SetCurrentItem)))