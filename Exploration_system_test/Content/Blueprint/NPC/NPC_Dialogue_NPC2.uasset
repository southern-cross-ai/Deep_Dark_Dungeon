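; NPC dialogue Blueprint for a dungeon guard who warns the player about a dark power deeper in the tunnels.
; It overrides Dialogue, calls the parent, then switches on DialogueTreeIndex, which has a single tree.
; Nested AddDialogue calls branch on the chosen option, and each ending clears progress and closes the conversation.
; The monster challenge, relic hint and sword reward exist only as text, with no quest or reward logic.
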(event EventBeginPlay
  (|CallParentFunction) ; 此节点被禁用，将不会被调用。\n从引脚连出引线来编译功能。
)

(event EventTick
  (params (DeltaSeconds :type Float%20%28single-precision%29))
  (|CallParentFunction DeltaSeconds) ; 此节点被禁用，将不会被调用。\n从引脚连出引线来编译功能。
)

(fn Dialogue
  (|CallParentFunction)
  (switch int (Variables|Default|GetDialogueTreeIndex)
    (:0
      (bind (_state _optionindex) (CallFunction|AddDialogue (Variables|Default|GetspeakerName) "Halt! Who goes there? Ah, a fellow adventurer... I’ve been stationed here to keep an eye on these cursed tunnels. It's not safe beyond this point." (Utilities|Array|MakeArray "Why are you here? What’s so dangerous about this place?" "I can handle myself. Step aside." "Maybe you’re right. I should turn back.")))
      (switch Utilities|FlowControl|Switch|SwitchonEnum_DialogueState _state
        (:NewEnumerator0
          (switch int _optionindex
            (:0
              (bind (_state_2 _optionindex_2) (CallFunction|AddDialogue (Variables|Default|GetspeakerName) "I’m here under orders from the King. Reports say a dark power has taken root deeper in the dungeon. Many have ventured in; few have returned. My job is to warn travelers like you." (Utilities|Array|MakeArray "Tell me more about this dark power." "What’s in it for you if I clear this dungeon?")))
              (switch Utilities|FlowControl|Switch|SwitchonEnum_DialogueState _state_2
                (:NewEnumerator0
                  (switch int _optionindex_2
                    (:0
                      (bind (_state_3 _optionindex_3) (CallFunction|AddDialogue (Variables|Default|GetspeakerName) "It’s a sorcerer, or so they say. His minions guard every passage, and traps lie around every corner. But he fears something... A relic hidden deep within. If you seek to defeat him, finding that relic is your best chance." (Utilities|Array|MakeArray "Thanks for the tip. I’ll find the relic and defeat him." "Sounds like too much trouble. I’ll pass.")))
                      (switch Utilities|FlowControl|Switch|SwitchonEnum_DialogueState _state_3
                        (:NewEnumerator0
                          (switch int _optionindex_3
                            (:0
                              _)
                            (:1
                              _))
                          (CallFunction|ClearDialogueProgress)
                          (CallFunction|CloseConversation))))
                    (:1
                      (bind (_state_4 _optionindex_4) (CallFunction|AddDialogue (Variables|Default|GetspeakerName) "If you can defeat the dark power, I’ll reward you with an enchanted sword, one that can pierce even the strongest armor. It’s a weapon worthy of a hero, and it’s yours if you help." (Utilities|Array|MakeArray "Deal. I’ll clear this dungeon for you." "An enchanted sword? Not interested.")))
                      (switch Utilities|FlowControl|Switch|SwitchonEnum_DialogueState _state_4
                        (:NewEnumerator0
                          (switch int _optionindex_4
                            (:0
                              _)
                            (:1
                              _))
                          (CallFunction|ClearDialogueProgress)
                          (CallFunction|CloseConversation))))))))
            (:1
              (bind (_state_5 _optionindex_5) (CallFunction|AddDialogue (Variables|Default|GetspeakerName) "Bold words! But bravery alone won't save you. If you truly wish to pass, prove your strength. Defeat the monster lurking in the chamber to the right, and I’ll let you through." (Utilities|Array|MakeArray "Fine, I’ll defeat the monster." "I don't need your permission to pass.")))
              (switch Utilities|FlowControl|Switch|SwitchonEnum_DialogueState _state_5
                (:NewEnumerator0
                  (switch int _optionindex_5
                    (:0
                      (bind _state_6 (CallFunction|AddDialogue (Variables|Default|GetspeakerName) "Good luck, then. The beast is a fierce one, but I have faith in you. Return here when you have proof of its defeat." (Utilities|Array|MakeArray "Leave")))
                      (switch Utilities|FlowControl|Switch|SwitchonEnum_DialogueState _state_6
                        (:NewEnumerator0
                          (CallFunction|ClearDialogueProgress)
                          (CallFunction|CloseConversation))))
                    (:1
                      (bind _state_7 (CallFunction|AddDialogue (Variables|Default|GetspeakerName) "Foolish! You might find more than you bargained for. Don’t say I didn’t warn you." (Utilities|Array|MakeArray "Leave")))
                      (switch Utilities|FlowControl|Switch|SwitchonEnum_DialogueState _state_7
                        (:NewEnumerator0
                          (CallFunction|ClearDialogueProgress)
                          (CallFunction|CloseConversation))))))))
            (:2
              (bind _state_8 (CallFunction|AddDialogue (Variables|Default|GetspeakerName) "A wise choice. There’s no shame in knowing when to retreat. Better to live and fight another day." (Utilities|Array|MakeArray "Leave")))
              (switch Utilities|FlowControl|Switch|SwitchonEnum_DialogueState _state_8
                (:NewEnumerator0
                  (CallFunction|ClearDialogueProgress)
                  (CallFunction|CloseConversation))))))))))