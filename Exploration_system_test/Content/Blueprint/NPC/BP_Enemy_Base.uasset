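; BP_Enemy_Base is a base enemy NPC with a name label and a proximity sphere for combat.
; The construction script fills the CharacterName text from CharacterNameTxt.
; TargetSphere overlaps set CanFight on BP_TopDownCharacter, true on entry and false on exit.
; ConversationClosed notifies InteractInstigator, and SetInteractableState always shows the name because its branch condition is constant true.
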(event OnComponentBeginOverlap(TargetSphere)
  (params (OverlappedComponent :type Primitive%20Component%20Object%20Reference) (OtherActor :type Actor%20Object%20Reference) (OtherComp :type Primitive%20Component%20Object%20Reference) (OtherBodyIndex :type Integer) (bFromSweep :type Boolean) (SweepResult :type Hit%20Result%20Structure%20%28by%20ref%29))
  (bind _asbp_top_down_character (Utilities|Casting|CastToBP_TopDownCharacter OtherActor))
  (Variables|/Game/TopDown/Blueprints/BP_TopDownCharacter.BP_TopDownCharacter_C|SetCanFight _asbp_top_down_character true))

(event OnComponentEndOverlap(TargetSphere)
  (params (OverlappedComponent :type Primitive%20Component%20Object%20Reference) (OtherActor :type Actor%20Object%20Reference) (OtherComp :type Primitive%20Component%20Object%20Reference) (OtherBodyIndex :type Integer))
  (bind _asbp_top_down_character (Utilities|Casting|CastToBP_TopDownCharacter OtherActor))
  (Variables|/Game/TopDown/Blueprints/BP_TopDownCharacter.BP_TopDownCharacter_C|SetCanFight _asbp_top_down_character false))

(event EventBeginPlay)

(event Collision|EventActorBeginOverlap
  (params (OtherActor :type Actor%20Object%20Reference)))

(event EventTick
  (params (DeltaSeconds :type Float%20%28single-precision%29)))

(event EventSetInteractableState
  (params (CanShowInteract? :type Boolean))
  (if true
    (Rendering|SetVisibility (Variables|Default|GetCharacterName) true false)
    (else
      (Rendering|SetVisibility (Variables|Default|GetCharacterName) false false))))

(event EventConversationClosed
  (Class|NPCInteractable|ConversationClosed(Message) (Variables|Default|GetInteractInstigator)))

(fn ConstructionScript
  (Rendering|Components|TextRender|SetText (Variables|Default|GetCharacterName) (Variables|Default|GetCharacterNameTxt)))