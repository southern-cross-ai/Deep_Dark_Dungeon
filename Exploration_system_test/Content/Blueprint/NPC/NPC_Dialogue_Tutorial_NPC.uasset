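; Tutorial NPC dialogue Blueprint for a wounded former guardian who warns the player about the trial of the sigils.
; It overrides the parent Dialogue function, switching on DialogueTreeIndex, with only the first tree defined.
; An opening four-option prompt branches through AddDialogue's Pass Through state and option index into short replies.
; Every branch ends by clearing dialogue progress and closing the conversation.
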(event EventBeginPlay
  (|CallParentFunction) ; 此节点被禁用，将不会被调用。\n从引脚连出引线来编译功能。
)

(event EventTick
  (params (DeltaSeconds :type Float%20%28single-precision%29))
  (|CallParentFunction DeltaSeconds) ; 此节点被禁用，将不会被调用。\n从引脚连出引线来编译功能。
)

(fn Dialogue
  (|CallParentFunction)
  (switch int (Variables|Default|GetDialogueTreeIndex)
    (:0
      (bind (_state _optionindex) (CallFunction|AddDialogue (Variables|Default|GetspeakerName) "...Another soul come to brave the depths. Hmph. 
" (Utilities|Array|MakeArray "What is this place?" "Are you a guardian?" "You look injured. Should I help you?" "...You sure talk a lot for a dead man.")))
      (switch Utilities|FlowControl|Switch|SwitchonEnum_DialogueState _state
        (:NewEnumerator0
          (switch int _optionindex
            (:0
              (bind _state_2 (CallFunction|AddDialogue (Variables|Default|GetspeakerName) "A prison, once. A tomb, later. Now? A trial. 
Only those who pass the trial of the sigils may go deeper." (Utilities|Array|MakeArray "Fine, I’ll find them.")))
              (switch Utilities|FlowControl|Switch|SwitchonEnum_DialogueState _state_2
                (:NewEnumerator0
                  (CallFunction|ClearDialogueProgress)
                  (CallFunction|CloseConversation))))
            (:1
              (bind _state_3 (CallFunction|AddDialogue (Variables|Default|GetspeakerName) "Once. I stood proud at the Gate of the Fifth Watch. 
Now... I am but a remnant. But my duty is not yet done." (Utilities|Array|MakeArray "Then help me.")))
              (switch Utilities|FlowControl|Switch|SwitchonEnum_DialogueState _state_3
                (:NewEnumerator0
                  (bind _state_4 (CallFunction|AddDialogue (Variables|Default|GetspeakerName) "I can only warn. Not fight." (Utilities|Array|MakeArray "Fine")))
                  (switch Utilities|FlowControl|Switch|SwitchonEnum_DialogueState _state_4
                    (:NewEnumerator0
                      (CallFunction|ClearDialogueProgress)
                      (CallFunction|CloseConversation))))))
            (:2
              (bind _state_5 (CallFunction|AddDialogue (Variables|Default|GetspeakerName) "*He chuckles weakly.* 
My wounds are older than you, whelp. 
Save your mercy for yourself. You’ll need it soon." (Utilities|Array|MakeArray "Leave")))
              (switch Utilities|FlowControl|Switch|SwitchonEnum_DialogueState _state_5
                (:NewEnumerator0
                  (CallFunction|ClearDialogueProgress)
                  (CallFunction|CloseConversation))))
            (:3
              (bind _state_6 (CallFunction|AddDialogue (Variables|Default|GetspeakerName) "*He glares at you silently for a moment.* 
... 
I like you. Maybe you won't die in the first room. 
Maybe." (Utilities|Array|MakeArray "Leave")))
              (switch Utilities|FlowControl|Switch|SwitchonEnum_DialogueState _state_6
                (:NewEnumerator0
                  (CallFunction|ClearDialogueProgress)
                  (CallFunction|CloseConversation))))))))))