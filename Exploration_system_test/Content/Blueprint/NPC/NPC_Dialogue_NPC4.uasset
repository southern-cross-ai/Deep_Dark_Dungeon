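; NPC dialogue Blueprint for a mysterious dungeon hermit who offers lore and quest hooks about a vault trial, a sorcerer's relic, and a destined hero.
; Overrides Dialogue, calls the parent, then runs a branching tree at DialogueTreeIndex 0 using nested AddDialogue calls switched on the chosen option.
; Final choices trigger no distinct outcomes; each leaf just clears dialogue progress and closes the conversation.
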(event EventBeginPlay
  (|CallParentFunction) ; 此节点被禁用，将不会被调用。\n从引脚连出引线来编译功能。
)

(event EventTick
  (params (DeltaSeconds :type Float%20%28single-precision%29))
  (|CallParentFunction DeltaSeconds) ; 此节点被禁用，将不会被调用。\n从引脚连出引线来编译功能。
)

(fn Dialogue
  (|CallParentFunction)
  (switch int (Variables|Default|GetDialogueTreeIndex)
    (:0
      (bind (_state _optionindex) (CallFunction|AddDialogue (Variables|Default|GetspeakerName) "Ah, a visitor... It has been many moons since I last spoke with another soul. Tell me, traveler, what brings you to this forsaken place?" (Utilities|Array|MakeArray "I’m seeking treasure and glory. Do you know anything that could help?" "I’m here to defeat the dark power rumored to be in this dungeon." "Just exploring. Who are you, and why are you here?")))
      (switch Utilities|FlowControl|Switch|SwitchonEnum_DialogueState _state
        (:NewEnumerator0
          (switch int _optionindex
            (:0
              (bind (_state_2 _optionindex_2) (CallFunction|AddDialogue (Variables|Default|GetspeakerName) "Treasure and glory, you say? Bah, such things are fleeting! However, I do possess knowledge of a hidden vault, sealed by ancient magic. But to find it, you must first pass a trial." (Utilities|Array|MakeArray "I’m ready. What is this trial?" "A trial? I’m not interested. Just tell me where the vault is.")))
              (switch Utilities|FlowControl|Switch|SwitchonEnum_DialogueState _state_2
                (:NewEnumerator0
                  (switch int _optionindex_2
                    (:0
                      (bind (_state_3 _optionindex_3) (CallFunction|AddDialogue (Variables|Default|GetspeakerName) "Patience, young one. Deep within this dungeon lies a beast that guards the key to the vault. Defeat it, and you shall have what you seek. Fail, and you may never see the light of day again." (Utilities|Array|MakeArray "I accept the trial. I will defeat the beast." "Sounds too risky. I’ll find another way.")))
                      (switch Utilities|FlowControl|Switch|SwitchonEnum_DialogueState _state_3
                        (:NewEnumerator0
                          (switch int _optionindex_3
                            (:0
                              _)
                            (:1
                              _))
                          (CallFunction|ClearDialogueProgress)
                          (CallFunction|CloseConversation))))
                    (:1
                      (bind (_state_4 _optionindex_4) (CallFunction|AddDialogue (Variables|Default|GetspeakerName) "Ah, but knowledge is not so freely given, traveler. Prove your worth, and only then shall the secrets be revealed." (Utilities|Array|MakeArray "Leave")))
                      (switch Utilities|FlowControl|Switch|SwitchonEnum_DialogueState _state_4
                        (:NewEnumerator0
                          (switch int _optionindex_4
                            (:0
                              _)
                            (:1
                              _))
                          (CallFunction|ClearDialogueProgress)
                          (CallFunction|CloseConversation))))))))
            (:1
              (bind (_state_5 _optionindex_5) (CallFunction|AddDialogue (Variables|Default|GetspeakerName) "Ah, the dark power... A vile sorcerer, twisting the very fabric of reality. You seek to end his reign? Very well. But know this: strength alone will not bring you victory." (Utilities|Array|MakeArray "What do I need, then?" "I don’t need your advice. I’ll defeat him my way.")))
              (switch Utilities|FlowControl|Switch|SwitchonEnum_DialogueState _state_5
                (:NewEnumerator0
                  (switch int _optionindex_5
                    (:0
                      (bind (_state_6 _optionindex_6) (CallFunction|AddDialogue (Variables|Default|GetspeakerName) "Wisdom, traveler. In the southern cavern lies an ancient relic, capable of dispelling the sorcerer's dark magic. Seek it out, and you may stand a chance against him. But be warned, the path is perilous." (Utilities|Array|MakeArray "Thank you. I’ll seek the relic." "I don’t trust you. I’ll do this on my own.")))
                      (switch Utilities|FlowControl|Switch|SwitchonEnum_DialogueState _state_6
                        (:NewEnumerator0
                          (switch int _optionindex_6
                            (:0
                              _)
                            (:1
                              _))
                          (CallFunction|ClearDialogueProgress)
                          (CallFunction|CloseConversation))))
                    (:1
                      (bind (_state_7 _optionindex_7) (CallFunction|AddDialogue (Variables|Default|GetspeakerName) "Then go, with stubborn pride as your only ally. But mark my words: without the right tools, you may find yourself lost in darkness." (Utilities|Array|MakeArray "Leave")))
                      (switch Utilities|FlowControl|Switch|SwitchonEnum_DialogueState _state_7
                        (:NewEnumerator0
                          (switch int _optionindex_7
                            (:0
                              _)
                            (:1
                              _))
                          (CallFunction|ClearDialogueProgress)
                          (CallFunction|CloseConversation))))))))
            (:2
              (bind (_state_8 _optionindex_8) (CallFunction|AddDialogue (Variables|Default|GetspeakerName) "Who am I? Just a shadow of the past, a keeper of secrets long forgotten. I came here seeking answers... and now I stay, watching as fools chase shadows. But you... you seem different." (Utilities|Array|MakeArray "Different how?" "You didn’t answer my question. Why are you here?")))
              (switch Utilities|FlowControl|Switch|SwitchonEnum_DialogueState _state_8
                (:NewEnumerator0
                  (switch int _optionindex_8
                    (:0
                      (bind (_state_9 _optionindex_9) (CallFunction|AddDialogue (Variables|Default|GetspeakerName) "You are not driven by mere greed or vengeance. I sense a deeper purpose in you. Perhaps... you are the one destined to end the darkness in these halls. But the choice is yours." (Utilities|Array|MakeArray "I will end the darkness. What must I do?" "I’m not here to be anyone’s savior.")))
                      (switch Utilities|FlowControl|Switch|SwitchonEnum_DialogueState _state_9
                        (:NewEnumerator0
                          (switch int _optionindex_9
                            (:0
                              _)
                            (:1
                              _))
                          (CallFunction|ClearDialogueProgress)
                          (CallFunction|CloseConversation))))
                    (:1
                      (bind (_state_10 _optionindex_10) (CallFunction|AddDialogue (Variables|Default|GetspeakerName) "I sought knowledge, and knowledge I found... at a great cost. Now, I remain, bound to this place by secrets too dangerous to reveal. If you wish to learn, you must first prove you are worthy of such burdens." (Utilities|Array|MakeArray "Then I shall prove myself." "I don't need your secrets.")))
                      (switch Utilities|FlowControl|Switch|SwitchonEnum_DialogueState _state_10
                        (:NewEnumerator0
                          (switch int _optionindex_10
                            (:0
                              _)
                            (:1
                              _))
                          (CallFunction|ClearDialogueProgress)
                          (CallFunction|CloseConversation))))))))))))))