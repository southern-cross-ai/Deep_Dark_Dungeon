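; NPC5 is an interactable NPC Blueprint that starts a conversation when interacted with.
; Its Interact event stores the instigator, then opens the conversation on NPCDialogueNPC5.
; The construction script assigns TxtCharacterName to CharacterNameTxt before running the parent construction script, leaving the rest of that setup to the parent class.
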(event EventBeginPlay
  (|CallParentFunction) ; 此节点被禁用，将不会被调用。\n从引脚连出引线来编译功能。
)

(event Collision|EventActorBeginOverlap
  (params (OtherActor :type Actor%20Object%20Reference))
  (|CallParentFunction OtherActor) ; 此节点被禁用，将不会被调用。\n从引脚连出引线来编译功能。
)

(event EventTick
  (params (DeltaSeconds :type Float%20%28single-precision%29))
  (|CallParentFunction DeltaSeconds) ; 此节点被禁用，将不会被调用。\n从引脚连出引线来编译功能。
)

(event EventInteract
  (params (Instigator :type Actor%20Object%20Reference))
  (Variables|Default|SetInteractInstigator Instigator)
  (Default|OpenConversation (Variables|Default|GetNPC_Dialogue_NPC5)))

(fn ConstructionScript
  (Variables|Default|SetCharacterNameTxt (Variables|Default|GetTxtCharacterName))
  (|CallParentFunction))