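; BP_SelectionCharacter is a character-selection Blueprint that previews the selectable skeletal meshes and records the current choice.
; Its ChangeCharacter event steps through the Character array, wrapping to the first entry after the last, and applies that entry to its Mesh component.
; It then stores the same mesh in GI_Selection's SkeletalMeshSelected, keeping the choice on the game instance.
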(event Custom|Change%20Character
  (if (< (Variables|Default|GetcurrentCharacterIndex) (- (Utilities|Array|Length (Variables|Default|Getcharacter)) 1))
    (Math|Integer|IncrementInt (Variables|Default|GetcurrentCharacterIndex)
      (:%20%20
        _))
    (else
      (Variables|Default|SetcurrentCharacterIndex 0)))
  (Components|SkeletalMesh|SetSkeletalMeshAsset (Variables|Default|GetMesh) (Utilities|Array|Get(acopy) (Variables|Default|Getcharacter) (Variables|Default|GetcurrentCharacterIndex)))
  (bind _asgi_selection (Utilities|Casting|CastToGI_Selection (Game|GetGameInstance)))
  (Variables|/Game/Blueprint/Character_Selection/GI_Selection.GI_Selection_C|SetskeletalMeshSelected _asgi_selection (Utilities|Array|Get(acopy) (Variables|Default|Getcharacter) (Variables|Default|GetcurrentCharacterIndex))))

(event EventBeginPlay)

(event Collision|EventActorBeginOverlap
  (params (OtherActor :type Actor%20Object%20Reference)))

(event EventTick
  (params (DeltaSeconds :type Float%20%28single-precision%29)))

(fn ConstructionScript)