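; Dialogue Blueprint for NPC5, a blacksmith in the tunnels who offers a sword upgrade for enchanted ore or a flame sword for a dragon scale.
; The overridden Dialogue function calls its parent, then builds a hardcoded branching tree at DialogueTreeIndex 0 from nested AddDialogue calls switched on OptionIndex.
; Final replies only clear dialogue progress and close the conversation; no quest, item or gold logic is attached.
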(event EventBeginPlay
  (|CallParentFunction) ; 此节点被禁用，将不会被调用。\n从引脚连出引线来编译功能。
)

(event EventTick
  (params (DeltaSeconds :type Float%20%28single-precision%29))
  (|CallParentFunction DeltaSeconds) ; 此节点被禁用，将不会被调用。\n从引脚连出引线来编译功能。
)

(fn Dialogue
  (|CallParentFunction)
  (switch int (Variables|Default|GetDialogueTreeIndex)
    (:0
      (bind (_state _optionindex) (CallFunction|AddDialogue (Variables|Default|GetspeakerName) "Ah, a new face in these dark tunnels! I see you carry a sword, but it looks like it's seen better days. Care for a bit of an upgrade?" (Utilities|Array|MakeArray "What can you do for my sword?" "I'm looking for a new weapon. Got anything special?" "I’m not interested. Just passing through.")))
      (switch Utilities|FlowControl|Switch|SwitchonEnum_DialogueState _state
        (:NewEnumerator0
          (switch int _optionindex
            (:0
              (bind (_state_2 _optionindex_2) (CallFunction|AddDialogue (Variables|Default|GetspeakerName) "I can strengthen your blade, make it sharper and more durable. But it won’t come cheap. Bring me some enchanted ore from the mines nearby, and I’ll get to work." (Utilities|Array|MakeArray "Where can I find this enchanted ore?" "I’ll pay you in gold instead." "I’m not up for mining. Forget it.")))
              (switch Utilities|FlowControl|Switch|SwitchonEnum_DialogueState _state_2
                (:NewEnumerator0
                  (switch int _optionindex_2
                    (:0
                      (bind (_state_3 _optionindex_3) (CallFunction|AddDialogue (Variables|Default|GetspeakerName) "The ore is deep within the eastern tunnels, guarded by creatures of the dark. It won’t be an easy task, but if you return with the ore, I promise to craft a weapon worthy of legend.\"" (Utilities|Array|MakeArray "I’ll find the ore and bring it back." "Too risky. I'll have to pass.")))
                      (switch Utilities|FlowControl|Switch|SwitchonEnum_DialogueState _state_3
                        (:NewEnumerator0
                          (switch int _optionindex_3
                            (:0
                              _)
                            (:1
                              _))
                          (CallFunction|ClearDialogueProgress)
                          (CallFunction|CloseConversation))))
                    (:1
                      (bind (_state_4 _optionindex_4) (CallFunction|AddDialogue (Variables|Default|GetspeakerName) "Heh, gold you say? That might work... for a lesser upgrade. But if you want the best, you’ll need to put in some effort. The enchanted ore is what truly makes the difference." (Utilities|Array|MakeArray "Fine, I’ll go get the ore." "Then just take my gold for the lesser upgrade." "Not worth it. I’m out.")))
                      (switch Utilities|FlowControl|Switch|SwitchonEnum_DialogueState _state_4
                        (:NewEnumerator0
                          (switch int _optionindex_4
                            (:0
                              _)
                            (:1
                              _)
                            (:2
                              _))
                          (CallFunction|ClearDialogueProgress)
                          (CallFunction|CloseConversation))))
                    (:2
                      (bind (_state_5 _optionindex_5) (CallFunction|AddDialogue (Variables|Default|GetspeakerName) "Suit yourself. A dull blade won’t do you much good in these parts, but it’s your choice." (Utilities|Array|MakeArray "Leave")))
                      (switch Utilities|FlowControl|Switch|SwitchonEnum_DialogueState _state_5
                        (:NewEnumerator0
                          (switch int _optionindex_5
                            (:0
                              _)
                            (:1
                              _))
                          (CallFunction|ClearDialogueProgress)
                          (CallFunction|CloseConversation))))))))
            (:1
              (bind (_state_6 _optionindex_6) (CallFunction|AddDialogue (Variables|Default|GetspeakerName) "A new weapon, you say? I do have something... rare. A flame sword, forged with the fire of a dragon’s breath. But such power comes at a price." (Utilities|Array|MakeArray "What’s the price?" "A flame sword? I’ll take it!" "Sounds too expensive. Never mind.")))
              (switch Utilities|FlowControl|Switch|SwitchonEnum_DialogueState _state_6
                (:NewEnumerator0
                  (switch int _optionindex_6
                    (:0
                      (bind (_state_7 _optionindex_7) (CallFunction|AddDialogue (Variables|Default|GetspeakerName) "You’ll need to bring me a dragon scale. Only then will I be able to forge the sword. There’s a cave to the north where the beast resides... if you’re brave enough to face it." (Utilities|Array|MakeArray "I’ll slay the dragon and bring you a scale." "A dragon? That’s madness. I’ll pass.")))
                      (switch Utilities|FlowControl|Switch|SwitchonEnum_DialogueState _state_7
                        (:NewEnumerator0
                          (switch int _optionindex_7
                            (:0
                              _)
                            (:1
                              _))
                          (CallFunction|ClearDialogueProgress)
                          (CallFunction|CloseConversation))))
                    (:1
                      (bind (_state_8 _optionindex_8) (CallFunction|AddDialogue (Variables|Default|GetspeakerName) "Not so fast! Power like this can’t be bought with mere gold. Prove your worth, bring me a dragon scale, and the sword shall be yours." (Utilities|Array|MakeArray "I’ll get the scale. Wait for me." "No thanks. I’m not facing a dragon.")))
                      (switch Utilities|FlowControl|Switch|SwitchonEnum_DialogueState _state_8
                        (:NewEnumerator0
                          (switch int _optionindex_8
                            (:0
                              _)
                            (:1
                              _))
                          (CallFunction|ClearDialogueProgress)
                          (CallFunction|CloseConversation))))
                    (:2
                      (bind (_state_9 _optionindex_9) (CallFunction|AddDialogue (Variables|Default|GetspeakerName) "Heh, a wise decision. Power always comes at a cost, and not all are willing to pay it." (Utilities|Array|MakeArray "Leave")))
                      (switch Utilities|FlowControl|Switch|SwitchonEnum_DialogueState _state_9
                        (:NewEnumerator0
                          (switch int _optionindex_9
                            (:0
                              _)
                            (:1
                              _))
                          (CallFunction|ClearDialogueProgress)
                          (CallFunction|CloseConversation))))))))
            (:2
              (bind _state_10 (CallFunction|AddDialogue (Variables|Default|GetspeakerName) "Hmph, just passing through, are you? Fair enough. But remember, a strong weapon can mean the difference between life and death in these tunnels." (Utilities|Array|MakeArray "Leave")))
              (switch Utilities|FlowControl|Switch|SwitchonEnum_DialogueState _state_10
                (:NewEnumerator0
                  (CallFunction|ClearDialogueProgress)
                  (CallFunction|CloseConversation))))))))))