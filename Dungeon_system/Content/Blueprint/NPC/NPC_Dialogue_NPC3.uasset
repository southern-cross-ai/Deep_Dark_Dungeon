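; Dialogue Blueprint for NPC3, a jester-like dungeon dweller who offers the player a riddle, a coin-flip wager or a brush-off.
; The Dialogue override calls its parent, then runs a hard-coded branching tree under DialogueTreeIndex 0 through nested AddDialogue option switches.
; Each ending clears dialogue progress and closes the conversation.
; Outcomes are text only: the coin flip always wins, and no key is actually granted.
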(event EventBeginPlay
  (|CallParentFunction) ; 此节点被禁用，将不会被调用。\n从引脚连出引线来编译功能。
)

(event EventTick
  (params (DeltaSeconds :type Float%20%28single-precision%29))
  (|CallParentFunction DeltaSeconds) ; 此节点被禁用，将不会被调用。\n从引脚连出引线来编译功能。
)

(fn Dialogue
  (|CallParentFunction)
  (switch int (Variables|Default|GetDialogueTreeIndex)
    (:0
      (bind (_state _optionindex) (CallFunction|AddDialogue (Variables|Default|GetspeakerName) "Hee hee hee! Look who stumbled into my little corner of darkness! Tell me, adventurer, do you seek fortune, fame, or just a bit of fun?" (Utilities|Array|MakeArray "Who are you, and why are you here?" "Fortune and fame, of course. What do you know?" "I don’t have time for your games, fool.")))
      (switch Utilities|FlowControl|Switch|SwitchonEnum_DialogueState _state
        (:NewEnumerator0
          (switch int _optionindex
            (:0
              (bind (_state_2 _optionindex_2) (CallFunction|AddDialogue (Variables|Default|GetspeakerName) "Oh, me? I’m but a humble entertainer, trapped in this dungeon like the rest of you. But I do know a secret or two… Care for a riddle? Solve it, and I’ll share what I know!" (Utilities|Array|MakeArray "Sure, give me the riddle." "No time for riddles. Just tell me what you know.")))
              (switch Utilities|FlowControl|Switch|SwitchonEnum_DialogueState _state_2
                (:NewEnumerator0
                  (switch int _optionindex_2
                    (:0
                      (bind (_state_3 _optionindex_3) (CallFunction|AddDialogue (Variables|Default|GetspeakerName) "Hee hee! Very well! Listen closely: 'I can be cracked, made, told, and played. What am I?' Solve this, and the secret is yours!" (Utilities|Array|MakeArray "A joke!" "An egg?")))
                      (switch Utilities|FlowControl|Switch|SwitchonEnum_DialogueState _state_3
                        (:NewEnumerator0
                          (switch int _optionindex_3
                            (:0
                              (bind (_state_4 _optionindex_4) (CallFunction|AddDialogue (Variables|Default|GetspeakerName) "Hee hee hee! Correct! A joke it is! Very clever, adventurer. As promised, here’s your prize: the passage to the west holds treasures, but beware, it is also full of traps!" (Utilities|Array|MakeArray "Thanks")))
                              (switch Utilities|FlowControl|Switch|SwitchonEnum_DialogueState _state_4
                                (:NewEnumerator0
                                  (switch int _optionindex_4
                                    (:0
                                      _)
                                    (:1
                                      _))
                                  (CallFunction|ClearDialogueProgress)
                                  (CallFunction|CloseConversation))))
                            (:1
                              (bind (_state_5 _optionindex_5) (CallFunction|AddDialogue (Variables|Default|GetspeakerName) "Oh, so close, but not quite! You may try again... or perhaps leave in ignorance. Your choice!" (Utilities|Array|MakeArray "Leave")))
                              (switch Utilities|FlowControl|Switch|SwitchonEnum_DialogueState _state_5
                                (:NewEnumerator0
                                  (switch int _optionindex_5
                                    (:0
                                      _)
                                    (:1
                                      _))
                                  (CallFunction|ClearDialogueProgress)
                                  (CallFunction|CloseConversation))))))))
                    (:1
                      (bind (_state_6 _optionindex_6) (CallFunction|AddDialogue (Variables|Default|GetspeakerName) "Impatient, are we? Very well, I’ll tell you this: the shadows in the east whisper secrets, but only to those who dare listen." (Utilities|Array|MakeArray "Leave")))
                      (switch Utilities|FlowControl|Switch|SwitchonEnum_DialogueState _state_6
                        (:NewEnumerator0
                          (switch int _optionindex_6
                            (:0
                              _)
                            (:1
                              _))
                          (CallFunction|ClearDialogueProgress)
                          (CallFunction|CloseConversation))))))))
            (:1
              (bind (_state_7 _optionindex_7) (CallFunction|AddDialogue (Variables|Default|GetspeakerName) "Fortune and fame, you say? Hee hee! Aren’t you the greedy one! Very well, I shall offer you a deal. In these tunnels lies a chest. I’ll give you the key, but only if you play my game." (Utilities|Array|MakeArray "I’m listening. What’s the game?" "I don’t trust you. Keep your key.")))
              (switch Utilities|FlowControl|Switch|SwitchonEnum_DialogueState _state_7
                (:NewEnumerator0
                  (switch int _optionindex_7
                    (:0
                      (bind (_state_8 _optionindex_8) (CallFunction|AddDialogue (Variables|Default|GetspeakerName) "Simple, really! I will toss this coin. Heads, you get the key. Tails, you must leave something of value behind. Care to gamble?" (Utilities|Array|MakeArray "Deal. Flip the coin." "No thanks, I don’t gamble.")))
                      (switch Utilities|FlowControl|Switch|SwitchonEnum_DialogueState _state_8
                        (:NewEnumerator0
                          (switch int _optionindex_8
                            (:0
                              (bind (_state_9 _optionindex_9) (CallFunction|AddDialogue (Variables|Default|GetspeakerName) "Hee hee! Fortune favors you today. The key is yours. Now, go forth and claim your prize!" (Utilities|Array|MakeArray "Thanks")))
                              (switch Utilities|FlowControl|Switch|SwitchonEnum_DialogueState _state_9
                                (:NewEnumerator0
                                  (switch int _optionindex_9
                                    (:0
                                      _)
                                    (:1
                                      _))
                                  (CallFunction|ClearDialogueProgress)
                                  (CallFunction|CloseConversation))))
                            (:1
                              (bind (_state_10 _optionindex_10) (CallFunction|AddDialogue (Variables|Default|GetspeakerName) "Hee hee, wise choice! Not everyone has the heart for risk. Maybe you’ll find another way to fortune." (Utilities|Array|MakeArray "Leave")))
                              (switch Utilities|FlowControl|Switch|SwitchonEnum_DialogueState _state_10
                                (:NewEnumerator0
                                  (switch int _optionindex_10
                                    (:0
                                      _)
                                    (:1
                                      _))
                                  (CallFunction|ClearDialogueProgress)
                                  (CallFunction|CloseConversation))))))))
                    (:1
                      (bind (_state_11 _optionindex_11) (CallFunction|AddDialogue (Variables|Default|GetspeakerName) "Oh, so cautious! Where’s the fun in that? Very well, keep your doubts. I’ll be here, should you change your mind." (Utilities|Array|MakeArray "Leave")))
                      (switch Utilities|FlowControl|Switch|SwitchonEnum_DialogueState _state_11
                        (:NewEnumerator0
                          (switch int _optionindex_11
                            (:0
                              _)
                            (:1
                              _))
                          (CallFunction|ClearDialogueProgress)
                          (CallFunction|CloseConversation))))))))
            (:2
              (bind _state_12 (CallFunction|AddDialogue (Variables|Default|GetspeakerName) "Oh, so serious! Fine, fine, I’ll leave you be. But remember, adventurer, laughter is the best weapon in dark places." (Utilities|Array|MakeArray "Leave")))
              (switch Utilities|FlowControl|Switch|SwitchonEnum_DialogueState _state_12
                (:NewEnumerator0
                  (CallFunction|ClearDialogueProgress)
                  (CallFunction|CloseConversation))))))))))