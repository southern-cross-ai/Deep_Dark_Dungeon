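; NPC dialogue Blueprint for an imprisoned character who begs the player for escape and offers rewards for defeating the Dark Sorcerer.
; It overrides the parent's Dialogue function, switching on DialogueTreeIndex (only tree 0 exists) and nesting AddDialogue calls branched by chosen option.
; Every branch ends by clearing dialogue progress and closing the conversation; final accept or decline choices trigger no quest or reward logic.
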(event EventBeginPlay
  (|CallParentFunction) ; 此节点被禁用，将不会被调用。\n从引脚连出引线来编译功能。
)

(event EventTick
  (params (DeltaSeconds :type Float%20%28single-precision%29))
  (|CallParentFunction DeltaSeconds) ; 此节点被禁用，将不会被调用。\n从引脚连出引线来编译功能。
)

(fn Dialogue
  (|CallParentFunction)
  (switch int (Variables|Default|GetDialogueTreeIndex)
    (:0
      (bind (_state _optionindex) (CallFunction|AddDialogue (Variables|Default|GetspeakerName) "Oh, brave adventurer! I can't believe someone has found me here. I've been trapped in this dungeon for so long... Please, help me escape!" (Utilities|Array|MakeArray "Who imprisoned you here, and why?" "I'll help you, but what's in it for me?" "I'm sorry, I can't get involved right now.")))
      (switch Utilities|FlowControl|Switch|SwitchonEnum_DialogueState _state
        (:NewEnumerator0
          (switch int _optionindex
            (:0
              (bind (_state_2 _optionindex_2) (CallFunction|AddDialogue (Variables|Default|GetspeakerName) "It was the Dark Sorcerer. He feared my power and sought to imprison me. Now, I'm just a prisoner, hoping for a chance at freedom." (Utilities|Array|MakeArray "If I defeat the Dark Sorcerer, will you reward me?" "I see... Tell me more about the Dark Sorcerer.")))
              (switch Utilities|FlowControl|Switch|SwitchonEnum_DialogueState _state_2
                (:NewEnumerator0
                  (switch int _optionindex_2
                    (:0
                      (bind (_state_3 _optionindex_3) (CallFunction|AddDialogue (Variables|Default|GetspeakerName) "Yes, of course! I can grant you the enchanted key that unlocks the gate to the hidden treasure room. But you must hurry, for the sorcerer watches over this dungeon with his minions." (Utilities|Array|MakeArray "I accept your quest. I will defeat the sorcerer." "Sounds too risky. I’m out.")))
                      (switch Utilities|FlowControl|Switch|SwitchonEnum_DialogueState _state_3
                        (:NewEnumerator0
                          (switch int _optionindex_3
                            (:0
                              _)
                            (:1
                              _))
                          (CallFunction|ClearDialogueProgress)
                          (CallFunction|CloseConversation))))
                    (:1
                      (bind (_state_4 _optionindex_4) (CallFunction|AddDialogue (Variables|Default|GetspeakerName) "He is a master of dark magic, able to manipulate shadows and summon creatures of the abyss. But he is not invincible; his weakness lies in his arrogance. Strike when he least expects it." (Utilities|Array|MakeArray "Thank you for the information. I’ll take him down." "This sounds too dangerous. I need to prepare first.")))
                      (switch Utilities|FlowControl|Switch|SwitchonEnum_DialogueState _state_4
                        (:NewEnumerator0
                          (switch int _optionindex_4
                            (:0
                              _)
                            (:1
                              _))
                          (CallFunction|ClearDialogueProgress)
                          (CallFunction|CloseConversation))))))))
            (:1
              (bind (_state_5 _optionindex_5) (CallFunction|AddDialogue (Variables|Default|GetspeakerName) "I understand your caution. If you help me, I will grant you a magical amulet that can shield you from dark magic. It will be invaluable as you explore deeper into this dungeon." (Utilities|Array|MakeArray "A magical amulet? You've got a deal." "I'm not convinced. Is that all you have to offer?")))
              (switch Utilities|FlowControl|Switch|SwitchonEnum_DialogueState _state_5
                (:NewEnumerator0
                  (switch int _optionindex_5
                    (:0
                      (bind (_state_6 _optionindex_6) (CallFunction|AddDialogue (Variables|Default|GetspeakerName) "Thank you! The Dark Sorcerer’s lair is further below. Defeat him, and the amulet is yours. May fortune favor you, brave adventurer." (Utilities|Array|MakeArray "Now you’re talking. I’ll help you." "No spell is worth risking my life for.")))
                      (switch Utilities|FlowControl|Switch|SwitchonEnum_DialogueState _state_6
                        (:NewEnumerator0
                          (switch int _optionindex_6
                            (:0
                              _)
                            (:1
                              _))
                          (CallFunction|ClearDialogueProgress)
                          (CallFunction|CloseConversation))))
                    (:1
                      (bind (_state_7 _optionindex_7) (CallFunction|AddDialogue (Variables|Default|GetspeakerName) "If it is power you seek, then know this: I am the keeper of an ancient spell that can bend reality itself. Aid me, and I will teach you its secrets." (Utilities|Array|MakeArray "Now you’re talking. I’ll help you." "No spell is worth risking my life for.")))
                      (switch Utilities|FlowControl|Switch|SwitchonEnum_DialogueState _state_7
                        (:NewEnumerator0
                          (switch int _optionindex_7
                            (:0
                              _)
                            (:1
                              _))
                          (CallFunction|ClearDialogueProgress)
                          (CallFunction|CloseConversation))))))))
            (:2
              (bind _state_8 (CallFunction|AddDialogue (Variables|Default|GetspeakerName) "I understand... This dungeon is full of peril, and not everyone is destined to be a hero. But if you change your mind, I will be here, waiting." (Utilities|Array|MakeArray "Leave")))
              (switch Utilities|FlowControl|Switch|SwitchonEnum_DialogueState _state_8
                (:NewEnumerator0
                  (CallFunction|ClearDialogueProgress)
                  (CallFunction|CloseConversation))))))))))