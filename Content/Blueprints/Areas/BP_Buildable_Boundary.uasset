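; Buildable boundary area actor: a resizable, rotation-locked box with an optional billboard and a child BP_Border that outlines it.
; The construction script turns scale-gizmo changes into stepped AreaSize and AreaHeight adjustments, resets scale to one, then sizes the box and border.
; SnapToGrid aligns the actor to the BP_BuildManager grid using its cell, area size and height step.
; BeginPlay destroys the border unless it is set to show in game.
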(event Custom|SnapToGrid
  (bind _returnvalue (Transformation|GetActorLocation))
  (bind _returnvalue_2 (Actor|GetActorOfClass "/Game/Blueprints/BP_BuildManager.BP_BuildManager_C"))
  (bind _output_get (Variables|Default|SetBuildManager _returnvalue_2))
  (Utilities|IsValid _output_get
    (:Is%20Valid
      (Transformation|SetActorLocation (Math|Conversions|ToVector(Vector2D) (Default|GetCenterOfRectangularArea (Variables|Default|GetBuildManager) (Default|GetCellfromWorldLocation (Variables|Default|GetBuildManager) _returnvalue) (Class|KismetMathLibrary|ToIntPoint(Vector2D) (/ (Variables|Settings|GetAreaSIze) (Variables|/Game/Blueprints/BP_BuildManager.BP_BuildManager_C|GetGridCellSizeXY (Variables|Default|GetBuildManager))))) (Default|RoundHeighttoGridStep (Variables|Default|GetBuildManager) (.Z (Math|Vector|BreakVector _returnvalue)))) false false))))

(event EventBeginPlay
  (if (not (Variables|Settings|GetShowBorderInGame))
    (Actor|DestroyActor (Variables|Default|GetAreaBorder))))

(fn ConstructionScript
  (Transformation|SetActorRotation "0, 0, 0")
  (CallFunction|AutoChangeSizebyScale) ; The scale of this actor automatically resizes the border
  (CallFunction|SetupBillboard)
  (CallFunction|SetupBorder)
  (Rendering|SetVisibility (Variables|Default|GetBox) (Variables|Settings|Editor|GetShowBox) false))

(fn AutoChangeSizebyScale
  (bind _returnvalue (Class|Actor|GetActorRelativeScale3D))
  (bind (_x _y _z) (Math|Vector|BreakVector _returnvalue))
  (bind (_x_2 _y_2 _z_2) (Math|Vector|BreakVector _returnvalue))
  (if (Math|Vector|Equal(Vector) (Class|Actor|GetActorRelativeScale3D) "1.000000,1.000000,1.000000" 0.01)
    _
    (else
      (Variables|Settings|SetAreaSIze (Math|Vector2D|MakeVector2D (Math|Float|SelectFloat (Math|Float|SelectFloat (.X (Math|Vector2D|BreakVector2D (Variables|Settings|GetAreaSIze))) (+ (.X (Math|Vector2D|BreakVector2D (Variables|Settings|GetAreaSIze))) (* (Math|Float|SelectFloat -1.0 1.0 (< _x 1.0)) (Math|Float|Clamp(Float) (/ (.X (Math|Vector2D|BreakVector2D (Variables|Settings|GetAreaSIze))) 2e+01) 1e+01 1e+04))) (== _x_2 1.0)) 0.0 (>= (Math|Float|SelectFloat (.X (Math|Vector2D|BreakVector2D (Variables|Settings|GetAreaSIze))) (+ (.X (Math|Vector2D|BreakVector2D (Variables|Settings|GetAreaSIze))) (* (Math|Float|SelectFloat -1.0 1.0 (< _x 1.0)) (Math|Float|Clamp(Float) (/ (.X (Math|Vector2D|BreakVector2D (Variables|Settings|GetAreaSIze))) 2e+01) 1e+01 1e+04))) (== _x_2 1.0)) 0.0)) (Math|Float|SelectFloat (Math|Float|SelectFloat (.Y (Math|Vector2D|BreakVector2D (Variables|Settings|GetAreaSIze))) (+ (.Y (Math|Vector2D|BreakVector2D (Variables|Settings|GetAreaSIze))) (* (Math|Float|SelectFloat -1.0 1.0 (< _y 1.0)) (Math|Float|Clamp(Float) (/ (.Y (Math|Vector2D|BreakVector2D (Variables|Settings|GetAreaSIze))) 2e+01) 1e+01 1e+04))) (== _y_2 1.0)) 0.0 (>= (Math|Float|SelectFloat (.Y (Math|Vector2D|BreakVector2D (Variables|Settings|GetAreaSIze))) (+ (.Y (Math|Vector2D|BreakVector2D (Variables|Settings|GetAreaSIze))) (* (Math|Float|SelectFloat -1.0 1.0 (< _y 1.0)) (Math|Float|Clamp(Float) (/ (.Y (Math|Vector2D|BreakVector2D (Variables|Settings|GetAreaSIze))) 2e+01) 1e+01 1e+04))) (== _y_2 1.0)) 0.0))))
      (Variables|Settings|SetAreaHeight (Math|Float|SelectFloat (Math|Float|SelectFloat (Variables|Settings|GetAreaHeight) (+ (Variables|Settings|GetAreaHeight) (* (Math|Float|SelectFloat -1.0 1.0 (< _z 1.0)) (Math|Float|Clamp(Float) (/ (Variables|Settings|GetAreaHeight) 2e+01) 0.1 5e+01))) (== _z_2 1.0)) 0.0 (>= (Math|Float|SelectFloat (Variables|Settings|GetAreaHeight) (+ (Variables|Settings|GetAreaHeight) (* (Math|Float|SelectFloat -1.0 1.0 (< _z 1.0)) (Math|Float|Clamp(Float) (/ (Variables|Settings|GetAreaHeight) 2e+01) 0.1 5e+01))) (== _z_2 1.0)) 0.0)))))
  (Transformation|SetActorScale3D "1.000000,1.000000,1.000000")
  (Components|Box|SetBoxExtent (Variables|Default|GetBox) (Math|Vector|MakeVector (.x (* (Variables|Settings|GetAreaSIze) 0.5)) (.y (* (Variables|Settings|GetAreaSIze) 0.5)) (* (Variables|Settings|GetAreaHeight) 0.5)) false))

(fn SetupBillboard
  (if (Variables|Settings|Editor|GetShowBillboard)
    (Transformation|SetRelativeLocation (Variables|Default|GetBillboard) (+ (Variables|Settings|Editor|GetBillboardOffset) (Math|Vector|MakeVector 0.0 0.0 (* (Variables|Settings|GetAreaHeight) 0.5))) false false)
    (else
      (Rendering|SetVisibility (Variables|Default|GetBillboard) false false))))

(fn SetupBorder
  (if (Variables|Settings|Editor|GetShowBorderInEditor)
    (bind _returnvalue (AddComponent|AddChildActorComponent false :!pinned true)) ; Set border parameters here, in the "Settings" rollout
    (bind _asbp_border (Utilities|Casting|CastToBP_Border (Variables|/Script/Engine.ChildActorComponent|GetChildActor _returnvalue)))
    (Variables|Default|SetAreaBorder _asbp_border)
    (Variables|/Game/Blueprints/Border/BP_Border.BP_Border_C|SetBorderSIze (Variables|Default|GetAreaBorder) (Variables|Settings|GetAreaSIze))
    (Variables|/Game/Blueprints/Border/BP_Border.BP_Border_C|SetBorderHeight (Variables|Default|GetAreaBorder) (Variables|Settings|GetAreaHeight))
    (Default|SetupBorder (Variables|Default|GetAreaBorder))))