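; Child building placer for demo style 05 that previews a placeable object on the BuildManager grid and spawns it.
; On cursor cell change or forced refresh, it centers the mesh on the footprint and checks every cell's validity, occupancy and height difference.
; Each tick, it optionally checks for units in the area and swaps the whole-mesh accepted or rejected material.
; BuildObject re-validates before spawning with cell and direction data.
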(event EventBeginPlay
  (|CallParentFunction) ; Object Data setting here
  (Variables|Default|SetForceUpdatePlaceIndicators true))

(event EventTick
  (params (DeltaSeconds :type Float%20%28single-precision%29))
  (CallFunction|DrawPlacementIndicators))

(fn ConstructionScript)

(fn RotateObjectPlacer
  (params (Left :type Boolean))
  (|CallParentFunction Left)
  (Variables|Default|SetForceUpdatePlaceIndicators true))

(fn DrawPlacementIndicators
  (bind _objectsize (Variables|Default|GetObjectSize))
  (bind _obectmesh (Variables|Default|GetObectMesh))
  (bind _buildmanager (Variables|Default|GetBuildManager))
  (bind _cellundercursor (Variables|/Game/Blueprints/BP_BuildManager.BP_BuildManager_C|GetCellUnderCursor _buildmanager))
  (bind _center (Default|GetCenterOfRectangularArea _buildmanager _cellundercursor _objectsize))
  (Utilities|FlowControl|Sequence
    (:then_0
      (if (or (Variables|/Game/Blueprints/BP_BuildManager.BP_BuildManager_C|GetCellUnderCursorHasChanged (Variables|Default|GetBuildManager)) (Variables|Default|GetForceUpdatePlaceIndicators))
        (Variables|Default|SetForceUpdatePlaceIndicators false)
        (Variables|Default|SetCanBuild true)
        (bind _location (Default|GetCellLocation _buildmanager _cellundercursor))
        (LocalVariables|SetBaseBuildLevelLOCAL (.z _location))
        (Transformation|SetWorldLocation (Variables|Default|GetObectMesh) (Math|Vector|MakeVector (.x _center) (.y _center) (LocalVariables|GetBaseBuildLevelLOCAL)) false false)
        (bind _cells (Default|GetCellsinRectangularArea (Variables|Default|GetBuildManager) (Variables|/Game/Blueprints/BP_BuildManager.BP_BuildManager_C|GetCellUnderCursor (Variables|Default|GetBuildManager)) (Variables|Default|GetObjectSize)))
        (for _array_element _cells
          (bind (_location_2 _success) (Default|GetCellLocation (Variables|Default|GetBuildManager) _array_element))
          (if (not (Math|Boolean|ANDBoolean (not (Default|GetOccupancyData (Variables|Default|GetBuildManager) _array_element)) (< (Math|Float|Absolute(Float) (- (.z _location_2) (LocalVariables|GetBaseBuildLevelLOCAL))) (Variables|Default|GetMaxHeightDifferenceForConstruction)) _success))
            (Variables|Default|SetCanBuild false)))))
    (:then_1
      (if (Variables|Default|GetCheckUnitsInBuildArea)
        (bind _unitsfound (Default|FindUnitsinRectangularArea (Variables|Default|GetBuildManager) (Variables|/Game/Blueprints/BP_BuildManager.BP_BuildManager_C|GetCellUnderCursor (Variables|Default|GetBuildManager)) (Variables|Default|GetObjectSize) "ObjectTypeQuery3" 5e+03))
        (Variables|Default|SetHasUnitsInBuildArea _unitsfound)
        (if _unitsfound
          (Variables|Default|SetForceUpdatePlaceIndicators true))))
    (:then_2
      (if (and (Variables|Default|GetCanBuild) (not (and (Variables|Default|GetCheckUnitsInBuildArea) (Variables|Default|GetHasUnitsInBuildArea))))
        (Rendering|Material|SetMaterial _obectmesh 0 (Variables|Default|GetBuildingAcceptedMaterial))
        (else
          (Rendering|Material|SetMaterial _obectmesh 0 (Variables|Default|GetBuildingRejectedMaterial)))))))

(fn BuildObject
  (bind _buildmanager (Variables|Default|GetBuildManager))
  (bind _buildmanager_2 (Variables|Default|GetBuildManager))
  (bind _objectsize (Variables|Default|GetObjectSize))
  (bind _cellundercursor (Variables|/Game/Blueprints/BP_BuildManager.BP_BuildManager_C|GetCellUnderCursor _buildmanager_2))
  (bind _center (Default|GetCenterOfRectangularArea _buildmanager _cellundercursor _objectsize))
  (Variables|Default|SetForceUpdatePlaceIndicators true)
  (CallFunction|DrawPlacementIndicators) ; Final check construction area
  (if (and (Variables|Default|GetCanBuild) (not (and (Variables|Default|GetCheckUnitsInBuildArea) (Variables|Default|GetHasUnitsInBuildArea))))
    (Variables|Default|SetForceUpdatePlaceIndicators true)
    (Game|SpawnActorfromClass (Variables|Default|GetPlaceableObjectClass) (Math|Transform|MakeTransform (Math|Vector|MakeVector (.x _center) (.y _center) (.z (Variables|/Game/Blueprints/BP_BuildManager.BP_BuildManager_C|GetLocationUnderCursor%28Camera%29 _buildmanager))) "0, 0, 0" "1.000000,1.000000,1.000000") "Undefined" "SelectDefaultAtRuntime" 0 (Variables|Default|GetObjectNameInTable) (Utilities|Struct|MakeS_PlaceableObjects_Dynamic_Data true _buildmanager _cellundercursor (Variables|Default|GetBuildDirection)) 0)))