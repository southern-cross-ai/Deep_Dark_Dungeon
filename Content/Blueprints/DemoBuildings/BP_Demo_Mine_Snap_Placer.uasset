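; Demo mine placer that snaps the building preview onto a free cell holding the matching resource type within the footprint under the cursor.
; Indicator planes and the preview mesh update when the cursor's cell changes or an update is forced, showing red/green-style accepted or rejected materials.
; An optional unit check marks occupied cells as rejected.
; BuildObject re-validates, then spawns the placeable centred on the snapped cell's area.
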(event EventBeginPlay
  (bind _objectsize (Variables|Default|GetObjectSize))
  (bind _buildmanager (Variables|Default|GetBuildManager))
  (bind _gridcellsizexy (Variables|/Game/Blueprints/BP_BuildManager.BP_BuildManager_C|GetGridCellSizeXY _buildmanager))
  (bind _returnvalue (/ _gridcellsizexy 1.1e+02))
  (|CallParentFunction)
  (Variables|Default|SetForceUpdatePlaceIndicators true)
  (for _index (range 0 (- (* (.x _objectsize) (.y _objectsize)) 1))
    (bind _staticmesh (CallFunction|GetReusableMesh (Variables|Default|GetPlaceIndicators) (Variables|Default|GetPlaceMeshUsingAmount) "/Game/Meshes/SM_Plane_100x100.SM_Plane_100x100" true))
    (Transformation|SetRelativeScale3D _staticmesh (Math|Vector|MakeVector _returnvalue _returnvalue 1.0))))

(event EventTick
  (params (DeltaSeconds :type Float%20%28single-precision%29))
  (CallFunction|DrawPlacementIndicators))

(fn ConstructionScript
  (|CallParentFunction))

(fn DrawPlacementIndicators
  (bind _buildmanager (Variables|Default|GetBuildManager))
  (Utilities|FlowControl|Sequence
    (:then_0
      (if (or (Variables|/Game/Blueprints/BP_BuildManager.BP_BuildManager_C|GetCellUnderCursorHasChanged (Variables|Default|GetBuildManager)) (Variables|Default|GetForceUpdatePlaceIndicators))
        (Variables|Default|SetForceUpdatePlaceIndicators false)
        (Variables|Default|SetCanBuild true)
        (Utilities|FlowControl|Sequence
          (:then_0
            (Variables|Default|SetHasResourceInBuildArea false)
            (bind _cells (Default|GetCellsinRectangularArea (Variables|Default|GetBuildManager) (Variables|/Game/Blueprints/BP_BuildManager.BP_BuildManager_C|GetCellUnderCursor (Variables|Default|GetBuildManager)) (Variables|Default|GetObjectSize)))
            (Variables|Default|SetLastCells _cells)
            (bind _array_element (Utilities|Array|ForEachLoopwithBreak (Variables|Default|GetLastCells) :!label _label)
              (:LoopBody
                (bind (_type _hasdata) (Default|GetResourceTypeData (Variables|Default|GetBuildManager) _array_element))
                (if (Math|Boolean|ANDBoolean (== (Variables|Default|GetResourceType) _type) _hasdata (not (.HasData (Default|GetObjectData (Variables|Default|GetBuildManager) _array_element))))
                  (Variables|Default|SetHasResourceInBuildArea true)
                  (Variables|Default|SetSnapCell _array_element)
                  (goto _label Break)))
              (:Completed
                (if (Variables|Default|GetHasResourceInBuildArea)
                  (bind _cells_2 (Default|GetCellsinRectangularArea (Variables|Default|GetBuildManager) (Variables|Default|GetSnapCell) (Variables|Default|GetObjectSize)))
                  (Variables|Default|SetLastCells _cells_2)
                  (for (_array_element_2 _array_index) (Variables|Default|GetLastCells)
                    (bind _location (Default|GetCellLocation (Variables|Default|GetBuildManager) _array_element_2))
                    (Transformation|SetWorldLocation (Utilities|Array|Get(acopy) (Variables|Default|GetPlaceIndicators) _array_index) _location false false)
                    (Rendering|Material|SetMaterial (Utilities|Array|Get(acopy) (Variables|Default|GetPlaceIndicators) _array_index) 0 (Variables|Default|GetPlaceAcceptedMaterial)))
                  (else
                    (for (_array_element_3 _array_index_2) (Variables|Default|GetLastCells)
                      (bind _location_2 (Default|GetCellLocation (Variables|Default|GetBuildManager) _array_element_3))
                      (Transformation|SetWorldLocation (Utilities|Array|Get(acopy) (Variables|Default|GetPlaceIndicators) _array_index_2) _location_2 false false)
                      (Rendering|Material|SetMaterial (Utilities|Array|Get(acopy) (Variables|Default|GetPlaceIndicators) _array_index_2) 0 (Variables|Default|GetPlaceRejectedMaterial))
                      (Variables|Default|SetCanBuild false)))))))
          (:then_1
            (bind _location_3 (Default|GetCellLocation (Variables|Default|GetBuildManager) (select (Variables|Default|GetHasResourceInBuildArea) (Variables|Default|GetSnapCell) (Variables|/Game/Blueprints/BP_BuildManager.BP_BuildManager_C|GetCellUnderCursor _buildmanager))))
            (Transformation|SetWorldLocation (Variables|Default|GetObectMesh) (Math|Vector|MakeVector (.x (Default|GetCenterOfRectangularArea _buildmanager (select (Variables|Default|GetHasResourceInBuildArea) (Variables|Default|GetSnapCell) (Variables|/Game/Blueprints/BP_BuildManager.BP_BuildManager_C|GetCellUnderCursor _buildmanager)) (Variables|Default|GetObjectSize))) (.y (Default|GetCenterOfRectangularArea _buildmanager (select (Variables|Default|GetHasResourceInBuildArea) (Variables|Default|GetSnapCell) (Variables|/Game/Blueprints/BP_BuildManager.BP_BuildManager_C|GetCellUnderCursor _buildmanager)) (Variables|Default|GetObjectSize))) (.z _location_3)) false false)))))
    (:then_1
      (if (Variables|Default|GetCheckUnitsInBuildArea)
        (if (Variables|Default|GetHasResourceInBuildArea)
          (bind (_unitsfound _unitsincells) (Default|FindUnitsinRectangularArea (Variables|Default|GetBuildManager) (Variables|Default|GetSnapCell) (Variables|Default|GetObjectSize) "ObjectTypeQuery3" 5e+03))
          (Variables|Default|SetHasUnitsInBuildArea _unitsfound)
          (if _unitsfound
            (Variables|Default|SetForceUpdatePlaceIndicators true)
            (for _array_element_4 _unitsincells
              (LocalVariables|SetIndexLOCAL (Utilities|Array|FindItem (Variables|Default|GetLastCells) _array_element_4))
              (if (>= (LocalVariables|GetIndexLOCAL) 0)
                (Rendering|Material|SetMaterial (Utilities|Array|Get(acopy) (Variables|Default|GetPlaceIndicators) (LocalVariables|GetIndexLOCAL)) 0 (Variables|Default|GetPlaceRejectedMaterial))))))))))

(fn BuildObject
  (bind _buildmanager (Variables|Default|GetBuildManager))
  (bind _objectsize (Variables|Default|GetObjectSize))
  (bind _snapcell (Variables|Default|GetSnapCell))
  (bind _center (Default|GetCenterOfRectangularArea _buildmanager _snapcell _objectsize))
  (Variables|Default|SetForceUpdatePlaceIndicators true)
  (CallFunction|DrawPlacementIndicators) ; Final check construction area
  (if (and (Variables|Default|GetCanBuild) (not (and (Variables|Default|GetCheckUnitsInBuildArea) (Variables|Default|GetHasUnitsInBuildArea))))
    (Variables|Default|SetForceUpdatePlaceIndicators true)
    (Game|SpawnActorfromClass (Variables|Default|GetPlaceableObjectClass) (Math|Transform|MakeTransform (Math|Vector|MakeVector (.x _center) (.y _center) (.z (Variables|/Game/Blueprints/BP_BuildManager.BP_BuildManager_C|GetLocationUnderCursor%28Camera%29 _buildmanager))) "0, 0, 0" "1.000000,1.000000,1.000000") "Undefined" "SelectDefaultAtRuntime" 0 (Variables|Default|GetObjectNameInTable) (Utilities|Struct|MakeS_PlaceableObjects_Dynamic_Data true _buildmanager _snapcell (Variables|Default|GetBuildDirection)) 0)))

(fn RotateObjectPlacer
  (params (Left :type Boolean))
  (|CallParentFunction Left)
  (Variables|Default|SetForceUpdatePlaceIndicators true))