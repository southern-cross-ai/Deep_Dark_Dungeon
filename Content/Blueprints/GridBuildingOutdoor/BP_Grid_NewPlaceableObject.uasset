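; Placeable grid building that constructs itself over time, then can be upgraded or moved.
; Tick accumulates SpawnedTime, which selects staged construction meshes until BuildingTime elapses, then the current level's mesh shows.
; Workers spawn nearby on first construction and are destroyed on completion; upgrading raises the level and restarts the timer.
; Moving a completed building passes its state to BP_BuildManager's active placer, frees occupied cells and destroys the actor.
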(event Custom|BuildingMovement
  (if (Variables|Default|GetbuildingComplete)
    (Utilities|FlowControl|Sequence
      (:then_0
        (bind _returnvalue (Actor|GetActorOfClass "/Game/Blueprints/BP_BuildManager.BP_BuildManager_C"))
        (Utilities|FlowControl|Delay 0.0001)
        (Default|EnableBuildingTool _returnvalue (Variables|Default|GetObjectNameInTable))
        (Components|StaticMesh|SetStaticMesh (Variables|/Game/Blueprints/BP_ObjectPlacer_Base_Class.BP_ObjectPlacer_Base_Class_C|GetObectMesh (Variables|/Game/Blueprints/BP_BuildManager.BP_BuildManager_C|GetActiveObjectPlacer _returnvalue)) (Variables|/Script/Engine.StaticMeshComponent|GetStaticMesh (Variables|Default|GetStaticMesh))) ; Change Placer Static Mesh
        ;[1 1 1] Parse Current Data Into New Building
        (bind _asbp_grid_new_placer (Utilities|Casting|CastToBP_Grid_NewPlacer (Variables|/Game/Blueprints/BP_BuildManager.BP_BuildManager_C|GetActiveObjectPlacer _returnvalue))
          (:then
            (Utilities|FlowControl|Sequence
              (:then_0
                (Variables|/Game/Blueprints/GridBuildingOutdoor/BP_Grid_NewPlacer.BP_Grid_NewPlacer_C|SetholdingOldBuilding _asbp_grid_new_placer true))
              (:then_1
                (Variables|/Game/Blueprints/GridBuildingOutdoor/BP_Grid_NewPlacer.BP_Grid_NewPlacer_C|SetcurrentLevel _asbp_grid_new_placer (Variables|Default|GetcurrentLevel)))
              (:then_2
                (Variables|/Game/Blueprints/GridBuildingOutdoor/BP_Grid_NewPlacer.BP_Grid_NewPlacer_C|SetbuildingComplete _asbp_grid_new_placer (Variables|Default|GetbuildingComplete)))
              (:then_3
                (Variables|/Game/Blueprints/GridBuildingOutdoor/BP_Grid_NewPlacer.BP_Grid_NewPlacer_C|SetspawnedTime _asbp_grid_new_placer (Variables|Default|GetspawnedTime)))))
          (:CastFailed
            (Development|PrintString "ERROR: Cast NewPlacer Failed" true true "(R=1.000000,G=0.003032,B=0.000000,A=1.000000)"))))
      (:then_1
        (for _array_element (Variables|Default|GetOccupiedCells)
          (Default|SetOccupancyData _returnvalue _array_element false)))
      (:then_3
        (Utilities|FlowControl|Delay 0.0001)
        (Actor|DestroyActor)))))

(event EventBeginPlay
  (|CallParentFunction)
  (Utilities|FlowControl|Sequence
    (:then_0
      (Actor|Tick|SetActorTickEnabled true))
    (:then_1
      (bind _returnvalue (Actor|GetActorOfClass "/Game/Blueprints/BP_BuildManager.BP_BuildManager_C"))
      (Default|DisableBuildingTool _returnvalue))
    (:then_2
      (Transformation|SetWorldRotation (Variables|Default|GetStaticMesh) (Math|Rotator|MakeRotator 0.0 0.0 (Utilities|Select :Index (Variables|Default|GetObjectDirection) :Option%200 0.0 :Option%201 9e+01 :Option%202 1.8e+02 :Option%203 -9e+01)) false false))))

(event EventTick
  (params (DeltaSeconds :type Float%20%28single-precision%29))
  (Utilities|FlowControl|Sequence
    (:then_0
      ;[1 1 1] Add spawned Time each Tick
      (bind _output_get (Variables|Default|SetspawnedTime (+ (Variables|Default|GetspawnedTime) DeltaSeconds)))
      (Development|PrintString (Utilities|String|ToString(Float) _output_get) false false "(R=0.848929,G=1.000000,B=0.423130,A=1.000000)" 2e+01))
    (:then_1
      (if (not (Variables|Default|GetbuildingComplete))
        (bind _mesh (CallFunction|GetBuildingProcedureMesh))
        (Components|StaticMesh|SetStaticMesh (Variables|Default|GetStaticMesh) _mesh)))))

(fn ConstructionScript)

(fn GetBuildingProcedureMesh
  (bind _workers (Variables|Default|GetWorkers))
  (bind _spawnedtime (Variables|Default|GetspawnedTime))
  (bind _buildingtime (Variables|Default|GetbuildingTime))
  (bind _buildingproceduremesh (Variables|Default|GetBuildingProcedureMesh))
  (bind _returnvalue (/ _spawnedtime _buildingtime))
  ;[1 1 1] Generate workers
  (if (Variables|Default|GetbHasWorkerSpawned)
    _
    (else
      (CallFunction|Worker self)
      (Variables|Default|SetbHasWorkerSpawned true)))
  (if (>= _returnvalue 1.0)
    (Variables|Default|SetbuildingComplete true)
    ;[1 1 1] Destroy workers
    (if (== (Utilities|Array|Length _workers) 0)
      _
      (else
        (for _array_element _workers
          (if (Utilities|IsValid _array_element)
            (Actor|DestroyActor _array_element)
            (else
              (return (Utilities|Array|Get(acopy) (Variables|Default|GetMeshLevels) (Variables|Default|GetcurrentLevel))))))))
    (return (Utilities|Array|Get(acopy) (Variables|Default|GetMeshLevels) (Variables|Default|GetcurrentLevel)))
    (else
      (return (Utilities|Array|Get(acopy) _buildingproceduremesh (Math|Float|Floor (* _returnvalue (Utilities|Array|Length _buildingproceduremesh))))))))

(fn UpgradeBuilding
  (if (< (Variables|Default|GetcurrentLevel) (- (Utilities|Array|Length (Variables|Default|GetMeshLevels)) 1))
    (Variables|Default|SetcurrentLevel (+ (Variables|Default|GetcurrentLevel) 1))
    (Variables|Default|SetspawnedTime 0.0)
    (Variables|Default|SetbuildingComplete false)
    (return true)
    (else
      (return false))))

(fn Worker
  (params (self2 :type Actor%20Object%20Reference))
  ;[1 1 1] Worker
  (for _index (range 0 2)
    (bind _returnvalue (Game|SpawnActorfromClass "/Game/Blueprints/Characters/BP_Worker.BP_Worker_C" (Math|Transform|MakeTransform (+ (Math|Vector|MakeVector (Math|Random|RandomFloatinRange -3e+02 3e+02) (Math|Random|RandomFloatinRange -3e+02 3e+02) 0.0) (Transformation|GetActorLocation self2)) (Math|Rotator|MakeRotator 0.0 0.0 (Math|Random|RandomFloatinRange 0.0 3.6e+02))) "AdjustIfPossibleButAlwaysSpawn" "MultiplyWithRoot" 0 0))
    (Utilities|Array|Add (Variables|Default|GetWorkers) _returnvalue)
    (Development|PrintString "Workers Added")))