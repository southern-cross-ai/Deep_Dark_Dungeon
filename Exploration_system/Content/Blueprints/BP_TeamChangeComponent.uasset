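; Team-change component that hands player control over to its owning pawn when HandleEvent fires.
; If the owner has an AI controller, SwitchController swaps possession, so the player takes the owner and that AI takes the previous pawn.
; The AI then moves that pawn to the ExplorationPlayerController's cached destination.
; HP and movement-point bars are hidden on the old BP_PlayerTeam pawn and shown on the new one.
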(event EventBeginPlay)

(event EventTick
  (params (DeltaSeconds :type Float%20%28single-precision%29)))

(event EventHandleEvent
  (CallFunction|SwitchController))

(fn SwitchController
  (bind _returnvalue (Game|GetPlayerController 0))
  (bind _returnvalue_2 (Components|GetOwner))
  (bind _returnvalue_3 (AI|GetAIController _returnvalue_2))
  (Variables|Default|SetTargetTeam _returnvalue_2)
  (Variables|Default|SetTargetAIController _returnvalue_3)
  (Utilities|IsValid _returnvalue_3
    (:Is%20Valid
      (Variables|Default|SetPlayerController _returnvalue)
      (bind _asexploration_player_controller (Utilities|Casting|CastToExplorationPlayerController _returnvalue))
      (Variables|Default|SetCurrentTeam (Pawn|GetControlledPawn _returnvalue))
      (Pawn|UnPossess (Variables|Default|GetPlayerController))
      (Pawn|UnPossess (Variables|Default|GetTargetAIController))
      (bind _aspawn (Utilities|Casting|CastToPawn (Variables|Default|GetTargetTeam)))
      (Pawn|Possess (Variables|Default|GetPlayerController) _aspawn)
      (Pawn|Possess (Variables|Default|GetTargetAIController) (Variables|Default|GetCurrentTeam))
      (AI|Navigation|SimpleMovetoLocation (Variables|Default|GetTargetAIController) (Variables|/Script/Exploration.ExplorationPlayerController|GetCachedDestination _asexploration_player_controller))
      (bind _asbp_player_team (Utilities|Casting|CastToBP_PlayerTeam (Variables|Default|GetCurrentTeam)))
      (Rendering|SetVisibility (Variables|/Game/Blueprints/BP_PlayerTeam.BP_PlayerTeam_C|GetHPbar _asbp_player_team) false false)
      (bind _asbp_player_team_2 (Utilities|Casting|CastToBP_PlayerTeam (Variables|Default|GetTargetTeam)))
      (Rendering|SetVisibility (Variables|/Game/Blueprints/BP_PlayerTeam.BP_PlayerTeam_C|GetHPbar _asbp_player_team_2) true false))))